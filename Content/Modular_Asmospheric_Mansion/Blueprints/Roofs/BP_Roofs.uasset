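; Modular roof piece for the atmospheric mansion kit, configured in the editor through type and variant enums.
; The construction script branches on corner, low, middle or side type, then assigns and shows the chosen variant's mesh on its own component.
; Optional paint settings push color, intensity, contrast and desaturation to that mesh's materials, and an enum swaps between two roof materials.
; BeginPlay calls a collision function on all components under the root.
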(event EventBeginPlay
  (CallFunction|FSetCollision (Variables|Default|GetDefaultSceneRoot) true))

(event Collision|EventActorBeginOverlap
  (params (OtherActor :type Actor%20Object%20Reference)))

(event EventTick
  (params (DeltaSeconds :type Float%20%28single-precision%29)))

(fn ConstructionScript
  (switch Utilities|FlowControl|Switch|SwitchonE_RoofTypes (Variables|Default|GetRoof%20Types)
    (:NewEnumerator0
      (|Corners))
    (:NewEnumerator1
      (|Low))
    (:NewEnumerator2
      (|Middle))
    (:NewEnumerator3
      (|Side))))

(fn SetMeshFunction
  (params (Target :type Static%20Mesh%20Component%20Object%20Reference) (NewMesh :type Static%20Mesh%20Object%20Reference))
  (Components|StaticMesh|SetStaticMesh Target NewMesh)
  (Rendering|SetVisibility Target true false)
  (CallFunction|PaintattribFunc (Utilities|Array|MakeArray Target)))

(fn ChangeMatParameters
  (params (PaintColor_Change :type Linear%20Color%20Structure :default "(R=1.000000,G=1.000000,B=1.000000,A=1.000000)") (Paint%20Density :type Float%20%28single-precision%29) (Paint%20Contrast :type Float%20%28single-precision%29) (Desaturation :type Float%20%28single-precision%29) (Target :type Array%20of%20Mesh%20Component%20Object%20References))
  (Rendering|Material|SetScalarParameterValueonMaterials Target "Paint_Intensity" Paint%20Density)
  (Rendering|Material|SetVectorParameterValueonMaterials Target "PaintColor" (Math|Conversions|ToVector(LinearColor) PaintColor_Change))
  (Rendering|Material|SetScalarParameterValueonMaterials Target "Paint_Contrast" Paint%20Contrast)
  (Rendering|Material|SetScalarParameterValueonMaterials Target "Desaturation" Desaturation))

(fn PaintattribFunc
  (params ([0] :type Array%20of%20Mesh%20Component%20Object%20References))
  (if (Variables|PaintAttribs|GetPaint%20Active%20?)
    (CallFunction|ChangeMatParameters (Variables|PaintAttribs|GetPaint%20Color%20Change) (Variables|PaintAttribs|GetPaint%20Density) (Variables|PaintAttribs|GetPaint%20Contrast) (Variables|PaintAttribs|GetDesaturation) [0])))

(fn ChangeRoofMatFunc
  (params ([0] :type Static%20Mesh%20Component%20Object%20Reference) ([1] :type Static%20Mesh%20Component%20Object%20Reference) ([2] :type Static%20Mesh%20Component%20Object%20Reference) ([3] :type Static%20Mesh%20Component%20Object%20Reference) ([4] :type Static%20Mesh%20Component%20Object%20Reference) ([5] :type Static%20Mesh%20Component%20Object%20Reference) ([6] :type Static%20Mesh%20Component%20Object%20Reference) ([7] :type Static%20Mesh%20Component%20Object%20Reference) ([8] :type Static%20Mesh%20Component%20Object%20Reference) ([9] :type Static%20Mesh%20Component%20Object%20Reference) ([10] :type Static%20Mesh%20Component%20Object%20Reference) ([11] :type Static%20Mesh%20Component%20Object%20Reference) ([12] :type Static%20Mesh%20Component%20Object%20Reference) ([13] :type Static%20Mesh%20Component%20Object%20Reference) ([14] :type Static%20Mesh%20Component%20Object%20Reference) ([15] :type Static%20Mesh%20Component%20Object%20Reference))
  (bind _array (Utilities|Array|MakeArray [0] [1] [2] [3] [4] [5] [6] [7] [8] [9] [10] [11] [12] [13] [14] [15]))
  (switch Utilities|FlowControl|Switch|SwitchonE_RoofMatTypes (Variables|Default|GetRoof%20Material%20Types)
    (:NewEnumerator0
      (Rendering|Material|SetMaterial _array 0 "/Game/Modular_Asmospheric_Mansion/Materials/Instance/MI_Roof.MI_Roof"))
    (:NewEnumerator1
      (Rendering|Material|SetMaterial _array 0 "/Game/Modular_Asmospheric_Mansion/Materials/Instance/Alternatives/MI_Roof_Tile_02.MI_Roof_Tile_02"))))