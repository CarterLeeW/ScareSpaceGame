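; BP_Base is a modular outer wall base piece for a mansion kit, configured in its construction script.
; BaseCorner shows a wood pillar; otherwise the Dimensions enum selects which wall mesh component to fill and reveal, including a windowed variant.
; For walls only, an optional paint pass sets material parameters for color, intensity, contrast and desaturation.
; Collision is applied to all descendant components on construction and again at BeginPlay.
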(event EventBeginPlay
  (CallFunction|FSetCollision (Variables|Default|GetDefaultSceneRoot) true))

(event Collision|EventActorBeginOverlap
  (params (OtherActor :type Actor%20Object%20Reference)))

(event EventTick
  (params (DeltaSeconds :type Float%20%28single-precision%29)))

(fn ConstructionScript
  (bind _sm_outer_wall_base_1x05m (Variables|Default|GetSM_outer_wall_base_1x05m))
  (bind _sm_outer_wall_base_1x1m (Variables|Default|GetSM_outer_wall_base_1x1m))
  (bind _sm_outer_wall_base_1x2m (Variables|Default|GetSM_outer_wall_base_1x2m))
  (bind _sm_outer_wall_base_1x3m (Variables|Default|GetSM_outer_wall_base_1x3m))
  (bind _sm_outer_wall_base_1x4m (Variables|Default|GetSM_outer_wall_base_1x4m))
  (bind _sm_outer_wall_base_windowed_1x4m (Variables|Default|GetSM_outer_wall_base_windowed_1x4m))
  (bind _sm_wood_pillar_04 (Variables|Default|GetSM_wood_pillar_04))
  (CallFunction|FSetCollision (Variables|Default|GetDefaultSceneRoot) true)
  (if (Variables|Default|GetBase%20Corner%20?)
    ;[0 0 0] Corner
    (Components|StaticMesh|SetStaticMesh _sm_wood_pillar_04 "/Game/Modular_Asmospheric_Mansion/Meshes/Planks/SM_wood_pillar_04.SM_wood_pillar_04")
    (Rendering|SetVisibility _sm_wood_pillar_04 true false)
    (else
      (switch Utilities|FlowControl|Switch|SwitchonE_Base_Dimension (Variables|Default|GetDimensions)
        (:NewEnumerator0
          _)
        (:NewEnumerator1
          _)
        (:NewEnumerator2
          _)
        (:NewEnumerator3
          _)
        (:NewEnumerator4
          _)
        (:NewEnumerator5
          _))
      (CallFunction|SetMeshDimensionFunction _sm_outer_wall_base_1x05m _sm_outer_wall_base_1x1m _sm_outer_wall_base_1x2m _sm_outer_wall_base_1x3m _sm_outer_wall_base_1x4m _sm_outer_wall_base_windowed_1x4m "/Game/Modular_Asmospheric_Mansion/Meshes/Base/SM_outer_wall_base_1x05m.SM_outer_wall_base_1x05m" "/Game/Modular_Asmospheric_Mansion/Meshes/Base/SM_outer_wall_base_1x1m.SM_outer_wall_base_1x1m" "/Game/Modular_Asmospheric_Mansion/Meshes/Base/SM_outer_wall_base_1x2m.SM_outer_wall_base_1x2m" "/Game/Modular_Asmospheric_Mansion/Meshes/Base/SM_outer_wall_base_1x3m.SM_outer_wall_base_1x3m" "/Game/Modular_Asmospheric_Mansion/Meshes/Base/SM_outer_wall_base_1x4m.SM_outer_wall_base_1x4m" "/Game/Modular_Asmospheric_Mansion/Meshes/Base/SM_outer_wall_base_windowed_1x4m.SM_outer_wall_base_windowed_1x4m")
      (CallFunction|PaintattribFunc (Utilities|Array|MakeArray _sm_outer_wall_base_1x05m _sm_outer_wall_base_1x1m _sm_outer_wall_base_1x2m _sm_outer_wall_base_1x3m _sm_outer_wall_base_1x4m _sm_outer_wall_base_windowed_1x4m)))))

(fn SetMeshDimensionFunction
  (params (A :type Static%20Mesh%20Component%20Object%20Reference) (B :type Static%20Mesh%20Component%20Object%20Reference) (C :type Static%20Mesh%20Component%20Object%20Reference) (D :type Static%20Mesh%20Component%20Object%20Reference) (F :type Static%20Mesh%20Component%20Object%20Reference) (G :type Static%20Mesh%20Component%20Object%20Reference) (MESH%20A :type Static%20Mesh%20Object%20Reference) (MESH%20B :type Static%20Mesh%20Object%20Reference) (MESH%20C :type Static%20Mesh%20Object%20Reference) (MESH%20D :type Static%20Mesh%20Object%20Reference) (MESH%20F :type Static%20Mesh%20Object%20Reference) (MESH%20G :type Static%20Mesh%20Object%20Reference))
  (switch Utilities|FlowControl|Switch|SwitchonE_Base_Dimension (Variables|Default|GetDimensions)
    (:NewEnumerator0
      (Components|StaticMesh|SetStaticMesh A MESH%20A)
      (Rendering|SetVisibility A true false))
    (:NewEnumerator1
      (Components|StaticMesh|SetStaticMesh B MESH%20B)
      (Rendering|SetVisibility B true false))
    (:NewEnumerator2
      (Components|StaticMesh|SetStaticMesh C MESH%20C)
      (Rendering|SetVisibility C true false))
    (:NewEnumerator3
      (Components|StaticMesh|SetStaticMesh D MESH%20D)
      (Rendering|SetVisibility D true false))
    (:NewEnumerator4
      (Components|StaticMesh|SetStaticMesh F MESH%20F)
      (Rendering|SetVisibility F true false))
    (:NewEnumerator5
      (Components|StaticMesh|SetStaticMesh G MESH%20G)
      (Rendering|SetVisibility G true false)))
  (return))

(fn ChangeMatParameters
  (params (PaintColor_Change :type Linear%20Color%20Structure :default "(R=1.000000,G=1.000000,B=1.000000,A=1.000000)") (Paint%20Density :type Float%20%28single-precision%29) (Paint%20Contrast :type Float%20%28single-precision%29) (Desaturation :type Float%20%28single-precision%29) (Target :type Array%20of%20Mesh%20Component%20Object%20References))
  (Rendering|Material|SetScalarParameterValueonMaterials Target "Paint_Intensity" Paint%20Density)
  (Rendering|Material|SetVectorParameterValueonMaterials Target "PaintColor" (Math|Conversions|ToVector(LinearColor) PaintColor_Change))
  (Rendering|Material|SetScalarParameterValueonMaterials Target "Paint_Contrast" Paint%20Contrast)
  (Rendering|Material|SetScalarParameterValueonMaterials Target "Desaturation" Desaturation))

(fn PaintattribFunc
  (params ([0] :type Array%20of%20Mesh%20Component%20Object%20References))
  (if (Variables|PaintAttrib|GetPaint%20Active%20?)
    (CallFunction|ChangeMatParameters (Variables|PaintAttrib|GetPaint%20Color%20Change) (Variables|PaintAttrib|GetPaint%20Density) (Variables|PaintAttrib|GetPaint%20Contrast) (Variables|PaintAttrib|GetDesaturation) [0])))