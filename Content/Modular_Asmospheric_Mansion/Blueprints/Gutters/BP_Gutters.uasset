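; Modular gutter actor for the mansion kit, offering straight, left/right, corner and pipe pieces selected through GutterTypes.
; The construction script calls SetMeshFunction, which assigns the chosen static mesh to its dedicated component and makes it visible.
; BeginPlay runs FSetCollision on the root and its descendants.
; Helper functions set paint color, density, contrast and desaturation material parameters, but no graph here invokes PaintattribFunc.
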(event EventBeginPlay
  (CallFunction|FSetCollision (Variables|Default|GetDefaultSceneRoot) true))

(event Collision|EventActorBeginOverlap
  (params (OtherActor :type Actor%20Object%20Reference)))

(event EventTick
  (params (DeltaSeconds :type Float%20%28single-precision%29)))

(fn ConstructionScript
  (switch Utilities|FlowControl|Switch|SwitchonE_Gutters_Type (Variables|Default|GetGutterTypes)
    (:NewEnumerator2
      _)
    (:NewEnumerator0
      _)
    (:NewEnumerator1
      _)
    (:NewEnumerator3
      _)
    (:NewEnumerator7
      _)
    (:NewEnumerator9
      _)
    (:NewEnumerator8
      _)
    (:NewEnumerator4
      _)
    (:NewEnumerator5
      _)
    (:NewEnumerator6
      _)
    (:NewEnumerator10
      _)
    (:NewEnumerator12
      _)
    (:NewEnumerator11
      _)
    (:NewEnumerator13
      _)
    (:NewEnumerator14
      _)
    (:NewEnumerator15
      _)
    (:NewEnumerator16
      _)
    (:NewEnumerator17
      _)
    (:NewEnumerator18
      _))
  (CallFunction|SetMeshFunction (Variables|Default|GetSM_gutter_1m) (Variables|Default|GetSM_gutter_1_5m_L) (Variables|Default|GetSM_gutter_1_5m_R) (Variables|Default|GetSM_gutter_2m) (Variables|Default|GetSM_gutter_3m) (Variables|Default|GetSM_gutter_3m_L) (Variables|Default|GetSM_gutter_3m_R) (Variables|Default|GetSM_gutter_3_5m) (Variables|Default|GetSM_gutter_3_5m_L) (Variables|Default|GetSM_gutter_3_5m_R) (Variables|Default|GetSM_gutter_4m) (Variables|Default|GetSM_gutter_4m_L) (Variables|Default|GetSM_gutter_4m_R) (Variables|Default|GetSM_gutter_4_5m) (Variables|Default|GetSM_gutter_4_5m_L) (Variables|Default|GetSM_gutter_4_5m_R) (Variables|Default|GetSM_gutter_corner_5x5m) (Variables|Default|GetSM_gutter_pipe_3m) (Variables|Default|GetSM_gutter_pipe_6m) "/Game/Modular_Asmospheric_Mansion/Meshes/Gutters/SM_gutter_1m.SM_gutter_1m" "/Game/Modular_Asmospheric_Mansion/Meshes/Gutters/SM_gutter_1_5m_L.SM_gutter_1_5m_L" "/Game/Modular_Asmospheric_Mansion/Meshes/Gutters/SM_gutter_1_5m_R.SM_gutter_1_5m_R" "/Game/Modular_Asmospheric_Mansion/Meshes/Gutters/SM_gutter_2m.SM_gutter_2m" "/Game/Modular_Asmospheric_Mansion/Meshes/Gutters/SM_gutter_3m.SM_gutter_3m" "/Game/Modular_Asmospheric_Mansion/Meshes/Gutters/SM_gutter_3m_L.SM_gutter_3m_L" "/Game/Modular_Asmospheric_Mansion/Meshes/Gutters/SM_gutter_3m_R.SM_gutter_3m_R" "/Game/Modular_Asmospheric_Mansion/Meshes/Gutters/SM_gutter_3_5m.SM_gutter_3_5m" "/Game/Modular_Asmospheric_Mansion/Meshes/Gutters/SM_gutter_3_5m_L.SM_gutter_3_5m_L" "/Game/Modular_Asmospheric_Mansion/Meshes/Gutters/SM_gutter_3_5m_R.SM_gutter_3_5m_R" "/Game/Modular_Asmospheric_Mansion/Meshes/Gutters/SM_gutter_4m.SM_gutter_4m" "/Game/Modular_Asmospheric_Mansion/Meshes/Gutters/SM_gutter_4m_L.SM_gutter_4m_L" "/Game/Modular_Asmospheric_Mansion/Meshes/Gutters/SM_gutter_4m_R.SM_gutter_4m_R" "/Game/Modular_Asmospheric_Mansion/Meshes/Gutters/SM_gutter_4_5m.SM_gutter_4_5m" "/Game/Modular_Asmospheric_Mansion/Meshes/Gutters/SM_gutter_4_5m_L.SM_gutter_4_5m_L" "/Game/Modular_Asmospheric_Mansion/Meshes/Gutters/SM_gutter_4_5m_R.SM_gutter_4_5m_R" "/Game/Modular_Asmospheric_Mansion/Meshes/Gutters/SM_gutter_corner_5x5m.SM_gutter_corner_5x5m" "/Game/Modular_Asmospheric_Mansion/Meshes/Gutters/SM_gutter_pipe_3m.SM_gutter_pipe_3m" "/Game/Modular_Asmospheric_Mansion/Meshes/Gutters/SM_gutter_pipe_6m.SM_gutter_pipe_6m"))

(fn SetMeshFunction
  (params (1 :type Static%20Mesh%20Component%20Object%20Reference) (2 :type Static%20Mesh%20Component%20Object%20Reference) (3 :type Static%20Mesh%20Component%20Object%20Reference) (4 :type Static%20Mesh%20Component%20Object%20Reference) (5 :type Static%20Mesh%20Component%20Object%20Reference) (6 :type Static%20Mesh%20Component%20Object%20Reference) (7 :type Static%20Mesh%20Component%20Object%20Reference) (8 :type Static%20Mesh%20Component%20Object%20Reference) (9 :type Static%20Mesh%20Component%20Object%20Reference) (10 :type Static%20Mesh%20Component%20Object%20Reference) (11 :type Static%20Mesh%20Component%20Object%20Reference) (12 :type Static%20Mesh%20Component%20Object%20Reference) (13 :type Static%20Mesh%20Component%20Object%20Reference) (14 :type Static%20Mesh%20Component%20Object%20Reference) (15 :type Static%20Mesh%20Component%20Object%20Reference) (16 :type Static%20Mesh%20Component%20Object%20Reference) (17 :type Static%20Mesh%20Component%20Object%20Reference) (18 :type Static%20Mesh%20Component%20Object%20Reference) (19 :type Static%20Mesh%20Component%20Object%20Reference) (MESH%201 :type Static%20Mesh%20Object%20Reference) (MESH%202 :type Static%20Mesh%20Object%20Reference) (MESH%203 :type Static%20Mesh%20Object%20Reference) (MESH%204 :type Static%20Mesh%20Object%20Reference) (MESH%205 :type Static%20Mesh%20Object%20Reference) (MESH%206 :type Static%20Mesh%20Object%20Reference) (MESH%207 :type Static%20Mesh%20Object%20Reference) (MESH%208 :type Static%20Mesh%20Object%20Reference) (MESH%209 :type Static%20Mesh%20Object%20Reference) (MESH%2010 :type Static%20Mesh%20Object%20Reference) (MESH%2011 :type Static%20Mesh%20Object%20Reference) (MESH%2012 :type Static%20Mesh%20Object%20Reference) (MESH%2013 :type Static%20Mesh%20Object%20Reference) (MESH%2014 :type Static%20Mesh%20Object%20Reference) (MESH%2015 :type Static%20Mesh%20Object%20Reference) (MESH%2016 :type Static%20Mesh%20Object%20Reference) (MESH%2017 :type Static%20Mesh%20Object%20Reference) (MESH%2018 :type Static%20Mesh%20Object%20Reference) (MESH%2019 :type Static%20Mesh%20Object%20Reference))
  (switch Utilities|FlowControl|Switch|SwitchonE_Gutters_Type (Variables|Default|GetGutterTypes)
    (:NewEnumerator2
      (Components|StaticMesh|SetStaticMesh 1 MESH%201)
      (Rendering|SetVisibility 1 true false)
      (return))
    (:NewEnumerator0
      (Components|StaticMesh|SetStaticMesh 2 MESH%202)
      (Rendering|SetVisibility 2 true false)
      (return))
    (:NewEnumerator1
      (Components|StaticMesh|SetStaticMesh 3 MESH%203)
      (Rendering|SetVisibility 3 true false)
      (return))
    (:NewEnumerator3
      (Components|StaticMesh|SetStaticMesh 4 MESH%204)
      (Rendering|SetVisibility 4 true false)
      (return))
    (:NewEnumerator7
      (Components|StaticMesh|SetStaticMesh 5 MESH%205)
      (Rendering|SetVisibility 5 true false)
      (return))
    (:NewEnumerator9
      (Components|StaticMesh|SetStaticMesh 6 MESH%206)
      (Rendering|SetVisibility 6 true false)
      (return))
    (:NewEnumerator8
      (Components|StaticMesh|SetStaticMesh 7 MESH%207)
      (Rendering|SetVisibility 7 true false)
      (return))
    (:NewEnumerator4
      (Components|StaticMesh|SetStaticMesh 8 MESH%208)
      (Rendering|SetVisibility 8 true false))
    (:NewEnumerator5
      (Components|StaticMesh|SetStaticMesh 9 MESH%209)
      (Rendering|SetVisibility 9 true false))
    (:NewEnumerator6
      (Components|StaticMesh|SetStaticMesh 10 MESH%2010)
      (Rendering|SetVisibility 10 true false))
    (:NewEnumerator10
      (Components|StaticMesh|SetStaticMesh 11 MESH%2011)
      (Rendering|SetVisibility 11 true false))
    (:NewEnumerator12
      (Components|StaticMesh|SetStaticMesh 12 MESH%2012)
      (Rendering|SetVisibility 12 true false))
    (:NewEnumerator11
      (Components|StaticMesh|SetStaticMesh 13 MESH%2013)
      (Rendering|SetVisibility 13 true false))
    (:NewEnumerator13
      (Components|StaticMesh|SetStaticMesh 14 MESH%2014)
      (Rendering|SetVisibility 14 true false))
    (:NewEnumerator14
      (Components|StaticMesh|SetStaticMesh 15 MESH%2015)
      (Rendering|SetVisibility 15 true false))
    (:NewEnumerator15
      (Components|StaticMesh|SetStaticMesh 16 MESH%2016)
      (Rendering|SetVisibility 16 true false))
    (:NewEnumerator16
      (Components|StaticMesh|SetStaticMesh 17 MESH%2017)
      (Rendering|SetVisibility 17 true false))
    (:NewEnumerator17
      (Components|StaticMesh|SetStaticMesh 18 MESH%2018)
      (Rendering|SetVisibility 18 true false))
    (:NewEnumerator18
      (Components|StaticMesh|SetStaticMesh 19 MESH%2019)
      (Rendering|SetVisibility 19 true false))))

(fn ChangeMatParameters
  (params (PaintColor_Change :type Linear%20Color%20Structure :default "(R=1.000000,G=1.000000,B=1.000000,A=1.000000)") (Paint%20Density :type Float%20%28single-precision%29) (Paint%20Contrast :type Float%20%28single-precision%29) (Desaturation :type Float%20%28single-precision%29) (Target :type Array%20of%20Mesh%20Component%20Object%20References))
  (Rendering|Material|SetScalarParameterValueonMaterials Target "Paint_Intensity" Paint%20Density)
  (Rendering|Material|SetVectorParameterValueonMaterials Target "PaintColor" (Math|Conversions|ToVector(LinearColor) PaintColor_Change))
  (Rendering|Material|SetScalarParameterValueonMaterials Target "Paint_Contrast" Paint%20Contrast)
  (Rendering|Material|SetScalarParameterValueonMaterials Target "Desaturation" Desaturation))

(fn PaintattribFunc
  (params ([0] :type Array%20of%20Mesh%20Component%20Object%20References))
  (if true
    (CallFunction|ChangeMatParameters "(R=1.000000,G=1.000000,B=1.000000,A=1.000000)" 0.0 0.0 0.0 [0])))