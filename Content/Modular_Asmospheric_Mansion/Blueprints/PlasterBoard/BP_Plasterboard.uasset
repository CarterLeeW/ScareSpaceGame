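; BP_Plasterboard is a configurable modular plasterboard piece, offered in several lengths or as a corner.
; The construction script either shows the corner mesh or uses the PlankTypes enum to assign and reveal the matching length mesh.
; For straight pieces, an optional paint pass pushes color, intensity, contrast and desaturation parameters to the mesh materials.
; BeginPlay calls FSetCollision on the root and all its descendants.
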(event EventBeginPlay
  (CallFunction|FSetCollision (Variables|Default|GetDefaultSceneRoot) true))

(event Collision|EventActorBeginOverlap
  (params (OtherActor :type Actor%20Object%20Reference)))

(event EventTick
  (params (DeltaSeconds :type Float%20%28single-precision%29)))

(fn ConstructionScript
  (bind _sm_plasterboard_05m (Variables|Default|GetSM_plasterboard_05m))
  (bind _sm_plasterboard_1m (Variables|Default|GetSM_plasterboard_1m))
  (bind _sm_plasterboard_2m (Variables|Default|GetSM_plasterboard_2m))
  (bind _sm_plasterboard_3m (Variables|Default|GetSM_plasterboard_3m))
  (bind _sm_plasterboard_4m (Variables|Default|GetSM_plasterboard_4m))
  (bind _sm_plasterboard_6m (Variables|Default|GetSM_plasterboard_6m))
  (bind _sm_plasterboard_corner (Variables|Default|GetSM_plasterboard_corner))
  (if (Variables|1-PlasterBoardsDimensions|GetPlasterBoard%20Corner%20?)
    (Components|StaticMesh|SetStaticMesh _sm_plasterboard_corner "/Game/Modular_Asmospheric_Mansion/Meshes/Plasterboard/SM_plasterboard_corner.SM_plasterboard_corner")
    (Rendering|SetVisibility _sm_plasterboard_corner true false)
    (else
      (switch Utilities|FlowControl|Switch|SwitchonE_Plasterboard_Dimensions (Variables|1-PlasterBoardsDimensions|GetPlankTypes)
        (:NewEnumerator0
          _)
        (:NewEnumerator1
          _)
        (:NewEnumerator2
          _)
        (:NewEnumerator3
          _)
        (:NewEnumerator4
          _)
        (:NewEnumerator5
          _)
        (:NewEnumerator6
          _))
      (CallFunction|SetMeshFunction _sm_plasterboard_05m _sm_plasterboard_1m _sm_plasterboard_2m _sm_plasterboard_3m _sm_plasterboard_4m _sm_plasterboard_6m "/Game/Modular_Asmospheric_Mansion/Meshes/Plasterboard/SM_plasterboard_05m.SM_plasterboard_05m" "/Game/Modular_Asmospheric_Mansion/Meshes/Plasterboard/SM_plasterboard_1m.SM_plasterboard_1m" "/Game/Modular_Asmospheric_Mansion/Meshes/Plasterboard/SM_plasterboard_2m.SM_plasterboard_2m" "/Game/Modular_Asmospheric_Mansion/Meshes/Plasterboard/SM_plasterboard_3m.SM_plasterboard_3m" "/Game/Modular_Asmospheric_Mansion/Meshes/Plasterboard/SM_plasterboard_4m.SM_plasterboard_4m" "/Game/Modular_Asmospheric_Mansion/Meshes/Plasterboard/SM_plasterboard_6m.SM_plasterboard_6m")
      (CallFunction|PaintattribFunc (Utilities|Array|MakeArray _sm_plasterboard_05m _sm_plasterboard_1m _sm_plasterboard_2m _sm_plasterboard_3m _sm_plasterboard_4m _sm_plasterboard_6m)))))

(fn SetMeshFunction
  (params (1 :type Static%20Mesh%20Component%20Object%20Reference) (2 :type Static%20Mesh%20Component%20Object%20Reference) (3 :type Static%20Mesh%20Component%20Object%20Reference) (4 :type Static%20Mesh%20Component%20Object%20Reference) (5 :type Static%20Mesh%20Component%20Object%20Reference) (6 :type Static%20Mesh%20Component%20Object%20Reference) (MESH%201 :type Static%20Mesh%20Object%20Reference) (MESH%202 :type Static%20Mesh%20Object%20Reference) (MESH%203 :type Static%20Mesh%20Object%20Reference) (MESH%204 :type Static%20Mesh%20Object%20Reference) (MESH%205 :type Static%20Mesh%20Object%20Reference) (MESH%206 :type Static%20Mesh%20Object%20Reference))
  (switch Utilities|FlowControl|Switch|SwitchonE_Plasterboard_Dimensions (Variables|1-PlasterBoardsDimensions|GetPlankTypes)
    (:NewEnumerator0
      (Components|StaticMesh|SetStaticMesh 1 MESH%201)
      (Rendering|SetVisibility 1 true false))
    (:NewEnumerator1
      (Components|StaticMesh|SetStaticMesh 2 MESH%202)
      (Rendering|SetVisibility 2 true false))
    (:NewEnumerator2
      (Components|StaticMesh|SetStaticMesh 3 MESH%203)
      (Rendering|SetVisibility 3 true false))
    (:NewEnumerator3
      (Components|StaticMesh|SetStaticMesh 4 MESH%204)
      (Rendering|SetVisibility 4 true false))
    (:NewEnumerator4
      (Components|StaticMesh|SetStaticMesh 5 MESH%205)
      (Rendering|SetVisibility 5 true false))
    (:NewEnumerator5
      (Components|StaticMesh|SetStaticMesh 6 MESH%206)
      (Rendering|SetVisibility 6 true false)))
  (return))

(fn ChangeMatParameters
  (params (PaintColor_Change :type Linear%20Color%20Structure :default "(R=1.000000,G=1.000000,B=1.000000,A=1.000000)") (Paint%20Density :type Float%20%28single-precision%29) (Paint%20Contrast :type Float%20%28single-precision%29) (Desaturation :type Float%20%28single-precision%29) (Target :type Array%20of%20Mesh%20Component%20Object%20References))
  (Rendering|Material|SetScalarParameterValueonMaterials Target "Paint_Intensity" Paint%20Density)
  (Rendering|Material|SetVectorParameterValueonMaterials Target "PaintColor" (Math|Conversions|ToVector(LinearColor) PaintColor_Change))
  (Rendering|Material|SetScalarParameterValueonMaterials Target "Paint_Contrast" Paint%20Contrast)
  (Rendering|Material|SetScalarParameterValueonMaterials Target "Desaturation" Desaturation))

(fn PaintattribFunc
  (params ([0] :type Array%20of%20Mesh%20Component%20Object%20References))
  (if (Variables|2-PaintAttrib|GetPaint%20Active%20?)
    (CallFunction|ChangeMatParameters (Variables|2-PaintAttrib|GetPaint%20Color%20Change) (Variables|2-PaintAttrib|GetPaint%20Density) (Variables|2-PaintAttrib|GetPaint%20Contrast) (Variables|2-PaintAttrib|GetDesaturation) [0])))