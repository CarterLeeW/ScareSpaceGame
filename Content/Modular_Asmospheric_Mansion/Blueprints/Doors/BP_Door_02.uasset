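; BP_Door_02 is a configurable door and frame prop for the modular mansion, with no interactive opening logic.
; The construction script optionally yaws the door to a set open angle and applies an enum-selected material to both meshes.
; ChangeMat then pushes paint color, intensity, contrast and desaturation into material parameters for per-instance variation.
; BeginPlay calls FSetCollision on the root and all descendants.
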(event EventBeginPlay
  (CallFunction|FSetCollision (Variables|Default|GetDefaultSceneRoot) true))

(event Collision|EventActorBeginOverlap
  (params (OtherActor :type Actor%20Object%20Reference)))

(event EventTick
  (params (DeltaSeconds :type Float%20%28single-precision%29)))

(fn ConstructionScript
  (bind _sm_door_frame_01 (Variables|Default|GetSM_door_frame_01))
  (Utilities|FlowControl|Sequence
    (:then_0
      (if (Variables|Default|GetDoor%20Open%20?)
        (Transformation|SetRelativeRotation (Variables|Default|GetSM_door_02) (Math|Rotator|MakeRotator 0.0 0.0 (* (Variables|Default|GetDoor%20A%20Open%20Angle) 1.0)) false false)))
    (:then_1
      (switch Utilities|FlowControl|Switch|SwitchonE_Door_Mat (Variables|Default|GetE_Door_Mat_Types)
        (:NewEnumerator0
          (Rendering|Material|SetMaterial _sm_door_frame_01 0 "/Game/Modular_Asmospheric_Mansion/Materials/Instance/MI_Dark_Wooden_Planks.MI_Dark_Wooden_Planks"))
        (:NewEnumerator1
          (Rendering|Material|SetMaterial _sm_door_frame_01 0 "/Game/Modular_Asmospheric_Mansion/Materials/Instance/MI_weathered_brown_planks.MI_weathered_brown_planks"))
        (:NewEnumerator2
          (Rendering|Material|SetMaterial _sm_door_frame_01 0 "/Game/Modular_Asmospheric_Mansion/Materials/Instance/Alternatives/MI_Outer_Wall_Tile_04.MI_Outer_Wall_Tile_04"))
        (:NewEnumerator3
          (Rendering|Material|SetMaterial _sm_door_frame_01 0 "/Game/Modular_Asmospheric_Mansion/Materials/Instance/Alternatives/MI_Outer_Wall_Tile_03.MI_Outer_Wall_Tile_03"))
        (:NewEnumerator4
          (Rendering|Material|SetMaterial (Variables|Default|GetSM_door_02) 0 "/Game/Modular_Asmospheric_Mansion/Materials/Instance/Alternatives/MI_Outer_Wall_Tile_02.MI_Outer_Wall_Tile_02"))))
    (:then_2
      ;[0 0 0 1 30] MaterialEdit
      (CallFunction|ChangeMat (Variables|MATERIALEDIT|GetPaint%20Color%20Change) (Variables|MATERIALEDIT|GetPaint%20Density) (Variables|MATERIALEDIT|GetPaint%20Contrast) (Variables|MATERIALEDIT|GetDesaturation) (Utilities|Array|MakeArray (Variables|Default|GetSM_door_02) (Variables|Default|GetSM_door_frame_01))))))

(fn ChangeMat
  (params (PaintColor_Change :type Linear%20Color%20Structure :default "(R=1.000000,G=1.000000,B=1.000000,A=1.000000)") (Paint%20Density :type Float%20%28single-precision%29) (Paint%20Contrast :type Float%20%28single-precision%29) (Desaturation :type Float%20%28single-precision%29) (Target :type Array%20of%20Mesh%20Component%20Object%20References))
  (Rendering|Material|SetScalarParameterValueonMaterials Target "Paint_Intensity" Paint%20Density)
  (Rendering|Material|SetVectorParameterValueonMaterials Target "PaintColor" (Math|Conversions|ToVector(LinearColor) PaintColor_Change))
  (Rendering|Material|SetScalarParameterValueonMaterials Target "Paint_Contrast" Paint%20Contrast)
  (Rendering|Material|SetScalarParameterValueonMaterials Target "Desaturation" Desaturation))