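; Modular mansion wall actor that builds one configurable wall piece in its construction script from size, wall type and A/B/C style.
; Enums select and reveal pre-placed inner mesh components, plus an optional outer wall; unsupported type/size combinations show the Empty component.
; Helper functions swap two inner material slots, set the outer material and optionally push paint and desaturation parameters.
; BeginPlay calls FSetCollision on the root and its descendants.
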(event EventBeginPlay
  (CallFunction|FSetCollision (Variables|Default|GetDefaultSceneRoot) true))

(event Collision|EventActorBeginOverlap
  (params (OtherActor :type Actor%20Object%20Reference)))

(event EventTick
  (params (DeltaSeconds :type Float%20%28single-precision%29)))

(fn ConstructionScript
  (bind _sm_outer_wall_door_3x3m (Variables|Default|GetSM_outer_wall_door_3x3m))
  (bind _sm_inner_wall_doubledoor_3x4m_a (Variables|Default|GetSM_inner_wall_doubledoor_3x4m_A))
  (bind _sm_inner_wall_3x2m_a (Variables|Default|GetSM_inner_wall_3x2m_A))
  (bind _sm_inner_wall_3x2m_c (Variables|Default|GetSM_inner_wall_3x2m_C))
  (bind _sm_outer_wall_wide_window_3x4m (Variables|Default|GetSM_outer_wall_wide_window_3x4m))
  (bind _sm_outer_wall_doubledoor_3x4m (Variables|Default|GetSM_outer_wall_doubledoor_3x4m))
  (bind _sm_outer_wall_door_3x3m_2 (Variables|Default|GetSM_outer_wall_door_3x3m))
  (bind _sm_outer_wall_windowed_3x3m (Variables|Default|GetSM_outer_wall_windowed_3x3m))
  (bind _sm_outer_wall_window_3x4m (Variables|Default|GetSM_outer_wall_window_3x4m))
  (bind _sm_outer_wall_singledoor_3x4m (Variables|Default|GetSM_outer_wall_singledoor_3x4m))
  (bind _sm_outer_wall_3x4m (Variables|Default|GetSM_outer_wall_3x4m))
  (bind _sm_outer_wall_3x0_5m (Variables|Default|GetSM_Outer_Wall_3x0_5m))
  (bind _sm_outer_wall_3x1m (Variables|Default|GetSM_outer_wall_3x1m))
  (bind _sm_outer_wall_3x2m (Variables|Default|GetSM_outer_wall_3x2m))
  (bind _sm_outer_wall_window_3x2m (Variables|Default|GetSM_outer_wall_window_3x2m))
  (bind _sm_outer_wall_widewindow_3x6m (Variables|Default|GetSM_outer_wall_widewindow_3x6m))
  (bind _sm_inner_wall_doubledoor_3x4m_b (Variables|Default|GetSM_inner_wall_doubledoor_3x4m_B))
  (bind _sm_inner_wall_doubledoor_3x4m_c (Variables|Default|GetSM_inner_wall_doubledoor_3x4m_C))
  (bind _sm_inner_wall_windowed_3x3m_b (Variables|Default|GetSM_inner_wall_windowed_3x3m_B))
  (bind _sm_inner_wall_windowed_3x3m_c (Variables|Default|GetSM_inner_wall_windowed_3x3m_C))
  (bind _sm_outer_wall_3x4m_2 (Variables|Default|GetSM_outer_wall_3x4m))
  (bind _sm_outer_wall_3x4m_3 (Variables|Default|GetSM_outer_wall_3x4m))
  (bind _sm_outer_wall_window_3x4m_2 (Variables|Default|GetSM_outer_wall_window_3x4m))
  (bind _sm_outer_wall_windowed_3x3m_2 (Variables|Default|GetSM_outer_wall_windowed_3x3m))
  (bind _sm_inner_wall_door_3x4m_c (Variables|Default|GetSM_inner_wall_door_3x4m_C))
  (bind _sm_outer_wall_singledoor_3x4m_2 (Variables|Default|GetSM_outer_wall_singledoor_3x4m))
  (bind _sm_outer_wall_wide_window_3x4m_2 (Variables|Default|GetSM_outer_wall_wide_window_3x4m))
  (bind _sm_inner_wall_wide_window_3x4m_a (Variables|Default|GetSM_inner_wall_wide_window_3x4m_A))
  (bind _sm_inner_wall_wide_window_3x4m_b (Variables|Default|GetSM_inner_wall_wide_window_3x4m_B))
  (bind _sm_inner_wall_wide_window_3x4m_c (Variables|Default|GetSM_inner_wall_wide_window_3x4m_C))
  (bind _sm_outer_wall_3x0_5m_2 (Variables|Default|GetSM_Outer_Wall_3x0_5m))
  (bind _sm_outer_wall_3x1m_2 (Variables|Default|GetSM_outer_wall_3x1m))
  (bind _sm_outer_wall_3x2m_2 (Variables|Default|GetSM_outer_wall_3x2m))
  (bind _sm_inner_wall_3x0_5m_b (Variables|Default|GetSM_inner_wall_3x0_5m_B))
  (bind _sm_outer_wall_window_3x2m_2 (Variables|Default|GetSM_outer_wall_window_3x2m))
  (bind _sm_inner_wall_window_3x2m_a (Variables|Default|GetSM_inner_wall_window_3x2m_A))
  (bind _sm_inner_wall_3x3m_a (Variables|Default|GetSM_inner_wall_3x3m_A))
  (bind _sm_inner_wall_window_3x2m_b (Variables|Default|GetSM_inner_wall_window_3x2m_B))
  (bind _sm_inner_wall_window_3x2m_c (Variables|Default|GetSM_inner_wall_window_3x2m_C))
  (bind _sm_inner_wall_widewindow_3x6m_a (Variables|Default|GetSM_inner_wall_widewindow_3x6m_A))
  (bind _sm_inner_wall_3x0_5m_c (Variables|Default|GetSM_inner_wall_3x0_5m_C))
  (bind _sm_inner_wall_widewindow_3x6m_b (Variables|Default|GetSM_inner_wall_widewindow_3x6m_B))
  (bind _sm_inner_wall_widewindow_3x6m_c (Variables|Default|GetSM_inner_wall_widewindow_3x6m_C))
  (bind _sm_outer_wall_widewindow_3x6m_2 (Variables|Default|GetSM_outer_wall_widewindow_3x6m))
  (bind _sm_inner_wall_3x4m_a (Variables|Default|GetSM_inner_wall_3x4m_A))
  (bind _sm_inner_wall_3x3m_b (Variables|Default|GetSM_inner_wall_3x3m_B))
  (bind _sm_inner_wall_3x1m_a (Variables|Default|GetSM_inner_wall_3x1m_A))
  (bind _sm_inner_wall_windowed_3x3m_a (Variables|Default|GetSM_inner_wall_windowed_3x3m_A))
  (bind _sm_inner_wall_3x3m_c (Variables|Default|GetSM_inner_wall_3x3m_C))
  (bind _sm_inner_wall_3x1m_b (Variables|Default|GetSM_inner_wall_3x1m_B))
  (bind _sm_inner_wall_3x1m_c (Variables|Default|GetSM_inner_wall_3x1m_C))
  (bind _sm_inner_wall_3x4m_b (Variables|Default|GetSM_inner_wall_3x4m_B))
  (bind _sm_inner_wall_3x0_5m_a (Variables|Default|GetSM_inner_wall_3x0_5m_A))
  (bind _sm_inner_wall_3x4m_c (Variables|Default|GetSM_inner_wall_3x4m_C))
  (bind _sm_inner_wall_door_3x4m_a (Variables|Default|GetSM_inner_wall_door_3x4m_A))
  (bind _sm_inner_wall_window_3x4m_a (Variables|Default|GetSM_inner_wall_window_3x4m_A))
  (bind _sm_inner_wall_window_3x4m_b (Variables|Default|GetSM_inner_wall_window_3x4m_B))
  (bind _sm_outer_wall_doubledoor_3x4m_2 (Variables|Default|GetSM_outer_wall_doubledoor_3x4m))
  (bind _sm_inner_wall_door_3x3m_a (Variables|Default|GetSM_inner_wall_door_3x3m_A))
  (bind _sm_inner_wall_door_3x3m_b (Variables|Default|GetSM_inner_wall_door_3x3m_B))
  (bind _sm_inner_wall_3x2m_b (Variables|Default|GetSM_inner_wall_3x2m_B))
  (bind _sm_inner_wall_door_3x4m_b (Variables|Default|GetSM_inner_wall_door_3x4m_B))
  (bind _sm_inner_wall_window_3x4m_c (Variables|Default|GetSM_inner_wall_window_3x4m_C))
  (Utilities|FlowControl|Sequence
    (:then_0
      (switch Utilities|FlowControl|Switch|SwitchonE_Wall_Dimension (Variables|INNERWALLS|GetE_Wall%20Dimension)
        (:NewEnumerator0
          ;[0 0 0] 3X05
          (CallFunction|SetMeshFunction _sm_inner_wall_3x0_5m_a _sm_inner_wall_3x0_5m_b _sm_inner_wall_3x0_5m_c "/Game/Modular_Asmospheric_Mansion/Meshes/Walls/SM_inner_wall_3x0_5m_A.SM_inner_wall_3x0_5m_A" "/Game/Modular_Asmospheric_Mansion/Meshes/Walls/SM_inner_wall_3x0_5m_B.SM_inner_wall_3x0_5m_B" "/Game/Modular_Asmospheric_Mansion/Meshes/Walls/SM_inner_wall_3x0_5m_C.SM_inner_wall_3x0_5m_C")
          (if (Variables|Default|GetADD%20OUTER%20WALL%20?)
            (Components|StaticMesh|SetStaticMesh _sm_outer_wall_3x0_5m_2 "/Game/Modular_Asmospheric_Mansion/Meshes/Walls/SM_Outer_Wall_3x0_5m.SM_Outer_Wall_3x0_5m")
            (Rendering|SetVisibility _sm_outer_wall_3x0_5m_2 true false))
          (CallFunction|MasterChangeMat _sm_inner_wall_3x0_5m_a _sm_inner_wall_3x0_5m_b _sm_inner_wall_3x0_5m_c _sm_inner_wall_3x0_5m_a _sm_inner_wall_3x0_5m_b _sm_inner_wall_3x0_5m_c)
          (CallFunction|PaintattribFunc _sm_inner_wall_3x0_5m_a _sm_inner_wall_3x0_5m_b _sm_inner_wall_3x0_5m_c))
        (:NewEnumerator1
          ;[0 0 0] 3X1
          (CallFunction|SetMeshFunction _sm_inner_wall_3x1m_a _sm_inner_wall_3x1m_b _sm_inner_wall_3x1m_c "/Game/Modular_Asmospheric_Mansion/Meshes/Walls/SM_inner_wall_3x1m_A.SM_inner_wall_3x1m_A" "/Game/Modular_Asmospheric_Mansion/Meshes/Walls/SM_inner_wall_3x1m_B.SM_inner_wall_3x1m_B" "/Game/Modular_Asmospheric_Mansion/Meshes/Walls/SM_inner_wall_3x1m_C.SM_inner_wall_3x1m_C")
          (if (Variables|Default|GetADD%20OUTER%20WALL%20?)
            (Components|StaticMesh|SetStaticMesh _sm_outer_wall_3x1m_2 "/Game/Modular_Asmospheric_Mansion/Meshes/Walls/SM_outer_wall_3x1m.SM_outer_wall_3x1m")
            (Rendering|SetVisibility _sm_outer_wall_3x1m_2 true false))
          (CallFunction|MasterChangeMat _sm_inner_wall_3x1m_a _sm_inner_wall_3x1m_b _sm_inner_wall_3x1m_c _sm_inner_wall_3x1m_a _sm_inner_wall_3x1m_b _sm_inner_wall_3x1m_c)
          (CallFunction|PaintattribFunc _sm_inner_wall_3x1m_a _sm_inner_wall_3x1m_b _sm_inner_wall_3x1m_c))
        (:NewEnumerator2
          ;[0 0 0] 3x2
          (switch Utilities|FlowControl|Switch|SwitchonE_WallTypes (Variables|WallTypes|GetE_Wall%20Types)
            (:NewEnumerator0
              (CallFunction|SetMeshFunction _sm_inner_wall_3x2m_a _sm_inner_wall_3x2m_b _sm_inner_wall_3x2m_c "/Game/Modular_Asmospheric_Mansion/Meshes/Walls/SM_inner_wall_3x2m_A.SM_inner_wall_3x2m_A" "/Game/Modular_Asmospheric_Mansion/Meshes/Walls/SM_inner_wall_3x2m_B.SM_inner_wall_3x2m_B" "/Game/Modular_Asmospheric_Mansion/Meshes/Walls/SM_inner_wall_3x2m_C.SM_inner_wall_3x2m_C")
              (if (Variables|Default|GetADD%20OUTER%20WALL%20?)
                (Components|StaticMesh|SetStaticMesh _sm_outer_wall_3x2m_2 "/Game/Modular_Asmospheric_Mansion/Meshes/Walls/SM_outer_wall_3x2m.SM_outer_wall_3x2m")
                (Rendering|SetVisibility _sm_outer_wall_3x2m_2 true false))
              (CallFunction|MasterChangeMat _sm_inner_wall_3x2m_a _sm_inner_wall_3x2m_b _sm_inner_wall_3x2m_c _sm_inner_wall_3x2m_a _sm_inner_wall_3x2m_b _sm_inner_wall_3x2m_c)
              (CallFunction|PaintattribFunc _sm_inner_wall_3x2m_a _sm_inner_wall_3x2m_b _sm_inner_wall_3x2m_c))
            (:NewEnumerator1
              (CallFunction|SetMeshFunction _sm_inner_wall_window_3x2m_a _sm_inner_wall_window_3x2m_b _sm_inner_wall_window_3x2m_c "/Game/Modular_Asmospheric_Mansion/Meshes/Walls/SM_inner_wall_window_3x2m_A.SM_inner_wall_window_3x2m_A" "/Game/Modular_Asmospheric_Mansion/Meshes/Walls/SM_inner_wall_window_3x2m_B.SM_inner_wall_window_3x2m_B" "/Game/Modular_Asmospheric_Mansion/Meshes/Walls/SM_inner_wall_window_3x2m_C.SM_inner_wall_window_3x2m_C")
              (if (Variables|Default|GetADD%20OUTER%20WALL%20?)
                (Components|StaticMesh|SetStaticMesh _sm_outer_wall_window_3x2m_2 "/Game/Modular_Asmospheric_Mansion/Meshes/Walls/SM_outer_wall_window_3x2m.SM_outer_wall_window_3x2m")
                (Rendering|SetVisibility _sm_outer_wall_window_3x2m_2 true false))
              (CallFunction|MasterChangeMat _sm_inner_wall_window_3x2m_a _sm_inner_wall_window_3x2m_b _sm_inner_wall_window_3x2m_c _sm_inner_wall_window_3x2m_a _sm_inner_wall_window_3x2m_b _sm_inner_wall_window_3x2m_c)
              (CallFunction|PaintattribFunc _sm_inner_wall_window_3x2m_a _sm_inner_wall_window_3x2m_b _sm_inner_wall_window_3x2m_c))
            (:NewEnumerator3
              ;[1 0 0] NO STYLE !
              (Rendering|SetVisibility (Variables|Default|GetEmpty) true false :!label _label))
            (:NewEnumerator5
              (goto _label))
            (:NewEnumerator6
              (goto _label))))
        (:NewEnumerator3
          ;[0 0 0] 3x3
          (switch Utilities|FlowControl|Switch|SwitchonE_WallTypes (Variables|WallTypes|GetE_Wall%20Types)
            (:NewEnumerator0
              (CallFunction|SetMeshFunction _sm_inner_wall_3x3m_a _sm_inner_wall_3x3m_b _sm_inner_wall_3x3m_c "/Game/Modular_Asmospheric_Mansion/Meshes/Walls/SM_inner_wall_3x3m_A.SM_inner_wall_3x3m_A" "/Game/Modular_Asmospheric_Mansion/Meshes/Walls/SM_inner_wall_3x3m_B.SM_inner_wall_3x3m_B" "/Game/Modular_Asmospheric_Mansion/Meshes/Walls/SM_inner_wall_3x3m_C.SM_inner_wall_3x3m_C")
              (if (Variables|Default|GetADD%20OUTER%20WALL%20?)
                (Components|StaticMesh|SetStaticMesh _sm_outer_wall_3x4m_2 "/Game/Modular_Asmospheric_Mansion/Meshes/Walls/SM_outer_wall_3x3m.SM_outer_wall_3x3m")
                (Rendering|SetVisibility _sm_outer_wall_3x4m_2 true false))
              (CallFunction|MasterChangeMat _sm_inner_wall_3x3m_a _sm_inner_wall_3x3m_b _sm_inner_wall_3x3m_c _sm_inner_wall_3x3m_a _sm_inner_wall_3x3m_b _sm_inner_wall_3x3m_c)
              (CallFunction|PaintattribFunc _sm_inner_wall_3x3m_a _sm_inner_wall_3x3m_b _sm_inner_wall_3x3m_c))
            (:NewEnumerator1
              (CallFunction|SetMeshFunction _sm_inner_wall_windowed_3x3m_a _sm_inner_wall_windowed_3x3m_b _sm_inner_wall_windowed_3x3m_c "/Game/Modular_Asmospheric_Mansion/Meshes/Walls/SM_inner_wall_windowed_3x3m_A.SM_inner_wall_windowed_3x3m_A" "/Game/Modular_Asmospheric_Mansion/Meshes/Walls/SM_inner_wall_windowed_3x3m_B.SM_inner_wall_windowed_3x3m_B" "/Game/Modular_Asmospheric_Mansion/Meshes/Walls/SM_inner_wall_windowed_3x3m_C.SM_inner_wall_windowed_3x3m_C")
              (if (Variables|Default|GetADD%20OUTER%20WALL%20?)
                (Components|StaticMesh|SetStaticMesh _sm_outer_wall_windowed_3x3m_2 "/Game/Modular_Asmospheric_Mansion/Meshes/Walls/SM_outer_wall_windowed_3x3m.SM_outer_wall_windowed_3x3m")
                (Rendering|SetVisibility _sm_outer_wall_windowed_3x3m_2 true false))
              (CallFunction|MasterChangeMat _sm_inner_wall_windowed_3x3m_a _sm_inner_wall_windowed_3x3m_b _sm_inner_wall_windowed_3x3m_c _sm_inner_wall_windowed_3x3m_a _sm_inner_wall_windowed_3x3m_b _sm_inner_wall_windowed_3x3m_c)
              (CallFunction|PaintattribFunc _sm_inner_wall_windowed_3x3m_a _sm_inner_wall_windowed_3x3m_b _sm_inner_wall_windowed_3x3m_c))
            (:NewEnumerator3
              (goto _label))
            (:NewEnumerator5
              (CallFunction|SetMeshFunction _sm_inner_wall_door_3x3m_a _sm_inner_wall_door_3x3m_b (Variables|Default|GetSM_inner_wall_door_3x3m_C) "/Game/Modular_Asmospheric_Mansion/Meshes/Walls/SM_inner_wall_door_3x3m_A.SM_inner_wall_door_3x3m_A" "/Game/Modular_Asmospheric_Mansion/Meshes/Walls/SM_inner_wall_door_3x3m_B.SM_inner_wall_door_3x3m_B" "/Game/Modular_Asmospheric_Mansion/Meshes/Walls/SM_inner_wall_door_3x3m_C.SM_inner_wall_door_3x3m_C")
              (if (Variables|Default|GetADD%20OUTER%20WALL%20?)
                (Components|StaticMesh|SetStaticMesh _sm_outer_wall_door_3x3m "/Game/Modular_Asmospheric_Mansion/Meshes/Walls/SM_outer_wall_door_3x3m.SM_outer_wall_door_3x3m")
                (Rendering|SetVisibility _sm_outer_wall_door_3x3m true false))
              (CallFunction|MasterChangeMat _sm_inner_wall_door_3x3m_a _sm_inner_wall_door_3x3m_b _sm_inner_wall_door_3x3m_b _sm_inner_wall_door_3x3m_a _sm_inner_wall_door_3x3m_b _sm_inner_wall_door_3x3m_b)
              (CallFunction|PaintattribFunc _sm_inner_wall_door_3x3m_a _sm_inner_wall_door_3x3m_b _sm_inner_wall_door_3x3m_b))
            (:NewEnumerator6
              (goto _label))))
        (:NewEnumerator4
          ;[0 0 0] 3x4
          (switch Utilities|FlowControl|Switch|SwitchonE_WallTypes (Variables|WallTypes|GetE_Wall%20Types)
            (:NewEnumerator0
              (CallFunction|SetMeshFunction _sm_inner_wall_3x4m_a _sm_inner_wall_3x4m_b _sm_inner_wall_3x4m_c "/Game/Modular_Asmospheric_Mansion/Meshes/Walls/SM_inner_wall_3x4m_A.SM_inner_wall_3x4m_A" "/Game/Modular_Asmospheric_Mansion/Meshes/Walls/SM_inner_wall_3x4m_B.SM_inner_wall_3x4m_B" "/Game/Modular_Asmospheric_Mansion/Meshes/Walls/SM_inner_wall_3x4m_C.SM_inner_wall_3x4m_C")
              (if (Variables|Default|GetADD%20OUTER%20WALL%20?)
                (Components|StaticMesh|SetStaticMesh _sm_outer_wall_3x4m_3 "/Game/Modular_Asmospheric_Mansion/Meshes/Walls/SM_outer_wall_3x4m.SM_outer_wall_3x4m")
                (Rendering|SetVisibility _sm_outer_wall_3x4m_3 true false))
              (CallFunction|MasterChangeMat _sm_inner_wall_3x4m_a _sm_inner_wall_3x4m_b _sm_inner_wall_3x4m_c _sm_inner_wall_3x4m_a _sm_inner_wall_3x4m_b _sm_inner_wall_3x4m_c)
              (CallFunction|PaintattribFunc _sm_inner_wall_3x4m_a _sm_inner_wall_3x4m_b _sm_inner_wall_3x4m_c))
            (:NewEnumerator1
              (CallFunction|SetMeshFunction _sm_inner_wall_window_3x4m_a _sm_inner_wall_window_3x4m_b _sm_inner_wall_window_3x4m_c "/Game/Modular_Asmospheric_Mansion/Meshes/Walls/SM_inner_wall_window_3x4m_A.SM_inner_wall_window_3x4m_A" "/Game/Modular_Asmospheric_Mansion/Meshes/Walls/SM_inner_wall_window_3x4m_B.SM_inner_wall_window_3x4m_B" "/Game/Modular_Asmospheric_Mansion/Meshes/Walls/SM_inner_wall_window_3x4m_C.SM_inner_wall_window_3x4m_C")
              (if (Variables|Default|GetADD%20OUTER%20WALL%20?)
                (Components|StaticMesh|SetStaticMesh _sm_outer_wall_window_3x4m_2 "/Game/Modular_Asmospheric_Mansion/Meshes/Walls/SM_outer_wall_window_3x4m.SM_outer_wall_window_3x4m")
                (Rendering|SetVisibility _sm_outer_wall_window_3x4m_2 true false))
              (CallFunction|MasterChangeMat _sm_inner_wall_window_3x4m_a _sm_inner_wall_window_3x4m_b _sm_inner_wall_window_3x4m_c _sm_inner_wall_window_3x4m_a _sm_inner_wall_window_3x4m_b _sm_inner_wall_window_3x4m_c)
              (CallFunction|PaintattribFunc _sm_inner_wall_window_3x4m_a _sm_inner_wall_window_3x4m_b _sm_inner_wall_window_3x4m_c))
            (:NewEnumerator3
              (CallFunction|SetMeshFunction _sm_inner_wall_wide_window_3x4m_a _sm_inner_wall_wide_window_3x4m_b _sm_inner_wall_wide_window_3x4m_c "/Game/Modular_Asmospheric_Mansion/Meshes/Walls/SM_inner_wall_wide_window_3x4m_A.SM_inner_wall_wide_window_3x4m_A" "/Game/Modular_Asmospheric_Mansion/Meshes/Walls/SM_inner_wall_wide_window_3x4m_B.SM_inner_wall_wide_window_3x4m_B" "/Game/Modular_Asmospheric_Mansion/Meshes/Walls/SM_inner_wall_wide_window_3x4m_C.SM_inner_wall_wide_window_3x4m_C")
              (if (Variables|Default|GetADD%20OUTER%20WALL%20?)
                (Components|StaticMesh|SetStaticMesh _sm_outer_wall_wide_window_3x4m_2 "/Game/Modular_Asmospheric_Mansion/Meshes/Walls/SM_outer_wall_wide_window_3x4m.SM_outer_wall_wide_window_3x4m")
                (Rendering|SetVisibility _sm_outer_wall_wide_window_3x4m_2 true false))
              (CallFunction|MasterChangeMat _sm_inner_wall_wide_window_3x4m_a _sm_inner_wall_wide_window_3x4m_b _sm_inner_wall_wide_window_3x4m_c _sm_inner_wall_wide_window_3x4m_a _sm_inner_wall_wide_window_3x4m_b _sm_inner_wall_wide_window_3x4m_c)
              (CallFunction|PaintattribFunc _sm_inner_wall_wide_window_3x4m_a _sm_inner_wall_wide_window_3x4m_b _sm_inner_wall_wide_window_3x4m_c))
            (:NewEnumerator5
              (CallFunction|SetMeshFunction _sm_inner_wall_door_3x4m_a _sm_inner_wall_door_3x4m_b _sm_inner_wall_door_3x4m_c "/Game/Modular_Asmospheric_Mansion/Meshes/Walls/SM_inner_wall_door_3x4m_A.SM_inner_wall_door_3x4m_A" "/Game/Modular_Asmospheric_Mansion/Meshes/Walls/SM_inner_wall_door_3x4m_B.SM_inner_wall_door_3x4m_B" "/Game/Modular_Asmospheric_Mansion/Meshes/Walls/SM_inner_wall_door_3x4m_C.SM_inner_wall_door_3x4m_C")
              (if (Variables|Default|GetADD%20OUTER%20WALL%20?)
                (Components|StaticMesh|SetStaticMesh _sm_outer_wall_singledoor_3x4m_2 "/Game/Modular_Asmospheric_Mansion/Meshes/Walls/SM_outer_wall_singledoor_3x4m.SM_outer_wall_singledoor_3x4m")
                (Rendering|SetVisibility _sm_outer_wall_singledoor_3x4m_2 true false))
              (CallFunction|MasterChangeMat _sm_inner_wall_door_3x4m_a _sm_inner_wall_door_3x4m_b _sm_inner_wall_door_3x4m_c _sm_inner_wall_door_3x4m_a _sm_inner_wall_door_3x4m_b _sm_inner_wall_door_3x4m_c)
              (CallFunction|PaintattribFunc _sm_inner_wall_door_3x4m_a _sm_inner_wall_door_3x4m_b _sm_inner_wall_door_3x4m_c))
            (:NewEnumerator6
              (CallFunction|SetMeshFunction _sm_inner_wall_doubledoor_3x4m_a _sm_inner_wall_doubledoor_3x4m_b _sm_inner_wall_doubledoor_3x4m_c "/Game/Modular_Asmospheric_Mansion/Meshes/Walls/SM_inner_wall_doubledoor_3x4m_A.SM_inner_wall_doubledoor_3x4m_A" "/Game/Modular_Asmospheric_Mansion/Meshes/Walls/SM_inner_wall_doubledoor_3x4m_B.SM_inner_wall_doubledoor_3x4m_B" "/Game/Modular_Asmospheric_Mansion/Meshes/Walls/SM_inner_wall_doubledoor_3x4m_C.SM_inner_wall_doubledoor_3x4m_C")
              (if (Variables|Default|GetADD%20OUTER%20WALL%20?)
                (Components|StaticMesh|SetStaticMesh _sm_outer_wall_doubledoor_3x4m_2 "/Game/Modular_Asmospheric_Mansion/Meshes/Walls/SM_outer_wall_doubledoor_3x4m.SM_outer_wall_doubledoor_3x4m")
                (Rendering|SetVisibility _sm_outer_wall_doubledoor_3x4m_2 true false))
              (CallFunction|MasterChangeMat _sm_inner_wall_doubledoor_3x4m_a _sm_inner_wall_doubledoor_3x4m_b _sm_inner_wall_doubledoor_3x4m_c _sm_inner_wall_doubledoor_3x4m_a _sm_inner_wall_doubledoor_3x4m_b _sm_inner_wall_doubledoor_3x4m_c)
              (CallFunction|PaintattribFunc _sm_inner_wall_doubledoor_3x4m_a _sm_inner_wall_doubledoor_3x4m_b _sm_inner_wall_doubledoor_3x4m_c))))
        (:NewEnumerator5
          ;[0 0 0 1 50] 3x6
          (CallFunction|SetMeshFunction _sm_inner_wall_widewindow_3x6m_a _sm_inner_wall_widewindow_3x6m_b _sm_inner_wall_widewindow_3x6m_c "/Game/Modular_Asmospheric_Mansion/Meshes/Walls/SM_inner_wall_widewindow_3x6m_A.SM_inner_wall_widewindow_3x6m_A" "/Game/Modular_Asmospheric_Mansion/Meshes/Walls/SM_inner_wall_widewindow_3x6m_B.SM_inner_wall_widewindow_3x6m_B" "/Game/Modular_Asmospheric_Mansion/Meshes/Walls/SM_inner_wall_widewindow_3x6m_C.SM_inner_wall_widewindow_3x6m_C")
          (if (Variables|Default|GetADD%20OUTER%20WALL%20?)
            (Components|StaticMesh|SetStaticMesh _sm_outer_wall_widewindow_3x6m_2 "/Game/Modular_Asmospheric_Mansion/Meshes/Walls/SM_outer_wall_widewindow_3x6m.SM_outer_wall_widewindow_3x6m")
            (Rendering|SetVisibility _sm_outer_wall_widewindow_3x6m_2 true false))
          (CallFunction|MasterChangeMat _sm_inner_wall_widewindow_3x6m_a _sm_inner_wall_widewindow_3x6m_b _sm_inner_wall_widewindow_3x6m_c _sm_inner_wall_widewindow_3x6m_a _sm_inner_wall_widewindow_3x6m_b _sm_inner_wall_widewindow_3x6m_c)
          (CallFunction|PaintattribFunc _sm_inner_wall_widewindow_3x6m_a _sm_inner_wall_widewindow_3x6m_b _sm_inner_wall_widewindow_3x6m_c))))
    (:then_1
      ;[1 0.09645 0] SetOuter Materials
      (if (Variables|PaintAttributes|GetPaint%20Outer%20Active%20?)
        (Rendering|Material|SetMaterial (Utilities|Array|MakeArray _sm_outer_wall_wide_window_3x4m _sm_outer_wall_doubledoor_3x4m _sm_outer_wall_door_3x3m_2 _sm_outer_wall_windowed_3x3m _sm_outer_wall_window_3x4m _sm_outer_wall_singledoor_3x4m _sm_outer_wall_3x4m _sm_outer_wall_3x0_5m _sm_outer_wall_3x1m _sm_outer_wall_3x2m _sm_outer_wall_window_3x2m _sm_outer_wall_widewindow_3x6m) 0 (Variables|Default|GetSet%20Outer%20Wall%20Mat))
        (CallFunction|ChangeMatParameters (Variables|PaintAttributes|GetPaint%20Color%20Change) (Variables|PaintAttributes|GetPaint%20Density) (Variables|PaintAttributes|GetPaint%20Contrast) (Variables|PaintAttributes|GetDesaturation) (Utilities|Array|MakeArray _sm_outer_wall_wide_window_3x4m _sm_outer_wall_doubledoor_3x4m _sm_outer_wall_door_3x3m_2 _sm_outer_wall_windowed_3x3m _sm_outer_wall_window_3x4m _sm_outer_wall_singledoor_3x4m _sm_outer_wall_3x4m _sm_outer_wall_3x0_5m _sm_outer_wall_3x1m _sm_outer_wall_3x2m _sm_outer_wall_window_3x2m _sm_outer_wall_widewindow_3x6m))
        (else
          ;[1 0.09645 0] SetOuter Materials
          (Rendering|Material|SetMaterial (Utilities|Array|MakeArray (Variables|Default|GetSM_outer_wall_wide_window_3x4m) (Variables|Default|GetSM_outer_wall_doubledoor_3x4m) (Variables|Default|GetSM_outer_wall_door_3x3m) (Variables|Default|GetSM_outer_wall_windowed_3x3m) (Variables|Default|GetSM_outer_wall_window_3x4m) (Variables|Default|GetSM_outer_wall_singledoor_3x4m) (Variables|Default|GetSM_outer_wall_3x4m) (Variables|Default|GetSM_Outer_Wall_3x0_5m) (Variables|Default|GetSM_outer_wall_3x1m) (Variables|Default|GetSM_outer_wall_3x2m) (Variables|Default|GetSM_outer_wall_window_3x2m) (Variables|Default|GetSM_outer_wall_widewindow_3x6m)) 0 (Variables|Default|GetSet%20Outer%20Wall%20Mat)))))))

(fn SetMeshFunction
  (params (A :type Static%20Mesh%20Component%20Object%20Reference) (B :type Static%20Mesh%20Component%20Object%20Reference) (C :type Static%20Mesh%20Component%20Object%20Reference) (MESH%20A :type Static%20Mesh%20Object%20Reference) (MESH%20B :type Static%20Mesh%20Object%20Reference) (MESH%20C :type Static%20Mesh%20Object%20Reference))
  (switch Utilities|FlowControl|Switch|SwitchonE_Style (Variables|INNERWALLS|GetSTYLE)
    (:NewEnumerator0
      (Components|StaticMesh|SetStaticMesh A MESH%20A)
      (Rendering|SetVisibility A true false))
    (:NewEnumerator1
      (Components|StaticMesh|SetStaticMesh B MESH%20B)
      (Rendering|SetVisibility B true false))
    (:NewEnumerator2
      (Components|StaticMesh|SetStaticMesh C MESH%20C)
      (Rendering|SetVisibility C true false)))
  (return))

(fn ChangeMatStyleFunctionIndex0
  (params (Target%20A :type Primitive%20Component%20Object%20Reference) (Target%20B :type Primitive%20Component%20Object%20Reference) (Target%20C :type Primitive%20Component%20Object%20Reference))
  (Utilities|FlowControl|Sequence
    (:then_0
      (CallFunction|MASTERCHANGEMATFUNCFORINDEX0 Target%20A))
    (:then_1
      (CallFunction|MASTERCHANGEMATFUNCFORINDEX0 Target%20B))
    (:then_2
      (CallFunction|MASTERCHANGEMATFUNCFORINDEX0 Target%20C))))

(fn MasterChangeMat
  (params (Target%20A%20Index%200 :type Primitive%20Component%20Object%20Reference) (Target%20B%20Index%200 :type Primitive%20Component%20Object%20Reference) (Target%20C%20Index%200 :type Primitive%20Component%20Object%20Reference) (Target%20A2%20Index1 :type Primitive%20Component%20Object%20Reference) (Target%20B2%20Index1 :type Primitive%20Component%20Object%20Reference) (Target%20C2%20Index1 :type Primitive%20Component%20Object%20Reference))
  (if (Variables|MaterialChangeInnerWall|GetChange%20Material%20?)
    (CallFunction|ChangeMatStyleFunctionIndex0 Target%20A%20Index%200 Target%20B%20Index%200 Target%20C%20Index%200)
    (CallFunction|ChangeMatStyleFunctionIndex1 Target%20A2%20Index1 Target%20B2%20Index1 Target%20C2%20Index1)))

(fn INDEX0MATFUNC
  (params (InputPin :type Primitive%20Component%20Object%20Reference))
  ;[0 0 0] STYLE A
  (switch Utilities|FlowControl|Switch|SwitchonE_Wall_Inner_Materials (Variables|MaterialChangeInnerWall|GetIndex%200%20Mat%20Type)
    (:NewEnumerator0
      (Rendering|Material|SetMaterial InputPin 0 "/Game/Modular_Asmospheric_Mansion/Materials/Instance/MI_weathered_brown_planks.MI_weathered_brown_planks"))
    (:NewEnumerator1
      (Rendering|Material|SetMaterial InputPin 0 "/Game/Modular_Asmospheric_Mansion/Materials/Instance/Alternatives/MI_Wallpaper_3.MI_Wallpaper_3"))
    (:NewEnumerator2
      (Rendering|Material|SetMaterial InputPin 0 "/Game/Modular_Asmospheric_Mansion/Materials/Instance/Alternatives/MI_Wallpaper_2.MI_Wallpaper_2"))
    (:NewEnumerator3
      (Rendering|Material|SetMaterial InputPin 0 "/Game/Modular_Asmospheric_Mansion/Materials/Instance/Alternatives/MI_Wallpaper_1.MI_Wallpaper_1"))
    (:NewEnumerator4
      (Rendering|Material|SetMaterial InputPin 0 "/Game/Modular_Asmospheric_Mansion/Materials/Instance/Alternatives/MI_Tiles_05.MI_Tiles_05"))
    (:NewEnumerator5
      (Rendering|Material|SetMaterial InputPin 0 "/Game/Modular_Asmospheric_Mansion/Materials/Instance/Alternatives/MI_Tiles_04.MI_Tiles_04"))
    (:NewEnumerator6
      (Rendering|Material|SetMaterial InputPin 0 "/Game/Modular_Asmospheric_Mansion/Materials/Instance/Alternatives/MI_Tiles_03.MI_Tiles_03"))
    (:NewEnumerator7
      (Rendering|Material|SetMaterial InputPin 0 "/Game/Modular_Asmospheric_Mansion/Materials/Instance/Alternatives/MI_Tiles_02.MI_Tiles_02"))
    (:NewEnumerator8
      (Rendering|Material|SetMaterial InputPin 0 "/Game/Modular_Asmospheric_Mansion/Materials/Instance/Alternatives/MI_Tiles_01.MI_Tiles_01"))
    (:NewEnumerator9
      (Rendering|Material|SetMaterial InputPin 0 "/Game/Modular_Asmospheric_Mansion/Materials/Instance/Alternatives/MI_Outer_Wall_Tile_04.MI_Outer_Wall_Tile_04"))
    (:NewEnumerator10
      (Rendering|Material|SetMaterial InputPin 0 "/Game/Modular_Asmospheric_Mansion/Materials/Instance/Alternatives/MI_Outer_Wall_Tile_03.MI_Outer_Wall_Tile_03"))
    (:NewEnumerator11
      (Rendering|Material|SetMaterial InputPin 0 "/Game/Modular_Asmospheric_Mansion/Materials/Instance/Alternatives/MI_Outer_Wall_Tile_02.MI_Outer_Wall_Tile_02"))))

(fn MASTERCHANGEMATFUNCFORINDEX0
  (params (InputPin :type Primitive%20Component%20Object%20Reference))
  (switch Utilities|FlowControl|Switch|SwitchonE_Style (Variables|INNERWALLS|GetSTYLE)
    (:NewEnumerator0
      (CallFunction|INDEX0MATFUNC InputPin))
    (:NewEnumerator1
      (CallFunction|INDEX0MATFUNC InputPin))
    (:NewEnumerator2
      (CallFunction|INDEX0MATFUNC InputPin))))

(fn INDEX1MATFUNC
  (params (InputPin :type Primitive%20Component%20Object%20Reference))
  ;[0 0 0] STYLE A
  (switch Utilities|FlowControl|Switch|SwitchonE_Wall_Inner_Materials (Variables|MaterialChangeInnerWall|GetIndex%201%20Mat%20Type)
    (:NewEnumerator0
      (Rendering|Material|SetMaterial InputPin 1 "/Game/Modular_Asmospheric_Mansion/Materials/Instance/MI_weathered_brown_planks.MI_weathered_brown_planks"))
    (:NewEnumerator1
      (Rendering|Material|SetMaterial InputPin 1 "/Game/Modular_Asmospheric_Mansion/Materials/Instance/Alternatives/MI_Wallpaper_3.MI_Wallpaper_3"))
    (:NewEnumerator2
      (Rendering|Material|SetMaterial InputPin 1 "/Game/Modular_Asmospheric_Mansion/Materials/Instance/Alternatives/MI_Wallpaper_2.MI_Wallpaper_2"))
    (:NewEnumerator3
      (Rendering|Material|SetMaterial InputPin 1 "/Game/Modular_Asmospheric_Mansion/Materials/Instance/Alternatives/MI_Wallpaper_1.MI_Wallpaper_1"))
    (:NewEnumerator4
      (Rendering|Material|SetMaterial InputPin 1 "/Game/Modular_Asmospheric_Mansion/Materials/Instance/Alternatives/MI_Tiles_05.MI_Tiles_05"))
    (:NewEnumerator5
      (Rendering|Material|SetMaterial InputPin 1 "/Game/Modular_Asmospheric_Mansion/Materials/Instance/Alternatives/MI_Tiles_04.MI_Tiles_04"))
    (:NewEnumerator6
      (Rendering|Material|SetMaterial InputPin 1 "/Game/Modular_Asmospheric_Mansion/Materials/Instance/Alternatives/MI_Tiles_03.MI_Tiles_03"))
    (:NewEnumerator7
      (Rendering|Material|SetMaterial InputPin 1 "/Game/Modular_Asmospheric_Mansion/Materials/Instance/Alternatives/MI_Tiles_02.MI_Tiles_02"))
    (:NewEnumerator8
      (Rendering|Material|SetMaterial InputPin 1 "/Game/Modular_Asmospheric_Mansion/Materials/Instance/Alternatives/MI_Tiles_01.MI_Tiles_01"))
    (:NewEnumerator9
      (Rendering|Material|SetMaterial InputPin 1 "/Game/Modular_Asmospheric_Mansion/Materials/Instance/Alternatives/MI_Outer_Wall_Tile_04.MI_Outer_Wall_Tile_04"))
    (:NewEnumerator10
      (Rendering|Material|SetMaterial InputPin 1 "/Game/Modular_Asmospheric_Mansion/Materials/Instance/Alternatives/MI_Outer_Wall_Tile_03.MI_Outer_Wall_Tile_03"))
    (:NewEnumerator11
      (Rendering|Material|SetMaterial InputPin 1 "/Game/Modular_Asmospheric_Mansion/Materials/Instance/Alternatives/MI_Outer_Wall_Tile_02.MI_Outer_Wall_Tile_02"))))

(fn ChangeMatStyleFunctionIndex1
  (params (Target%20A :type Primitive%20Component%20Object%20Reference) (Target%20B :type Primitive%20Component%20Object%20Reference) (Target%20C :type Primitive%20Component%20Object%20Reference))
  (Utilities|FlowControl|Sequence
    (:then_0
      (CallFunction|MASTERCHANGEMATFUNCFORINDEX1 Target%20A))
    (:then_1
      (CallFunction|MASTERCHANGEMATFUNCFORINDEX1 Target%20B))
    (:then_2
      (CallFunction|MASTERCHANGEMATFUNCFORINDEX1 Target%20C))))

(fn MASTERCHANGEMATFUNCFORINDEX1
  (params (InputPin :type Primitive%20Component%20Object%20Reference))
  (switch Utilities|FlowControl|Switch|SwitchonE_Style (Variables|INNERWALLS|GetSTYLE)
    (:NewEnumerator0
      (CallFunction|INDEX1MATFUNC InputPin))
    (:NewEnumerator1
      (CallFunction|INDEX1MATFUNC InputPin))
    (:NewEnumerator2
      (CallFunction|INDEX1MATFUNC InputPin))))

(fn ChangeMatParameters
  (params (PaintColor_Change :type Linear%20Color%20Structure :default "(R=1.000000,G=1.000000,B=1.000000,A=1.000000)") (Paint%20Density :type Float%20%28double-precision%29) (Paint%20Contrast :type Float%20%28double-precision%29) (Desaturation :type Float%20%28double-precision%29) (Target :type Array%20of%20Mesh%20Component%20Object%20References))
  (Rendering|Material|SetScalarParameterValueonMaterials Target "Paint_Intensity" Paint%20Density)
  (Rendering|Material|SetVectorParameterValueonMaterials Target "PaintColor" (Math|Conversions|ToVector(LinearColor) PaintColor_Change))
  (Rendering|Material|SetScalarParameterValueonMaterials Target "Paint_Contrast" Paint%20Contrast)
  (Rendering|Material|SetScalarParameterValueonMaterials Target "Desaturation" Desaturation))

(fn PaintattribFunc
  (params ([0] :type Mesh%20Component%20Object%20Reference) ([1] :type Mesh%20Component%20Object%20Reference) ([2] :type Mesh%20Component%20Object%20Reference) ([3] :type Mesh%20Component%20Object%20Reference))
  (if (Variables|PaintAttributes|GetPaint%20Inner%20Active%20?)
    (CallFunction|ChangeMatParameters (Variables|PaintAttributes|GetPaint%20Color%20Change) (Variables|PaintAttributes|GetPaint%20Density) (Variables|PaintAttributes|GetPaint%20Contrast) (Variables|PaintAttributes|GetDesaturation) (Utilities|Array|MakeArray [0] [1] [2] [3]))))