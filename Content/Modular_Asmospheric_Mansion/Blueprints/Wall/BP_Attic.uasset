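; Modular attic inner wall piece for the mansion kit, switchable between straight lengths, a corner, window and windowless variants through the AtticTypes selector.
; The construction script assigns the mesh matching the selected type to its dedicated component and makes it visible.
; When PaintActive is set, it pushes paint color, intensity, contrast and desaturation into the wall materials.
; Collision is applied across the root's descendants at construction and again on BeginPlay.
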(event EventBeginPlay
  (CallFunction|FSetCollision (Variables|Default|GetDefaultSceneRoot) true))

(event Collision|EventActorBeginOverlap
  (params (OtherActor :type Actor%20Object%20Reference)))

(event EventTick
  (params (DeltaSeconds :type Float%20%28single-precision%29)))

(fn ConstructionScript
  (bind _sm_inner_attic_wall_05m (Variables|Default|GetSM_inner_attic_wall_05m))
  (bind _sm_inner_attic_wall_window_01 (Variables|Default|GetSM_inner_attic_wall_window_01))
  (bind _sm_inner_attic_wall_window_02 (Variables|Default|GetSM_inner_attic_wall_window_02))
  (bind _sm_inner_attic_wall_windowless_01 (Variables|Default|GetSM_inner_attic_wall_windowless_01))
  (bind _sm_inner_attic_wall_windowless_02 (Variables|Default|GetSM_inner_attic_wall_windowless_02))
  (bind _sm_inner_attic_wall_windowless_03_a (Variables|Default|GetSM_inner_attic_wall_windowless_03_A))
  (bind _sm_inner_attic_wall_windowless_03_b (Variables|Default|GetSM_inner_attic_wall_windowless_03_B))
  (bind _sm_inner_attic_wall_1m (Variables|Default|GetSM_inner_attic_wall_1m))
  (bind _sm_inner_attic_wall_2m (Variables|Default|GetSM_inner_attic_wall_2m))
  (bind _sm_inner_attic_wall_3m (Variables|Default|GetSM_inner_attic_wall_3m))
  (bind _sm_inner_attic_wall_4m (Variables|Default|GetSM_inner_attic_wall_4m))
  (bind _sm_inner_attic_wall_corner (Variables|Default|GetSM_inner_attic_wall_corner))
  (bind _sm_inner_attic_wall_double_window_01 (Variables|Default|GetSM_inner_attic_wall_double_window_01))
  (bind _sm_inner_attic_wall_double_window_02 (Variables|Default|GetSM_inner_attic_wall_double_window_02))
  (switch Utilities|FlowControl|Switch|SwitchonE_AtticTypes (Variables|Default|GetAttic%20Types)
    (:NewEnumerator0
      _)
    (:NewEnumerator1
      _)
    (:NewEnumerator2
      _)
    (:NewEnumerator3
      _)
    (:NewEnumerator4
      _)
    (:NewEnumerator5
      _)
    (:NewEnumerator6
      _)
    (:NewEnumerator7
      _)
    (:NewEnumerator8
      _)
    (:NewEnumerator9
      _)
    (:NewEnumerator10
      _)
    (:NewEnumerator11
      _)
    (:NewEnumerator12
      _)
    (:NewEnumerator13
      _))
  (CallFunction|SetMeshFunction _sm_inner_attic_wall_05m _sm_inner_attic_wall_1m _sm_inner_attic_wall_2m _sm_inner_attic_wall_3m _sm_inner_attic_wall_4m _sm_inner_attic_wall_corner _sm_inner_attic_wall_double_window_01 _sm_inner_attic_wall_double_window_02 _sm_inner_attic_wall_window_01 _sm_inner_attic_wall_window_02 _sm_inner_attic_wall_windowless_01 _sm_inner_attic_wall_windowless_02 _sm_inner_attic_wall_windowless_03_a _sm_inner_attic_wall_windowless_03_b "/Game/Modular_Asmospheric_Mansion/Meshes/Walls/SM_inner_attic_wall_05m.SM_inner_attic_wall_05m" "/Game/Modular_Asmospheric_Mansion/Meshes/Walls/SM_inner_attic_wall_1m.SM_inner_attic_wall_1m" "/Game/Modular_Asmospheric_Mansion/Meshes/Walls/SM_inner_attic_wall_2m.SM_inner_attic_wall_2m" "/Game/Modular_Asmospheric_Mansion/Meshes/Walls/SM_inner_attic_wall_3m.SM_inner_attic_wall_3m" "/Game/Modular_Asmospheric_Mansion/Meshes/Walls/SM_inner_attic_wall_4m.SM_inner_attic_wall_4m" "/Game/Modular_Asmospheric_Mansion/Meshes/Walls/SM_inner_attic_wall_corner.SM_inner_attic_wall_corner" "/Game/Modular_Asmospheric_Mansion/Meshes/Walls/SM_inner_attic_wall_double_window_01.SM_inner_attic_wall_double_window_01" "/Game/Modular_Asmospheric_Mansion/Meshes/Walls/SM_inner_attic_wall_double_window_02.SM_inner_attic_wall_double_window_02" "/Game/Modular_Asmospheric_Mansion/Meshes/Walls/SM_inner_attic_wall_window_01.SM_inner_attic_wall_window_01" "/Game/Modular_Asmospheric_Mansion/Meshes/Walls/SM_inner_attic_wall_window_02.SM_inner_attic_wall_window_02" "/Game/Modular_Asmospheric_Mansion/Meshes/Walls/SM_inner_attic_wall_windowless_01.SM_inner_attic_wall_windowless_01" "/Game/Modular_Asmospheric_Mansion/Meshes/Walls/SM_inner_attic_wall_windowless_02.SM_inner_attic_wall_windowless_02" "/Game/Modular_Asmospheric_Mansion/Meshes/Walls/SM_inner_attic_wall_windowless_03_A.SM_inner_attic_wall_windowless_03_A" "/Game/Modular_Asmospheric_Mansion/Meshes/Walls/SM_inner_attic_wall_windowless_03_B.SM_inner_attic_wall_windowless_03_B")
  (CallFunction|PaintattribFunc (Utilities|Array|MakeArray _sm_inner_attic_wall_05m _sm_inner_attic_wall_1m _sm_inner_attic_wall_2m _sm_inner_attic_wall_3m _sm_inner_attic_wall_4m _sm_inner_attic_wall_corner _sm_inner_attic_wall_double_window_01 _sm_inner_attic_wall_double_window_02 _sm_inner_attic_wall_window_01 _sm_inner_attic_wall_window_02 _sm_inner_attic_wall_windowless_01 _sm_inner_attic_wall_windowless_02 _sm_inner_attic_wall_windowless_03_a _sm_inner_attic_wall_windowless_03_b))
  (CallFunction|FSetCollision (Variables|Default|GetDefaultSceneRoot) true))

(fn SetMeshFunction
  (params (Target :type Static%20Mesh%20Component%20Object%20Reference) (Target1 :type Static%20Mesh%20Component%20Object%20Reference) (Target2 :type Static%20Mesh%20Component%20Object%20Reference) (Target3 :type Static%20Mesh%20Component%20Object%20Reference) (Target4 :type Static%20Mesh%20Component%20Object%20Reference) (Target5 :type Static%20Mesh%20Component%20Object%20Reference) (Target6 :type Static%20Mesh%20Component%20Object%20Reference) (Target7 :type Static%20Mesh%20Component%20Object%20Reference) (Target8 :type Static%20Mesh%20Component%20Object%20Reference) (Target9 :type Static%20Mesh%20Component%20Object%20Reference) (Target10 :type Static%20Mesh%20Component%20Object%20Reference) (Target11 :type Static%20Mesh%20Component%20Object%20Reference) (Target12 :type Static%20Mesh%20Component%20Object%20Reference) (Target13 :type Static%20Mesh%20Component%20Object%20Reference) (NewMesh :type Static%20Mesh%20Object%20Reference) (NewMesh1 :type Static%20Mesh%20Object%20Reference) (NewMesh2 :type Static%20Mesh%20Object%20Reference) (NewMesh3 :type Static%20Mesh%20Object%20Reference) (NewMesh4 :type Static%20Mesh%20Object%20Reference) (NewMesh5 :type Static%20Mesh%20Object%20Reference) (NewMesh6 :type Static%20Mesh%20Object%20Reference) (NewMesh7 :type Static%20Mesh%20Object%20Reference) (NewMesh8 :type Static%20Mesh%20Object%20Reference) (NewMesh9 :type Static%20Mesh%20Object%20Reference) (NewMesh10 :type Static%20Mesh%20Object%20Reference) (NewMesh11 :type Static%20Mesh%20Object%20Reference) (NewMesh12 :type Static%20Mesh%20Object%20Reference) (NewMesh13 :type Static%20Mesh%20Object%20Reference))
  (switch Utilities|FlowControl|Switch|SwitchonE_AtticTypes (Variables|Default|GetAttic%20Types)
    (:NewEnumerator0
      (Components|StaticMesh|SetStaticMesh Target NewMesh)
      (Rendering|SetVisibility Target true false))
    (:NewEnumerator1
      (Components|StaticMesh|SetStaticMesh Target1 NewMesh1)
      (Rendering|SetVisibility Target1 true false))
    (:NewEnumerator2
      (Components|StaticMesh|SetStaticMesh Target2 NewMesh2)
      (Rendering|SetVisibility Target2 true false))
    (:NewEnumerator3
      (Components|StaticMesh|SetStaticMesh Target3 NewMesh3)
      (Rendering|SetVisibility Target3 true false))
    (:NewEnumerator4
      (Components|StaticMesh|SetStaticMesh Target4 NewMesh4)
      (Rendering|SetVisibility Target4 true false))
    (:NewEnumerator5
      (Components|StaticMesh|SetStaticMesh Target5 NewMesh5)
      (Rendering|SetVisibility Target5 true false))
    (:NewEnumerator6
      (Components|StaticMesh|SetStaticMesh Target6 NewMesh6)
      (Rendering|SetVisibility Target6 true false))
    (:NewEnumerator7
      (Components|StaticMesh|SetStaticMesh Target7 NewMesh7)
      (Rendering|SetVisibility Target7 true false))
    (:NewEnumerator8
      (Components|StaticMesh|SetStaticMesh Target8 NewMesh8)
      (Rendering|SetVisibility Target8 true false))
    (:NewEnumerator9
      (Components|StaticMesh|SetStaticMesh Target9 NewMesh9)
      (Rendering|SetVisibility Target9 true false))
    (:NewEnumerator10
      (Components|StaticMesh|SetStaticMesh Target10 NewMesh10)
      (Rendering|SetVisibility Target10 true false))
    (:NewEnumerator11
      (Components|StaticMesh|SetStaticMesh Target11 NewMesh11)
      (Rendering|SetVisibility Target11 true false))
    (:NewEnumerator12
      (Components|StaticMesh|SetStaticMesh Target12 NewMesh12)
      (Rendering|SetVisibility Target12 true false))
    (:NewEnumerator13
      (Components|StaticMesh|SetStaticMesh Target13 NewMesh13)
      (Rendering|SetVisibility Target13 true false)))
  (return))

(fn ChangeMatParameters
  (params (PaintColor_Change :type Linear%20Color%20Structure :default "(R=1.000000,G=1.000000,B=1.000000,A=1.000000)") (Paint%20Density :type Float%20%28single-precision%29) (Paint%20Contrast :type Float%20%28single-precision%29) (Desaturation :type Float%20%28single-precision%29) (NewParam :type Array%20of%20Mesh%20Component%20Object%20References))
  (Rendering|Material|SetScalarParameterValueonMaterials NewParam "Paint_Intensity" Paint%20Density)
  (Rendering|Material|SetVectorParameterValueonMaterials NewParam "PaintColor" (Math|Conversions|ToVector(LinearColor) PaintColor_Change))
  (Rendering|Material|SetScalarParameterValueonMaterials NewParam "Paint_Contrast" Paint%20Contrast)
  (Rendering|Material|SetScalarParameterValueonMaterials NewParam "Desaturation" Desaturation)
  (return))

(fn PaintattribFunc
  (params ([0] :type Array%20of%20Mesh%20Component%20Object%20References))
  (if (Variables|PaintAttrib|GetPaint%20Active%20?)
    (CallFunction|ChangeMatParameters (Variables|PaintAttrib|GetPaint%20Color%20Change) (Variables|PaintAttrib|GetPaint%20Density) (Variables|PaintAttrib|GetPaint%20Contrast) (Variables|PaintAttrib|GetDesaturation) [0])))