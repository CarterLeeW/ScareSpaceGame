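; Modular mansion wall corner actor that shows either an outer wood pillar or one of six inner corner wall meshes, picked by variables.
; The construction script sets the mesh, then for inner corners optionally assigns materials from preset lists to slots 0 and 1 and applies paint and desaturation parameters.
; All STYLE branches call the same material function, so that switch has no effect.
; BeginPlay calls FSetCollision on the root and its descendants.
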(event EventBeginPlay
  (CallFunction|FSetCollision (Variables|Default|GetDefaultSceneRoot) true))

(event Collision|EventActorBeginOverlap
  (params (OtherActor :type Actor%20Object%20Reference)))

(event EventTick
  (params (DeltaSeconds :type Float%20%28single-precision%29)))

(fn ConstructionScript
  (bind _sm_wood_pillar_03 (Variables|Default|GetSM_wood_pillar_03))
  (bind _sm_inner_wall_3m_corner_a (Variables|Default|GetSM_inner_wall_3m_corner_A))
  (bind _sm_inner_wall_3m_corner_b (Variables|Default|GetSM_inner_wall_3M_corner_B))
  (bind _sm_inner_wall_3m_corner_c (Variables|Default|GetSM_inner_wall_3M_corner_C))
  (bind _sm_inner_wall_corner_a (Variables|Default|GetSM_inner_wall_corner_A))
  (bind _sm_inner_wall_corner_b (Variables|Default|GetSM_inner_wall_corner_B))
  (bind _sm_inner_wall_corner_c (Variables|Default|GetSM_inner_wall_corner_C))
  (if (Variables|Default|GetOuter%20Corner%20)
    (Components|StaticMesh|SetStaticMesh _sm_wood_pillar_03 "/Game/Modular_Asmospheric_Mansion/Meshes/Planks/SM_wood_pillar_03.SM_wood_pillar_03")
    (Rendering|SetVisibility _sm_wood_pillar_03 true false)
    (else
      (switch Utilities|FlowControl|Switch|SwitchonE_Wall_CornersType (Variables|Default|GetWallCorner%20Types)
        (:NewEnumerator0
          _)
        (:NewEnumerator1
          _)
        (:NewEnumerator2
          _)
        (:NewEnumerator3
          _)
        (:NewEnumerator4
          _)
        (:NewEnumerator5
          _))
      (CallFunction|SetMeshFunction _sm_inner_wall_3m_corner_a _sm_inner_wall_3m_corner_b _sm_inner_wall_3m_corner_c _sm_inner_wall_corner_a _sm_inner_wall_corner_b _sm_inner_wall_corner_c "/Game/Modular_Asmospheric_Mansion/Meshes/Walls/SM_inner_wall_3m_corner_A.SM_inner_wall_3m_corner_A" "/Game/Modular_Asmospheric_Mansion/Meshes/Walls/SM_inner_wall_3M_corner_B.SM_inner_wall_3M_corner_B" "/Game/Modular_Asmospheric_Mansion/Meshes/Walls/SM_inner_wall_3M_corner_C.SM_inner_wall_3M_corner_C" "/Game/Modular_Asmospheric_Mansion/Meshes/Walls/SM_inner_wall_corner_A.SM_inner_wall_corner_A" "/Game/Modular_Asmospheric_Mansion/Meshes/Walls/SM_inner_wall_corner_B.SM_inner_wall_corner_B" "/Game/Modular_Asmospheric_Mansion/Meshes/Walls/SM_inner_wall_corner_C.SM_inner_wall_corner_C")
      (CallFunction|MasterChangeMat _sm_inner_wall_3m_corner_a _sm_inner_wall_3m_corner_b _sm_inner_wall_3m_corner_c _sm_inner_wall_3m_corner_a _sm_inner_wall_3m_corner_b _sm_inner_wall_3m_corner_c)
      (CallFunction|MasterChangeMat _sm_inner_wall_corner_a _sm_inner_wall_corner_b _sm_inner_wall_corner_c _sm_inner_wall_corner_a _sm_inner_wall_corner_b _sm_inner_wall_corner_c)
      (CallFunction|PaintattribFunc (Utilities|Array|MakeArray _sm_inner_wall_3m_corner_a _sm_inner_wall_3m_corner_b _sm_inner_wall_3m_corner_c _sm_inner_wall_corner_a _sm_inner_wall_corner_b _sm_inner_wall_corner_c)))))

(fn SetMeshFunction
  (params (A :type Static%20Mesh%20Component%20Object%20Reference) (B :type Static%20Mesh%20Component%20Object%20Reference) (C :type Static%20Mesh%20Component%20Object%20Reference) (D :type Static%20Mesh%20Component%20Object%20Reference) (F :type Static%20Mesh%20Component%20Object%20Reference) (G :type Static%20Mesh%20Component%20Object%20Reference) (MESH%20A :type Static%20Mesh%20Object%20Reference) (MESH%20B :type Static%20Mesh%20Object%20Reference) (MESH%20C :type Static%20Mesh%20Object%20Reference) (MESH%20D :type Static%20Mesh%20Object%20Reference) (MESH%20F :type Static%20Mesh%20Object%20Reference) (MESH%20G :type Static%20Mesh%20Object%20Reference))
  (switch Utilities|FlowControl|Switch|SwitchonE_Wall_CornersType (Variables|Default|GetWallCorner%20Types)
    (:NewEnumerator0
      (Components|StaticMesh|SetStaticMesh A MESH%20A)
      (Rendering|SetVisibility A true false))
    (:NewEnumerator1
      (Components|StaticMesh|SetStaticMesh B MESH%20B)
      (Rendering|SetVisibility B true false))
    (:NewEnumerator2
      (Components|StaticMesh|SetStaticMesh C MESH%20C)
      (Rendering|SetVisibility C true false))
    (:NewEnumerator3
      (Components|StaticMesh|SetStaticMesh D MESH%20D)
      (Rendering|SetVisibility D true false))
    (:NewEnumerator4
      (Components|StaticMesh|SetStaticMesh F MESH%20F)
      (Rendering|SetVisibility F true false))
    (:NewEnumerator5
      (Components|StaticMesh|SetStaticMesh G MESH%20G)
      (Rendering|SetVisibility G true false)))
  (return))

(fn MASTERCHANGEMATFUNCFORINDEX0
  (params (InputPin :type Primitive%20Component%20Object%20Reference))
  (switch Utilities|FlowControl|Switch|SwitchonE_Style (Variables|INNERWALLS|GetSTYLE)
    (:NewEnumerator0
      (CallFunction|INDEX0MATFUNC InputPin))
    (:NewEnumerator1
      (CallFunction|INDEX0MATFUNC InputPin))
    (:NewEnumerator2
      (CallFunction|INDEX0MATFUNC InputPin))))

(fn INDEX0MATFUNC
  (params (Input :type Primitive%20Component%20Object%20Reference))
  ;[0 0 0] STYLE A
  (switch Utilities|FlowControl|Switch|SwitchonE_Wall_Inner_Materials (Variables|Default|GetIndex%200%20Mat%20Type)
    (:NewEnumerator0
      (Rendering|Material|SetMaterial Input 0 "/Game/Modular_Asmospheric_Mansion/Materials/Instance/MI_weathered_brown_planks.MI_weathered_brown_planks"))
    (:NewEnumerator1
      (Rendering|Material|SetMaterial Input 0 "/Game/Modular_Asmospheric_Mansion/Materials/Instance/Alternatives/MI_Wallpaper_3.MI_Wallpaper_3"))
    (:NewEnumerator2
      (Rendering|Material|SetMaterial Input 0 "/Game/Modular_Asmospheric_Mansion/Materials/Instance/Alternatives/MI_Wallpaper_2.MI_Wallpaper_2"))
    (:NewEnumerator3
      (Rendering|Material|SetMaterial Input 0 "/Game/Modular_Asmospheric_Mansion/Materials/Instance/Alternatives/MI_Wallpaper_1.MI_Wallpaper_1"))
    (:NewEnumerator4
      (Rendering|Material|SetMaterial Input 0 "/Game/Modular_Asmospheric_Mansion/Materials/Instance/Alternatives/MI_Tiles_05.MI_Tiles_05"))
    (:NewEnumerator5
      (Rendering|Material|SetMaterial Input 0 "/Game/Modular_Asmospheric_Mansion/Materials/Instance/Alternatives/MI_Tiles_04.MI_Tiles_04"))
    (:NewEnumerator6
      (Rendering|Material|SetMaterial Input 0 "/Game/Modular_Asmospheric_Mansion/Materials/Instance/Alternatives/MI_Tiles_03.MI_Tiles_03"))
    (:NewEnumerator7
      (Rendering|Material|SetMaterial Input 0 "/Game/Modular_Asmospheric_Mansion/Materials/Instance/Alternatives/MI_Tiles_02.MI_Tiles_02"))
    (:NewEnumerator8
      (Rendering|Material|SetMaterial Input 0 "/Game/Modular_Asmospheric_Mansion/Materials/Instance/Alternatives/MI_Tiles_01.MI_Tiles_01"))
    (:NewEnumerator9
      (Rendering|Material|SetMaterial Input 0 "/Game/Modular_Asmospheric_Mansion/Materials/Instance/Alternatives/MI_Outer_Wall_Tile_04.MI_Outer_Wall_Tile_04"))
    (:NewEnumerator10
      (Rendering|Material|SetMaterial Input 0 "/Game/Modular_Asmospheric_Mansion/Materials/Instance/Alternatives/MI_Outer_Wall_Tile_03.MI_Outer_Wall_Tile_03"))
    (:NewEnumerator11
      (Rendering|Material|SetMaterial Input 0 "/Game/Modular_Asmospheric_Mansion/Materials/Instance/Alternatives/MI_Outer_Wall_Tile_02.MI_Outer_Wall_Tile_02"))))

(fn INDEX1MATFUNC
  (params (Input :type Primitive%20Component%20Object%20Reference))
  ;[0 0 0] STYLE A
  (switch Utilities|FlowControl|Switch|SwitchonE_Wall_Inner_Materials (Variables|Default|GetIndex%201%20Mat%20Type)
    (:NewEnumerator0
      (Rendering|Material|SetMaterial Input 1 "/Game/Modular_Asmospheric_Mansion/Materials/Instance/MI_weathered_brown_planks.MI_weathered_brown_planks"))
    (:NewEnumerator1
      (Rendering|Material|SetMaterial Input 1 "/Game/Modular_Asmospheric_Mansion/Materials/Instance/Alternatives/MI_Wallpaper_3.MI_Wallpaper_3"))
    (:NewEnumerator2
      (Rendering|Material|SetMaterial Input 1 "/Game/Modular_Asmospheric_Mansion/Materials/Instance/Alternatives/MI_Wallpaper_2.MI_Wallpaper_2"))
    (:NewEnumerator3
      (Rendering|Material|SetMaterial Input 1 "/Game/Modular_Asmospheric_Mansion/Materials/Instance/Alternatives/MI_Wallpaper_1.MI_Wallpaper_1"))
    (:NewEnumerator4
      (Rendering|Material|SetMaterial Input 1 "/Game/Modular_Asmospheric_Mansion/Materials/Instance/Alternatives/MI_Tiles_05.MI_Tiles_05"))
    (:NewEnumerator5
      (Rendering|Material|SetMaterial Input 1 "/Game/Modular_Asmospheric_Mansion/Materials/Instance/Alternatives/MI_Tiles_04.MI_Tiles_04"))
    (:NewEnumerator6
      (Rendering|Material|SetMaterial Input 1 "/Game/Modular_Asmospheric_Mansion/Materials/Instance/Alternatives/MI_Tiles_03.MI_Tiles_03"))
    (:NewEnumerator7
      (Rendering|Material|SetMaterial Input 1 "/Game/Modular_Asmospheric_Mansion/Materials/Instance/Alternatives/MI_Tiles_02.MI_Tiles_02"))
    (:NewEnumerator8
      (Rendering|Material|SetMaterial Input 1 "/Game/Modular_Asmospheric_Mansion/Materials/Instance/Alternatives/MI_Tiles_01.MI_Tiles_01"))
    (:NewEnumerator9
      (Rendering|Material|SetMaterial Input 1 "/Game/Modular_Asmospheric_Mansion/Materials/Instance/Alternatives/MI_Outer_Wall_Tile_04.MI_Outer_Wall_Tile_04"))
    (:NewEnumerator10
      (Rendering|Material|SetMaterial Input 1 "/Game/Modular_Asmospheric_Mansion/Materials/Instance/Alternatives/MI_Outer_Wall_Tile_03.MI_Outer_Wall_Tile_03"))
    (:NewEnumerator11
      (Rendering|Material|SetMaterial Input 1 "/Game/Modular_Asmospheric_Mansion/Materials/Instance/Alternatives/MI_Outer_Wall_Tile_02.MI_Outer_Wall_Tile_02"))))

(fn ChangeMatStyleFunctionIndex0
  (params (InputPin_1 :type Primitive%20Component%20Object%20Reference) (InputPin_2 :type Primitive%20Component%20Object%20Reference) (InputPin_3 :type Primitive%20Component%20Object%20Reference))
  (Utilities|FlowControl|Sequence
    (:then_0
      (CallFunction|MASTERCHANGEMATFUNCFORINDEX0 InputPin_1))
    (:then_1
      (CallFunction|MASTERCHANGEMATFUNCFORINDEX0 InputPin_2))
    (:then_2
      (CallFunction|MASTERCHANGEMATFUNCFORINDEX0 InputPin_3))))

(fn ChangeMatStyleFunctionIndex1
  (params (InputPin_1 :type Primitive%20Component%20Object%20Reference) (InputPin_2 :type Primitive%20Component%20Object%20Reference) (InputPin_3 :type Primitive%20Component%20Object%20Reference))
  (Utilities|FlowControl|Sequence
    (:then_0
      (CallFunction|MASTERCHANGEMATFUNCFORINDEX1 InputPin_1))
    (:then_1
      (CallFunction|MASTERCHANGEMATFUNCFORINDEX1 InputPin_2))
    (:then_2
      (CallFunction|MASTERCHANGEMATFUNCFORINDEX1 InputPin_3))))

(fn MASTERCHANGEMATFUNCFORINDEX1
  (params (InputPin :type Primitive%20Component%20Object%20Reference))
  (switch Utilities|FlowControl|Switch|SwitchonE_Style (Variables|INNERWALLS|GetSTYLE)
    (:NewEnumerator0
      (CallFunction|INDEX1MATFUNC InputPin))
    (:NewEnumerator1
      (CallFunction|INDEX1MATFUNC InputPin))
    (:NewEnumerator2
      (CallFunction|INDEX1MATFUNC InputPin))))

(fn MasterChangeMat
  (params (Target%20A%20Index%200 :type Primitive%20Component%20Object%20Reference) (Target%20B%20Index%200 :type Primitive%20Component%20Object%20Reference) (Target%20C%20Index%200 :type Primitive%20Component%20Object%20Reference) (Target%20A2%20Index1 :type Primitive%20Component%20Object%20Reference) (Target%20B2%20Index1 :type Primitive%20Component%20Object%20Reference) (Target%20C2%20Index1 :type Primitive%20Component%20Object%20Reference))
  (if (Variables|Default|Get1-Change%20Material%20?)
    (CallFunction|ChangeMatStyleFunctionIndex0 Target%20A%20Index%200 Target%20B%20Index%200 Target%20C%20Index%200)
    (CallFunction|ChangeMatStyleFunctionIndex1 Target%20A2%20Index1 Target%20B2%20Index1 Target%20C2%20Index1)))

(fn ChangeMatParameters
  (params (PaintColor_Change :type Linear%20Color%20Structure :default "(R=1.000000,G=1.000000,B=1.000000,A=1.000000)") (Paint%20Density :type Float%20%28single-precision%29) (Paint%20Contrast :type Float%20%28single-precision%29) (Desaturation :type Float%20%28single-precision%29) (Target :type Array%20of%20Mesh%20Component%20Object%20References))
  (Rendering|Material|SetScalarParameterValueonMaterials Target "Paint_Intensity" Paint%20Density)
  (Rendering|Material|SetVectorParameterValueonMaterials Target "PaintColor" (Math|Conversions|ToVector(LinearColor) PaintColor_Change))
  (Rendering|Material|SetScalarParameterValueonMaterials Target "Paint_Contrast" Paint%20Contrast)
  (Rendering|Material|SetScalarParameterValueonMaterials Target "Desaturation" Desaturation))

(fn PaintattribFunc
  (params ([0] :type Array%20of%20Mesh%20Component%20Object%20References))
  (if (Variables|PaintAttributes|GetPaint%20Active%20?)
    (CallFunction|ChangeMatParameters (Variables|PaintAttributes|GetPaint%20Color%20Change) (Variables|PaintAttributes|GetPaint%20Density) (Variables|PaintAttributes|GetPaint%20Contrast) (Variables|PaintAttributes|GetDesaturation) [0])))