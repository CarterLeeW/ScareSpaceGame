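; Modular mansion stairs actor that lets one Blueprint serve as any of several inner or outer stair and handrail pieces.
; The Construction Script uses a bool and two type enums to assign the chosen mesh to its dedicated component and make it visible.
; When PaintActive is set, it pushes paint color, intensity, contrast and desaturation to the materials of that set's components.
; BeginPlay calls FSetCollision on the root and all descendants.
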(event EventBeginPlay
  (CallFunction|FSetCollision (Variables|Default|GetDefaultSceneRoot) true))

(event Collision|EventActorBeginOverlap
  (params (OtherActor :type Actor%20Object%20Reference)))

(event EventTick
  (params (DeltaSeconds :type Float%20%28single-precision%29)))

(fn ConstructionScript
  (bind _sm_inner_stairs_handrail_01_a (Variables|Default|GetSM_inner_stairs_handrail_01_A))
  (bind _sm_inner_stairs_handrail_01_b (Variables|Default|GetSM_inner_stairs_handrail_01_B))
  (bind _sm_inner_stairs_handrail_01_c (Variables|Default|GetSM_inner_stairs_handrail_01_C))
  (bind _sm_inner_stairs_handrail_02_a (Variables|Default|GetSM_inner_stairs_handrail_02_A))
  (bind _sm_inner_stairs_handrail_02_b (Variables|Default|GetSM_inner_stairs_handrail_02_B))
  (bind _sm_inner_stairs_handrail_02_c (Variables|Default|GetSM_inner_stairs_handrail_02_C))
  (bind _sm_inner_stairs_handrail_03_a (Variables|Default|GetSM_inner_stairs_handrail_03_A))
  (bind _sm_inner_stairs_handrail_03_b (Variables|Default|GetSM_inner_stairs_handrail_03_B))
  (bind _sm_inner_stairs_top_ceiling (Variables|Default|GetSM_inner_stairs_top_ceiling))
  (bind _sm_outer_stairs_01 (Variables|Default|GetSM_outer_stairs_01))
  (bind _sm_outer_stairs_02 (Variables|Default|GetSM_outer_stairs_02))
  (bind _sm_outer_stairs_w_handrail_01 (Variables|Default|GetSM_outer_stairs_w_handrail_01))
  (bind _sm_outer_stairs_w_handrail_02 (Variables|Default|GetSM_outer_stairs_w_handrail_02))
  (bind _sm_wood_handrail_01 (Variables|Default|GetSM_wood_handrail_01))
  (bind _sm_wood_handrail_02 (Variables|Default|GetSM_wood_handrail_02))
  (bind _sm_wood_handrail_03 (Variables|Default|GetSM_wood_handrail_03))
  (bind _sm_inner_stairs_01_a (Variables|Default|GetSM_inner_stairs_01_A))
  (bind _sm_inner_stairs_01_b (Variables|Default|GetSM_inner_stairs_01_B))
  (if (Variables|Default|GetInner%20or%20Outer%20Stairs%20?)
    (switch Utilities|FlowControl|Switch|SwitchonE_Stairs_InnerTypes (Variables|Default|GetInnerTypes)
      (:NewEnumerator0
        _)
      (:NewEnumerator1
        _)
      (:NewEnumerator2
        _)
      (:NewEnumerator3
        _)
      (:NewEnumerator4
        _)
      (:NewEnumerator5
        _)
      (:NewEnumerator6
        _)
      (:NewEnumerator7
        _)
      (:NewEnumerator8
        _)
      (:NewEnumerator9
        _)
      (:NewEnumerator10
        _))
    (CallFunction|SetMeshInnerFunction _sm_inner_stairs_01_a _sm_inner_stairs_01_b _sm_inner_stairs_handrail_01_a _sm_inner_stairs_handrail_01_b _sm_inner_stairs_handrail_01_c _sm_inner_stairs_handrail_02_a _sm_inner_stairs_handrail_02_b _sm_inner_stairs_handrail_02_c _sm_inner_stairs_handrail_03_a _sm_inner_stairs_handrail_03_b _sm_inner_stairs_top_ceiling "/Game/Modular_Asmospheric_Mansion/Meshes/Stairs/SM_inner_stairs_01_A.SM_inner_stairs_01_A" "/Game/Modular_Asmospheric_Mansion/Meshes/Stairs/SM_inner_stairs_01_B.SM_inner_stairs_01_B" "/Game/Modular_Asmospheric_Mansion/Meshes/Stairs/SM_inner_stairs_handrail_01_A.SM_inner_stairs_handrail_01_A" "/Game/Modular_Asmospheric_Mansion/Meshes/Stairs/SM_inner_stairs_handrail_01_B.SM_inner_stairs_handrail_01_B" "/Game/Modular_Asmospheric_Mansion/Meshes/Stairs/SM_inner_stairs_handrail_01_C.SM_inner_stairs_handrail_01_C" "/Game/Modular_Asmospheric_Mansion/Meshes/Stairs/SM_inner_stairs_handrail_02_A.SM_inner_stairs_handrail_02_A" "/Game/Modular_Asmospheric_Mansion/Meshes/Stairs/SM_inner_stairs_handrail_02_B.SM_inner_stairs_handrail_02_B" "/Game/Modular_Asmospheric_Mansion/Meshes/Stairs/SM_inner_stairs_handrail_02_C.SM_inner_stairs_handrail_02_C" "/Game/Modular_Asmospheric_Mansion/Meshes/Stairs/SM_inner_stairs_handrail_03_A.SM_inner_stairs_handrail_03_A" "/Game/Modular_Asmospheric_Mansion/Meshes/Stairs/SM_inner_stairs_handrail_03_B.SM_inner_stairs_handrail_03_B" "/Game/Modular_Asmospheric_Mansion/Meshes/Stairs/SM_inner_stairs_top_ceiling.SM_inner_stairs_top_ceiling")
    (CallFunction|PaintattribFunc (Utilities|Array|MakeArray _sm_inner_stairs_01_a _sm_inner_stairs_01_b _sm_inner_stairs_handrail_01_a _sm_inner_stairs_handrail_01_b _sm_inner_stairs_handrail_01_c _sm_inner_stairs_handrail_02_a _sm_inner_stairs_handrail_02_b _sm_inner_stairs_handrail_02_c _sm_inner_stairs_handrail_03_a _sm_inner_stairs_handrail_03_b _sm_inner_stairs_top_ceiling))
    (else
      (switch Utilities|FlowControl|Switch|SwitchonE_Stairs_OuterTypes (Variables|Default|GetOuterTypes)
        (:NewEnumerator0
          _)
        (:NewEnumerator1
          _)
        (:NewEnumerator2
          _)
        (:NewEnumerator3
          _)
        (:NewEnumerator4
          _)
        (:NewEnumerator5
          _)
        (:NewEnumerator6
          _))
      (CallFunction|SetMeshOuterFunction _sm_outer_stairs_01 _sm_outer_stairs_02 _sm_outer_stairs_w_handrail_01 _sm_outer_stairs_w_handrail_02 _sm_wood_handrail_01 _sm_wood_handrail_02 _sm_wood_handrail_03 0 0 0 0 "/Game/Modular_Asmospheric_Mansion/Meshes/Stairs/SM_outer_stairs_01.SM_outer_stairs_01" "/Game/Modular_Asmospheric_Mansion/Meshes/Stairs/SM_outer_stairs_02.SM_outer_stairs_02" "/Game/Modular_Asmospheric_Mansion/Meshes/Stairs/SM_outer_stairs_w_handrail_01.SM_outer_stairs_w_handrail_01" "/Game/Modular_Asmospheric_Mansion/Meshes/Stairs/SM_outer_stairs_w_handrail_02.SM_outer_stairs_w_handrail_02" "/Game/Modular_Asmospheric_Mansion/Meshes/Stairs/SM_wood_handrail_01.SM_wood_handrail_01" "/Game/Modular_Asmospheric_Mansion/Meshes/Stairs/SM_wood_handrail_02.SM_wood_handrail_02" "/Game/Modular_Asmospheric_Mansion/Meshes/Stairs/SM_wood_handrail_03.SM_wood_handrail_03")
      (CallFunction|PaintattribFunc (Utilities|Array|MakeArray _sm_outer_stairs_01 _sm_outer_stairs_02 _sm_outer_stairs_w_handrail_01 _sm_outer_stairs_w_handrail_02 _sm_wood_handrail_01 _sm_wood_handrail_02 _sm_wood_handrail_03 0 0 0 0)))))

(fn SetMeshInnerFunction
  (params (1 :type Static%20Mesh%20Component%20Object%20Reference) (2 :type Static%20Mesh%20Component%20Object%20Reference) (3 :type Static%20Mesh%20Component%20Object%20Reference) (4 :type Static%20Mesh%20Component%20Object%20Reference) (5 :type Static%20Mesh%20Component%20Object%20Reference) (6 :type Static%20Mesh%20Component%20Object%20Reference) (7 :type Static%20Mesh%20Component%20Object%20Reference) (8 :type Static%20Mesh%20Component%20Object%20Reference) (9 :type Static%20Mesh%20Component%20Object%20Reference) (10 :type Static%20Mesh%20Component%20Object%20Reference) (11 :type Static%20Mesh%20Component%20Object%20Reference) (MESH%201 :type Static%20Mesh%20Object%20Reference) (MESH%202 :type Static%20Mesh%20Object%20Reference) (MESH%203 :type Static%20Mesh%20Object%20Reference) (MESH%204 :type Static%20Mesh%20Object%20Reference) (MESH%205 :type Static%20Mesh%20Object%20Reference) (MESH%206 :type Static%20Mesh%20Object%20Reference) (MESH%207 :type Static%20Mesh%20Object%20Reference) (MESH%208 :type Static%20Mesh%20Object%20Reference) (MESH%209 :type Static%20Mesh%20Object%20Reference) (MESH%2010 :type Static%20Mesh%20Object%20Reference) (MESH%2011 :type Static%20Mesh%20Object%20Reference))
  (switch Utilities|FlowControl|Switch|SwitchonE_Stairs_InnerTypes (Variables|Default|GetInnerTypes)
    (:NewEnumerator0
      (Components|StaticMesh|SetStaticMesh 1 MESH%201)
      (Rendering|SetVisibility 1 true false)
      (return))
    (:NewEnumerator1
      (Components|StaticMesh|SetStaticMesh 2 MESH%202)
      (Rendering|SetVisibility 2 true false)
      (return))
    (:NewEnumerator2
      (Components|StaticMesh|SetStaticMesh 3 MESH%203)
      (Rendering|SetVisibility 3 true false)
      (return))
    (:NewEnumerator3
      (Components|StaticMesh|SetStaticMesh 4 MESH%204)
      (Rendering|SetVisibility 4 true false)
      (return))
    (:NewEnumerator4
      (Components|StaticMesh|SetStaticMesh 5 MESH%205)
      (Rendering|SetVisibility 5 true false)
      (return))
    (:NewEnumerator5
      (Components|StaticMesh|SetStaticMesh 6 MESH%206)
      (Rendering|SetVisibility 6 true false)
      (return))
    (:NewEnumerator6
      (Components|StaticMesh|SetStaticMesh 7 MESH%207)
      (Rendering|SetVisibility 7 true false)
      (return))
    (:NewEnumerator7
      (Components|StaticMesh|SetStaticMesh 8 MESH%208)
      (Rendering|SetVisibility 8 true false))
    (:NewEnumerator8
      (Components|StaticMesh|SetStaticMesh 9 MESH%209)
      (Rendering|SetVisibility 9 true false))
    (:NewEnumerator9
      (Components|StaticMesh|SetStaticMesh 10 MESH%2010)
      (Rendering|SetVisibility 10 true false))
    (:NewEnumerator10
      (Components|StaticMesh|SetStaticMesh 11 MESH%2011)
      (Rendering|SetVisibility 11 true false))))

(fn ChangeMatParameters
  (params (PaintColor_Change :type Linear%20Color%20Structure :default "(R=1.000000,G=1.000000,B=1.000000,A=1.000000)") (Paint%20Density :type Float%20%28single-precision%29) (Paint%20Contrast :type Float%20%28single-precision%29) (Desaturation :type Float%20%28single-precision%29) (Target :type Array%20of%20Mesh%20Component%20Object%20References))
  (Rendering|Material|SetScalarParameterValueonMaterials Target "Paint_Intensity" Paint%20Density)
  (Rendering|Material|SetVectorParameterValueonMaterials Target "PaintColor" (Math|Conversions|ToVector(LinearColor) PaintColor_Change))
  (Rendering|Material|SetScalarParameterValueonMaterials Target "Paint_Contrast" Paint%20Contrast)
  (Rendering|Material|SetScalarParameterValueonMaterials Target "Desaturation" Desaturation))

(fn PaintattribFunc
  (params ([0] :type Array%20of%20Mesh%20Component%20Object%20References))
  (if (Variables|PaintAttrib|GetPaint%20Active%20?)
    (CallFunction|ChangeMatParameters (Variables|PaintAttrib|GetPaint%20Color%20Change) (Variables|PaintAttrib|GetPaint%20Density) (Variables|PaintAttrib|GetPaint%20Contrast) (Variables|PaintAttrib|GetDesaturation) [0])))

(fn SetMeshOuterFunction
  (params (1 :type Static%20Mesh%20Component%20Object%20Reference) (2 :type Static%20Mesh%20Component%20Object%20Reference) (3 :type Static%20Mesh%20Component%20Object%20Reference) (4 :type Static%20Mesh%20Component%20Object%20Reference) (5 :type Static%20Mesh%20Component%20Object%20Reference) (6 :type Static%20Mesh%20Component%20Object%20Reference) (7 :type Static%20Mesh%20Component%20Object%20Reference) (8 :type Static%20Mesh%20Component%20Object%20Reference) (9 :type Static%20Mesh%20Component%20Object%20Reference) (10 :type Static%20Mesh%20Component%20Object%20Reference) (11 :type Static%20Mesh%20Component%20Object%20Reference) (MESH%201 :type Static%20Mesh%20Object%20Reference) (MESH%202 :type Static%20Mesh%20Object%20Reference) (MESH%203 :type Static%20Mesh%20Object%20Reference) (MESH%204 :type Static%20Mesh%20Object%20Reference) (MESH%205 :type Static%20Mesh%20Object%20Reference) (MESH%206 :type Static%20Mesh%20Object%20Reference) (MESH%207 :type Static%20Mesh%20Object%20Reference) (MESH%208 :type Static%20Mesh%20Object%20Reference) (MESH%209 :type Static%20Mesh%20Object%20Reference) (MESH%2010 :type Static%20Mesh%20Object%20Reference) (MESH%2011 :type Static%20Mesh%20Object%20Reference))
  (switch Utilities|FlowControl|Switch|SwitchonE_Stairs_OuterTypes (Variables|Default|GetOuterTypes)
    (:NewEnumerator0
      (Components|StaticMesh|SetStaticMesh 1 MESH%201)
      (Rendering|SetVisibility 1 true false))
    (:NewEnumerator1
      (Components|StaticMesh|SetStaticMesh 2 MESH%202)
      (Rendering|SetVisibility 2 true false))
    (:NewEnumerator2
      (Components|StaticMesh|SetStaticMesh 3 MESH%203)
      (Rendering|SetVisibility 3 true false))
    (:NewEnumerator3
      (Components|StaticMesh|SetStaticMesh 4 MESH%204)
      (Rendering|SetVisibility 4 true false))
    (:NewEnumerator4
      (Components|StaticMesh|SetStaticMesh 5 MESH%205)
      (Rendering|SetVisibility 5 true false))
    (:NewEnumerator5
      (Components|StaticMesh|SetStaticMesh 6 MESH%206)
      (Rendering|SetVisibility 6 true false))
    (:NewEnumerator6
      (Components|StaticMesh|SetStaticMesh 7 MESH%207)
      (Rendering|SetVisibility 7 true false)))
  (return))