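; Double basement gate with physics-driven pivotable doors, kept locked until the story reaches the AnswerPhone1 phase or the generator is first interacted with.
; On BeginPlay both leaves take their lock state from the linear story progression subsystem's current phase.
; The generator's first interaction unlocks both, then a physics workaround zeroes the left constraint's angular drive, torques that leaf open and blocks closing for a second.
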(event OnFirstInteractionOccured(Generator)
  (bind _leftpivotable (Variables|Default|GetLeftPivotable))
  ;[0.15 0.15 0.15 0.5] Just awful patchwork fix for the physics engine
  (Variables|/Script/ScareSpace.PivotableComponent|SetbIsLocked (Variables|Default|GetLeftPivotable) false)
  (Variables|/Script/ScareSpace.PivotableComponent|SetbIsLocked (Variables|Default|GetRightPivotable) false)
  (Variables|/Script/ScareSpace.PivotableComponent|SetbCanClose _leftpivotable false)
  (Variables|/Script/ScareSpace.PivotableComponent|SetbIsClosed _leftpivotable false)
  (Class|PhysicsConstraintComponent|SetAngularDriveParams (Variables|Default|GetLeftPhysicsConstraint) 0.0 0.0 0.0)
  (Class|PrimitiveComponent|AddTorqueinDegrees (Variables|Default|GetLeftDoorMesh) "0.000000,-5000.000000,0.000000" "None" true)
  (Utilities|FlowControl|Delay 1.0)
  (Variables|/Script/ScareSpace.PivotableComponent|SetbCanClose (Variables|Default|GetLeftPivotable) true))

(event EventBeginPlay
  (bind _returnvalue (Utilities|Enum|LiteralenumEStoryPhase "AnswerPhone1"))
  (bind _returnvalue_2 (Subsystems|GetLinearStoryProgressionSubsystem))
  (bind _returnvalue_3 (Class|LinearStoryProgressionSubsystem|GetCurrentPhase _returnvalue_2))
  (bind _returnvalue_4 (Math|Conversions|ToInteger(Byte) _returnvalue))
  (bind _returnvalue_5 (< _returnvalue_3 _returnvalue_4))
  (Variables|/Script/ScareSpace.PivotableComponent|SetbIsLocked (Variables|Default|GetLeftPivotable) _returnvalue_5)
  (Variables|/Script/ScareSpace.PivotableComponent|SetbIsLocked (Variables|Default|GetRightPivotable) _returnvalue_5))

(fn ConstructionScript
  (|CallParentFunction))