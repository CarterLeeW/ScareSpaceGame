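; Garage fence gate that swings open and shut automatically as BP_Nomad_Character enters and leaves OldManTrigger.
; After a short delay on entry, OpenGate unlocks the Pivotable, zeroes the PhysicsConstraint's angular drive and torques DoorMesh open, re-allowing closing a second later.
; On exit, CloseGate allows closing and applies an opposing torque, so motion is physics-driven rather than animated.
; An unconnected timed open/close sequence never runs.
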(event OnComponentBeginOverlap(OldManTrigger)
  (params (OverlappedComponent :type Primitive%20Component%20Object%20Reference) (OtherActor :type Actor%20Object%20Reference) (OtherComp :type Primitive%20Component%20Object%20Reference) (OtherBodyIndex :type Integer) (bFromSweep :type Boolean) (SweepResult :type Hit%20Result%20Structure%20%28by%20ref%29))
  (Utilities|Casting|CastToBP_Nomad_Character OtherActor)
  (Utilities|FlowControl|Delay 0.5)
  (CallFunction|OpenGate))

(event OnComponentEndOverlap(OldManTrigger)
  (params (OverlappedComponent :type Primitive%20Component%20Object%20Reference) (OtherActor :type Actor%20Object%20Reference) (OtherComp :type Primitive%20Component%20Object%20Reference) (OtherBodyIndex :type Integer))
  (Utilities|Casting|CastToBP_Nomad_Character OtherActor)
  (CallFunction|CloseGate))

(event Custom|Open%20Gate
  (bind _pivotable (Variables|Default|GetPivotable))
  (Variables|/Script/ScareSpace.PivotableComponent|SetbIsLocked _pivotable false)
  (Variables|/Script/ScareSpace.PivotableComponent|SetbCanClose _pivotable false)
  (Variables|/Script/ScareSpace.PivotableComponent|SetbIsClosed _pivotable false)
  (Class|PhysicsConstraintComponent|SetAngularDriveParams (Variables|Default|GetPhysicsConstraint) 0.0 0.0 0.0)
  (Class|PrimitiveComponent|AddTorqueinDegrees (Variables|Default|GetDoorMesh) "-5000000.000000,-5000.000000,0.000000" "None" true)
  (Utilities|FlowControl|Delay 1.0)
  (Variables|/Script/ScareSpace.PivotableComponent|SetbCanClose (Variables|Default|GetPivotable) true))

(event Custom|Close%20Gate
  (Variables|/Script/ScareSpace.PivotableComponent|SetbCanClose (Variables|Default|GetPivotable) true)
  (Class|PrimitiveComponent|AddTorqueinDegrees (Variables|Default|GetDoorMesh) "500000.000000,500000.000000,0.000000" "None" true))

(event EventBeginPlay
  (|CallParentFunction))

(event Collision|EventActorBeginOverlap
  (params (OtherActor :type Actor%20Object%20Reference))
  (|CallParentFunction OtherActor) ; This node is disabled and will not be called.\nDrag off pins to build functionality.
)

(event EventTick
  (params (DeltaSeconds :type Float%20%28single-precision%29))
  (|CallParentFunction DeltaSeconds) ; This node is disabled and will not be called.\nDrag off pins to build functionality.
)

(fn ConstructionScript
  (|CallParentFunction))