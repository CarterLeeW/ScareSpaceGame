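; Double basement gate whose lock state follows linear story progression and a linked generator.
; On BeginPlay, both pivotable leaves lock if the current story phase is earlier than AnswerPhone1.
; The generator's first interaction swings the left leaf partly open, bypassing its lock, and unlocks the right leaf without explicitly clearing the left leaf's lock.
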(event OnFirstInteractionOccured(Generator)
  (Class|SimplePivotableComponent|OpenPivotableProgrammatically (Variables|Default|GetLeftPivotable) 4e+01 5.0 true)
  (Class|SimplePivotableComponent|SetIsLocked (Variables|Default|GetRightPivotable) false))

(event EventBeginPlay
  (bind _returnvalue (Utilities|Enum|LiteralenumEStoryPhase "AnswerPhone1"))
  (bind _returnvalue_2 (Subsystems|GetLinearStoryProgressionSubsystem))
  (bind _returnvalue_3 (Class|LinearStoryProgressionSubsystem|GetCurrentPhase _returnvalue_2))
  (bind _returnvalue_4 (Math|Conversions|ToInteger(Byte) _returnvalue))
  (bind _returnvalue_5 (< _returnvalue_3 _returnvalue_4))
  (Class|SimplePivotableComponent|SetIsLocked (Variables|Default|GetLeftPivotable) _returnvalue_5)
  (Class|SimplePivotableComponent|SetIsLocked (Variables|Default|GetRightPivotable) _returnvalue_5))

(fn ConstructionScript
  (|CallParentFunction))