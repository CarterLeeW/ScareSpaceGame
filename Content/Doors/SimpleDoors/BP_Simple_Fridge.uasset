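; BP_Simple_Fridge is a fridge variant among the simple doors that can carry an attached note on its door.
; Its construction script runs the parent's, then, if AttachedNote is valid, attaches it to DoorMesh with relative transforms kept.
; The event graph holds only disabled default events, so the Blueprint adds no runtime logic of its own.
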(event EventBeginPlay
  (|CallParentFunction) ; This node is disabled and will not be called.\nDrag off pins to build functionality.
)

(event Collision|EventActorBeginOverlap
  (params (OtherActor :type Actor%20Object%20Reference))
  (|CallParentFunction OtherActor) ; This node is disabled and will not be called.\nDrag off pins to build functionality.
)

(event EventTick
  (params (DeltaSeconds :type Float%20%28single-precision%29))
  (|CallParentFunction DeltaSeconds) ; This node is disabled and will not be called.\nDrag off pins to build functionality.
)

(fn ConstructionScript
  (bind _attached_note (Variables|Default|GetAttached%20Note))
  (|CallParentFunction)
  (Utilities|IsValid _attached_note
    (:Is%20Valid
      (Transformation|AttachComponentToComponent _attached_note (Variables|Default|GetDoorMesh) "None" "KeepRelative" "KeepRelative" "KeepRelative" true))))