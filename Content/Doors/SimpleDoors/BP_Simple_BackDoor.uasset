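; BP_Simple_BackDoor is the house back door, adding story journal mementos around unlocking it with a key.
; When interaction begins during the ArriveAtHouse phase while its Pivotable is locked, it adds an unlock memento, plus a get-spare-key memento if the player's inventory lacks the back door key.
; Using an item on the door removes both mementos through the LinearStoryProgressionSubsystem.
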(event OnInteractionBegins(Pivotable)
  (params (Interactor :type Interactor%20Component%20Object%20Reference))
  ;[0.15 0.15 0.15 0.5] Very first part of the game. If locked, add memento to get key from shed
  (if (and (Utilities|Enum|Equal(Enum) (Class|LinearStoryProgressionSubsystem|GetCurrentPhase (Subsystems|GetLinearStoryProgressionSubsystem)) "ArriveAtHouse") (Variables|/Script/ScareSpace.SimplePivotableComponent|GetbIsLocked (Variables|Default|GetPivotable)))
    (Class|LinearStoryProgressionSubsystem|AddJournalEntry (Subsystems|GetLinearStoryProgressionSubsystem) (Variables|Default|GetMemento%20Unlock%20Back%20Door%20Handle))
    ;[0.15 0.15 0.15 0.5] Add memento to get spare key if key isn't already in inventory. Also has to be locked
    (bind _asbp_player_character (Utilities|Casting|CastToBP_PlayerCharacter (Game|GetPlayerCharacter 0)))
    (if (not (Utilities|Array|ContainsItem (Class|InventoryComponent|GetInventoryItems (Variables|/Script/ScareSpace.PlayerCharacter|GetInventoryComponent _asbp_player_character)) (Variables|Default|GetBack%20Door%20Key%20Handle)))
      (Class|LinearStoryProgressionSubsystem|AddJournalEntry (Subsystems|GetLinearStoryProgressionSubsystem) (Variables|Default|GetMemento%20Get%20Spare%20Key%20Handle)))))

(event OnInteractwithItem(Pivotable)
  (params (Interactor :type Interactor%20Component%20Object%20Reference))
  (Class|LinearStoryProgressionSubsystem|RemoveJournalEntry (Subsystems|GetLinearStoryProgressionSubsystem) (Variables|Default|GetMemento%20Unlock%20Back%20Door%20Handle))
  (Class|LinearStoryProgressionSubsystem|RemoveJournalEntry (Subsystems|GetLinearStoryProgressionSubsystem) (Variables|Default|GetMemento%20Get%20Spare%20Key%20Handle)))

(event EventBeginPlay
  (|CallParentFunction) ; This node is disabled and will not be called.\nDrag off pins to build functionality.
)

(event Collision|EventActorBeginOverlap
  (params (OtherActor :type Actor%20Object%20Reference))
  (|CallParentFunction OtherActor) ; This node is disabled and will not be called.\nDrag off pins to build functionality.
)

(event EventTick
  (params (DeltaSeconds :type Float%20%28single-precision%29))
  (|CallParentFunction DeltaSeconds) ; This node is disabled and will not be called.\nDrag off pins to build functionality.
)

(fn ConstructionScript
  (|CallParentFunction))