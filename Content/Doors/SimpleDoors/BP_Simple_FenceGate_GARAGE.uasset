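; BP_Simple_FenceGate_GARAGE is a garage fence gate that opens and closes automatically for the Neighbor character.
; An OldManTrigger volume filters overlaps to BP_Neighbor and, after a short delay, tells the Pivotable component to swing open programmatically, bypassing any lock.
; When the Neighbor leaves the volume, the same Pivotable is closed programmatically.
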(event OnComponentBeginOverlap(OldManTrigger)
  (params (OverlappedComponent :type Primitive%20Component%20Object%20Reference) (OtherActor :type Actor%20Object%20Reference) (OtherComp :type Primitive%20Component%20Object%20Reference) (OtherBodyIndex :type Integer) (bFromSweep :type Boolean) (SweepResult :type Hit%20Result%20Structure%20%28by%20ref%29))
  (Utilities|Casting|CastToBP_Neighbor OtherActor)
  (Utilities|FlowControl|Delay 0.5)
  (Class|SimplePivotableComponent|OpenPivotableProgrammatically (Variables|Default|GetPivotable) 1.1e+02 5.0 true))

(event OnComponentEndOverlap(OldManTrigger)
  (params (OverlappedComponent :type Primitive%20Component%20Object%20Reference) (OtherActor :type Actor%20Object%20Reference) (OtherComp :type Primitive%20Component%20Object%20Reference) (OtherBodyIndex :type Integer))
  (Utilities|Casting|CastToBP_Neighbor OtherActor)
  (Class|SimplePivotableComponent|ClosePivotableProgrammatically (Variables|Default|GetPivotable) 5.0))

(event EventBeginPlay
  (|CallParentFunction) ; This node is disabled and will not be called.\nDrag off pins to build functionality.
)

(event Collision|EventActorBeginOverlap
  (params (OtherActor :type Actor%20Object%20Reference))
  (|CallParentFunction OtherActor) ; This node is disabled and will not be called.\nDrag off pins to build functionality.
)

(event EventTick
  (params (DeltaSeconds :type Float%20%28single-precision%29))
  (|CallParentFunction DeltaSeconds) ; This node is disabled and will not be called.\nDrag off pins to build functionality.
)

(fn ConstructionScript
  (|CallParentFunction))