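; Player character Blueprint that keeps the journal in step with the game's linear story.
; On BeginPlay it binds to the story progression subsystem's phase-advanced event and applies the current phase to set the initial journal state.
; The phase handler clears the journal's mementos, then switches on the phase to add its matching memento, plus Mom's letter note on arrival at the house.
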(event EventBeginPlay
  (EventDispatchers|AssignOnStoryPhaseAdvanced (Subsystems|GetLinearStoryProgressionSubsystem) (EventDispatchers|CreateEvent :!event Journal-StoryPhaseEvent))
  (Journal|Journal-SetStateforPhaseOfGame))

(fn ConstructionScript)

(fn Journal-StoryPhaseEvent
  (params (NewPhase :type EStoryPhase%20Enum :default "ArriveAtHouse"))
  (Class|JournalComponent|ClearMementosfromJournal (Variables|Default|GetJournalComponent))
  (switch Utilities|FlowControl|Switch|SwitchonEStoryPhase NewPhase
    (:ArriveAtHouse
      (Class|JournalComponent|AddItemtoJournal (Variables|Default|GetJournalComponent) (LocalVariables|GetMemento%20First%20Arrival%20Handle))
      (Class|JournalComponent|AddItemtoJournal (Variables|Default|GetJournalComponent) (LocalVariables|GetNote%20Letter%20From%20Mom)))
    (:StartBasementFire
      (Class|JournalComponent|AddItemtoJournal (Variables|Default|GetJournalComponent) (LocalVariables|GetMemento%20Start%20Fire)))
    (:FeedCat
      (Class|JournalComponent|AddItemtoJournal (Variables|Default|GetJournalComponent) (LocalVariables|GetMemento%20Feed%20Cat)))
    (:BringInMail
      (Class|JournalComponent|AddItemtoJournal (Variables|Default|GetJournalComponent) (LocalVariables|GetMemento%20Bring%20in%20Mail)))
    (:GoToBed
      (Class|JournalComponent|AddItemtoJournal (Variables|Default|GetJournalComponent) (LocalVariables|GetMemento%20Go%20To%20Bed)))
    (:GetWater
      (Class|JournalComponent|AddItemtoJournal (Variables|Default|GetJournalComponent) (LocalVariables|GetMemento%20Get%20Water)))
    (:WatchTV
      (Class|JournalComponent|AddItemtoJournal (Variables|Default|GetJournalComponent) (LocalVariables|GetMemento%20Watch%20TV)))
    (:StartGenerator
      (Class|JournalComponent|AddItemtoJournal (Variables|Default|GetJournalComponent) (LocalVariables|GetMemento%20Start%20Generator)))
    (:AnswerPhone1
      (Class|JournalComponent|AddItemtoJournal (Variables|Default|GetJournalComponent) (LocalVariables|GetMemento%20Answer%20Phone%201)))
    (:FindCabinetKey
      (Class|JournalComponent|AddItemtoJournal (Variables|Default|GetJournalComponent) (LocalVariables|GetMemento%20Find%20Cabinet%20Key)))))

(fn Journal-SetStateforPhaseOfGame
  (Journal|Journal-StoryPhaseEvent (Class|LinearStoryProgressionSubsystem|GetCurrentPhase (Subsystems|GetLinearStoryProgressionSubsystem))))