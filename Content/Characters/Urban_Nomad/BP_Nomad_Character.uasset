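; Urban Nomad NPC character that can walk away through two target points and then remove itself from the level.
; The walk-away event uses AI MoveTo to reach the first target, then calls itself for the second and destroys the actor shortly after arrival.
; A lifetime timer started after the first leg also destroys it.
; Helper functions forward head look-at and tracking changes to its Animation Blueprint.
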(event Custom|Start%20Walking%20Away%20Sequence
  (params (First%20Destination :type Boolean))
  (bind _asab_urban_nomad (Utilities|Casting|CastToAB_Urban_Nomad (Components|SkeletalMesh|GetAnimInstance (Variables|Character|GetMesh))))
  (AI|AIMoveTo _asab_urban_nomad self (Math|Vector|SelectVector (Transformation|GetActorLocation (Variables|Default|GetFirst%20Walk%20Away%20Target)) (Transformation|GetActorLocation (Variables|Default|GetSecond%20Walk%20Away%20Target)) First%20Destination) 0 5e+01 false
    (:OnSuccess
      (if First%20Destination
        (Utilities|FlowControl|Delay 1.0)
        (CallFunction|StartWalkingAwaySequence false)
        (CallFunction|SetActorLife 6e+01)
        (else
          (Utilities|FlowControl|Delay 5.0)
          (Actor|DestroyActor))))))

(event Custom|Set%20Actor%20Life
  (params (Life%20in%20Seconds :type Float%20%28double-precision%29))
  (Utilities|FlowControl|Delay Life%20in%20Seconds)
  (Actor|DestroyActor))

(event EventBeginPlay)

(event Collision|EventActorBeginOverlap
  (params (OtherActor :type Actor%20Object%20Reference)))

(event EventTick
  (params (DeltaSeconds :type Float%20%28single-precision%29)))

(fn ConstructionScript)

(fn ChangeLookatTarget
  (params (Target%20Location :type Vector%20%28by%20ref%29) (Enable%20Tracking :type Boolean))
  (bind _asab_urban_nomad (Utilities|Casting|CastToAB_Urban_Nomad (Components|SkeletalMesh|GetAnimInstance (Variables|Character|GetMesh))))
  (Default|UpdateHeadLookat _asab_urban_nomad Target%20Location Enable%20Tracking))

(fn DisableHeadTracking
  (bind _asab_urban_nomad (Utilities|Casting|CastToAB_Urban_Nomad (Components|SkeletalMesh|GetAnimInstance (Variables|Character|GetMesh))))
  (Default|DisableHeadTracking _asab_urban_nomad))

(fn UpdateHeadTrackingComponent
  (params (New%20Look%20at%20Component :type Scene%20Component%20Object%20Reference))
  (bind _asab_urban_nomad (Utilities|Casting|CastToAB_Urban_Nomad (Components|SkeletalMesh|GetAnimInstance (Variables|Character|GetMesh))))
  (Default|UpdateHeadTrackingComponent _asab_urban_nomad New%20Look%20at%20Component))