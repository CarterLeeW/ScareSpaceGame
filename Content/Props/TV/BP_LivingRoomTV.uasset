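; Living room TV prop that plays a video when the player interacts with it during the WatchTV story phase.
; It enables its simple interactable component only in that phase, checked on BeginPlay and on each phase change from the linear story progression subsystem.
; Interacting opens the media source, shows the screen mesh after a short delay and disables further interaction.
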(event OnInteracted(BP_SimpleInteractableComponent)
  (params (Interactor :type Interactor%20Component%20Object%20Reference))
  (Variables|Default|SetIsTVOn true)
  (Media|MediaPlayer|OpenSource (Variables|Default|GetTVMedia) "/Game/Movies/Living_Dead_LQ.Living_Dead_LQ")
  (Utilities|FlowControl|Delay 0.3)
  (Rendering|SetVisibility (Variables|Default|GetTV%20Screen) true false)
  (Variables|/Script/ScareSpace.InteractableComponent|SetbCanInteract (Variables|Default|GetBP_SimpleInteractableComponent) false))

(event Custom|OnStoryPhaseAdvanced_Event
  (params (NewPhase :type EStoryPhase%20Enum :default "ArriveAtHouse"))
  (Variables|/Script/ScareSpace.InteractableComponent|SetbCanInteract (Variables|Default|GetBP_SimpleInteractableComponent) (Utilities|Enum|Equal(Enum) NewPhase "WatchTV")))

(event EventBeginPlay
  (Variables|/Script/ScareSpace.InteractableComponent|SetbCanInteract (Variables|Default|GetBP_SimpleInteractableComponent) (Utilities|Enum|Equal(Enum) (Class|LinearStoryProgressionSubsystem|GetCurrentPhase (Subsystems|GetLinearStoryProgressionSubsystem)) "WatchTV"))
  (EventDispatchers|AssignOnStoryPhaseAdvanced (Subsystems|GetLinearStoryProgressionSubsystem) (delegate Custom|OnStoryPhaseAdvanced_Event)))

(fn ConstructionScript)