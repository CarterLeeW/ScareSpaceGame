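; Guest bathroom sink prop the player uses to brush teeth during the GoToBed story phase.
; A simple interactable component is enabled only while the linear story progression subsystem reports that phase, checked at BeginPlay and on each phase change.
; On interaction, it adds a "teeth_brushed" tag to the interactor's component tags and disables further interaction.
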(event OnInteracted(BP_SimpleInteractableComponent)
  (params (Interactor :type Interactor%20Component%20Object%20Reference))
  (Utilities|Array|Add (Variables|/Script/Engine.ActorComponent|GetComponentTags Interactor) "teeth_brushed")
  (Variables|/Script/ScareSpace.InteractableComponent|SetbCanInteract (Variables|Default|GetBP_SimpleInteractableComponent) false))

(event Custom|OnStoryPhaseAdvanced_Event
  (params (NewPhase :type EStoryPhase%20Enum :default "ArriveAtHouse"))
  (Variables|/Script/ScareSpace.InteractableComponent|SetbCanInteract (Variables|Default|GetBP_SimpleInteractableComponent) (Utilities|Enum|Equal(Enum) NewPhase "GoToBed")))

(event EventBeginPlay
  (Variables|/Script/ScareSpace.InteractableComponent|SetbCanInteract (Variables|Default|GetBP_SimpleInteractableComponent) (Utilities|Enum|Equal(Enum) (Class|LinearStoryProgressionSubsystem|GetCurrentPhase (Subsystems|GetLinearStoryProgressionSubsystem)) "GoToBed"))
  (EventDispatchers|AssignOnStoryPhaseAdvanced (Subsystems|GetLinearStoryProgressionSubsystem) (delegate Custom|OnStoryPhaseAdvanced_Event)))

(fn ConstructionScript)