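; A story telephone prop that rings and plays a dialogue when answered during the two AnswerPhone phases.
; It listens to the LinearStoryProgressionSubsystem to enable interaction, starting the ring sound after a short delay when either phase begins.
; Interacting stops any ringing and starts that phase's dialogue sequence focused on the phone.
; When a dialogue ends, it plays a hang-up sound and advances the story to FindCabinetKey or UnlockSubBasementDoor respectively.
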(event OnInteracted(BP_SimpleInteractableComponent)
  (params (Interactor :type Interactor%20Component%20Object%20Reference))
  (bind _returnvalue (Subsystems|GetLinearStoryProgressionSubsystem))
  (bind _ringingsound (Variables|Default|GetRingingSound))
  (bind _returnvalue_2 (Class|LinearStoryProgressionSubsystem|GetCurrentPhase _returnvalue))
  (Utilities|IsValid _ringingsound
    (:Is%20Valid
      (Audio|Components|Audio|Stop _ringingsound)
      (Variables|Default|SetAnswered true)
      (Audio|PlaySoundatLocation "/Game/Props/Telephone/SW_PhoneHangUp.SW_PhoneHangUp" (Transformation|GetActorLocation) "0, 0, 0" 1.0 1.0 0.0 0 0 0 0))
    (:Is%20Not%20Valid
      _))
  (if (Utilities|Enum|Equal(Enum) _returnvalue_2 "AnswerPhone1")
    (bind _dialogue_object (CallFunction|StartDialogueSequence "/Game/Data/Dialogue/DDA_Telephone_1.DDA_Telephone_1" self))
    (EventDispatchers|AssignDialogueEnds _dialogue_object (delegate Custom|Dialogue%201%20Ends))
    (Variables|/Script/ScareSpace.InteractableComponent|SetbCanInteract (Variables|Default|GetBP_SimpleInteractableComponent) false)
    (elif (Utilities|Enum|Equal(Enum) _returnvalue_2 "AnswerPhone2")
      (bind _dialogue_object_2 (CallFunction|StartDialogueSequence "/Game/Data/Dialogue/DDA_Telephone_2.DDA_Telephone_2" self))
      (EventDispatchers|AssignDialogueEnds _dialogue_object_2 (delegate Custom|Dialogue%202%20Ends)))))

(event Custom|OnStoryPhaseAdvanced_Event
  (params (NewPhase :type EStoryPhase%20Enum :default "ArriveAtHouse"))
  (bind _returnvalue (Utilities|Enum|Equal(Enum) NewPhase "AnswerPhone1"))
  (bind _returnvalue_2 (Utilities|Enum|Equal(Enum) NewPhase "AnswerPhone2"))
  (bind _returnvalue_3 (or _returnvalue _returnvalue_2))
  (Variables|/Script/ScareSpace.InteractableComponent|SetbCanInteract (Variables|Default|GetBP_SimpleInteractableComponent) _returnvalue_3)
  (if _returnvalue_3
    (Utilities|FlowControl|Delay 5.0)
    (bind _returnvalue_4 (Audio|SpawnSoundatLocation "/Game/Props/Telephone/MSS_Phone.MSS_Phone" (Transformation|GetActorLocation) "0, 0, 0" 1.0 1.0 0.0 0 0))
    (Variables|Default|SetRingingSound _returnvalue_4)
    (Variables|Default|SetAnswered false)))

(event Custom|Dialogue%201%20Ends
  (Audio|PlaySoundatLocation "/Game/Props/Telephone/SW_PhoneHangUp.SW_PhoneHangUp" (Transformation|GetActorLocation) "0, 0, 0" 1.0 1.0 0.0 0 0 0 0)
  (Class|LinearStoryProgressionSubsystem|AdvancetoPhase (Subsystems|GetLinearStoryProgressionSubsystem) "FindCabinetKey"))

(event Custom|Dialogue%202%20Ends
  (Audio|PlaySoundatLocation "/Game/Props/Telephone/SW_PhoneHangUp.SW_PhoneHangUp" (Transformation|GetActorLocation) "0, 0, 0" 1.0 1.0 0.0 0 0 0 0)
  (Class|LinearStoryProgressionSubsystem|AdvancetoPhase (Subsystems|GetLinearStoryProgressionSubsystem) "UnlockSubBasementDoor"))

(event EventBeginPlay
  (bind _returnvalue (Subsystems|GetLinearStoryProgressionSubsystem))
  (bind _returnvalue_2 (Class|LinearStoryProgressionSubsystem|GetCurrentPhase _returnvalue))
  (Variables|/Script/ScareSpace.InteractableComponent|SetbCanInteract (Variables|Default|GetBP_SimpleInteractableComponent) (or (Utilities|Enum|Equal(Enum) _returnvalue_2 "AnswerPhone1") (Utilities|Enum|Equal(Enum) _returnvalue_2 "AnswerPhone2")))
  (EventDispatchers|AssignOnStoryPhaseAdvanced (Subsystems|GetLinearStoryProgressionSubsystem) (delegate Custom|OnStoryPhaseAdvanced_Event)))

(fn ConstructionScript)