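; Living room couch prop that runs the WatchTV story beat, interactable only during that phase of the linear story subsystem.
; Interacting with the TV off shows a hint line; with it on, input and capsule collision are disabled and a timeline lerps the player onto the couch.
; The LS_TVScene sequence then plays, and a second timeline moves the player to a post-cutscene point.
; Control returns, the story advances to StartGenerator, and dialogue gives the next objective.
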(event OnInteracted(BP_SimpleInteractableComponent)
  (params (Interactor :type Interactor%20Component%20Object%20Reference))
  (if (Variables|/Game/Props/TV/BP_LivingRoomTV.BP_LivingRoomTV_C|GetIsTVOn (Variables|Default|GetLiving%20Room%20TV))
    (Variables|/Script/ScareSpace.InteractableComponent|SetbCanInteract (Variables|Default|GetBP_SimpleInteractableComponent) false)
    ;[0.15 0.15 0.15 0.5] Prep character for sitting
    (bind _asplayer_character (Utilities|Casting|CastToPlayerCharacter (Game|GetPlayerCharacter 0)))
    (Collision|SetCollisionEnabled (Variables|/Script/Engine.Character|GetCapsuleComponent _asplayer_character) "NoCollision")
    (Class|SimpleFlashlightComponent|TurnFlashlightOff (Variables|/Script/ScareSpace.PlayerCharacter|GetFlashlightComponent _asplayer_character))
    (bind _asmain_player_controller (Utilities|Casting|CastToMainPlayerController (Game|GetPlayerController 0)))
    (Class|MainPlayerController|DisablePlayerInput _asmain_player_controller)
    (CallFunction|SetPlayerNewLocationandRotation)
    (bind _alpha (Timeline|Move%20to%20couch Play)
      (:Update
        (CallFunction|LerpCharacterLocationandRotation _alpha (Variables|Default|GetCouch%20Sitting%20Point)))
      (:Finished
        (bind _returnvalue (Sequencer|Player|CreateLevelSequencePlayer "/Game/LevelSequences/LS_TVScene.LS_TVScene"))
        (Sequencer|Player|Play _returnvalue :!class /Script/MovieScene.MovieSceneSequencePlayer)
        (EventDispatchers|AssignOnFinished _returnvalue (delegate Custom|OnFinished_Event))))
    (else
      (CallFunction|DisplayInternalDialogue (Utilities|Text|MakeLiteralText "The TV could help me sleep") 3.0))))

(event Custom|OnStoryPhaseAdvanced_Event
  (params (NewPhase :type EStoryPhase%20Enum :default "ArriveAtHouse"))
  (Variables|/Script/ScareSpace.InteractableComponent|SetbCanInteract (Variables|Default|GetBP_SimpleInteractableComponent) (Utilities|Enum|Equal(Enum) NewPhase "WatchTV")))

(event Custom|OnFinished_Event
  (CallFunction|SetPlayerNewLocationandRotation)
  (bind _alpha (Timeline|Stand%20up PlayFromStart)
    (:Update
      (CallFunction|LerpCharacterLocationandRotation _alpha (Variables|Default|GetPost%20Cutscene%20Point)))
    (:Finished
      (Collision|SetCollisionEnabled (Variables|/Script/Engine.Character|GetCapsuleComponent (Game|GetPlayerCharacter 0)) "QueryAndPhysics")
      (bind _asmain_player_controller (Utilities|Casting|CastToMainPlayerController (Game|GetPlayerController 0)))
      (Class|MainPlayerController|EnablePlayerInput _asmain_player_controller)
      (Class|LinearStoryProgressionSubsystem|AdvancetoPhase (Subsystems|GetLinearStoryProgressionSubsystem) "StartGenerator")
      (CallFunction|DisplayInternalDialogue (Utilities|Text|MakeLiteralText "I guess I should check the generator out back.") 3.0)
      (Utilities|FlowControl|Delay 4.0)
      (CallFunction|DisplayInternalDialogue (Utilities|Text|MakeLiteralText "The flashlight must be under the kitchen sink") 3.0))))

(event EventBeginPlay
  (Variables|/Script/ScareSpace.InteractableComponent|SetbCanInteract (Variables|Default|GetBP_SimpleInteractableComponent) (Utilities|Enum|Equal(Enum) (Class|LinearStoryProgressionSubsystem|GetCurrentPhase (Subsystems|GetLinearStoryProgressionSubsystem)) "WatchTV"))
  (EventDispatchers|AssignOnStoryPhaseAdvanced (Subsystems|GetLinearStoryProgressionSubsystem) (delegate Custom|OnStoryPhaseAdvanced_Event)))

(fn ConstructionScript)

(fn LerpCharacterLocationandRotation
  (params (Alpha :type Float%20%28single-precision%29) (New%20Target%20Point :type Target%20Point%20Object%20Reference))
  (Transformation|SetActorLocation (Game|GetPlayerCharacter 0) (Math|Vector|Lerp(Vector) (Variables|Default|GetStarting%20Player%20Location) (Transformation|GetActorLocation New%20Target%20Point) Alpha) false true)
  (Pawn|SetControlRotation (Game|GetPlayerController 0) (Math|Rotator|Lerp(Rotator) (Variables|Default|GetStarting%20Player%20Rotation) (Transformation|GetActorRotation New%20Target%20Point) Alpha true)))

(fn SetPlayerNewLocationandRotation
  (Variables|Default|SetStarting%20Player%20Location (Transformation|GetActorLocation (Game|GetPlayerCharacter 0)))
  (Variables|Default|SetStarting%20Player%20Rotation (Pawn|GetControlRotation (Game|GetPlayerController 0) :!class /Script/Engine.Controller)))