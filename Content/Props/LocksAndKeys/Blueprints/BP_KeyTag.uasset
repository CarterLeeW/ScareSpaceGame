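; BP_KeyTag is a key tag prop with a configurable label and colors.
; Its construction script creates a dynamic material on the SMKeytag mesh to apply the outer color, then sets the Text component's content, color and world size from the Name, TextColor and TextSize variables.
; The event graph holds only disabled placeholder events, so the Blueprint adds no gameplay logic of its own.
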(event EventBeginPlay)

(event Collision|EventActorBeginOverlap
  (params (OtherActor :type Actor%20Object%20Reference)))

(event EventTick
  (params (DeltaSeconds :type Float%20%28single-precision%29)))

(fn ConstructionScript
  (bind _text (Variables|Default|GetText))
  (bind _returnvalue (Rendering|Material|CreateDynamicMaterialInstance (Variables|Default|GetSM_Keytag) 0 0 "None" :!class /Script/Engine.PrimitiveComponent))
  (Rendering|Material|SetVectorParameterValue _returnvalue "BaseColor" (Variables|Default|GetOuterColor) :!class /Script/Engine.MaterialInstanceDynamic)
  (Rendering|Components|TextRender|SetText _text (Variables|Default|GetName))
  (Rendering|Components|TextRender|SetTextRenderColor _text (Variables|Default|GetTextColor))
  (Rendering|Components|TextRender|SetWorldSize _text (Variables|Default|GetTextSize)))