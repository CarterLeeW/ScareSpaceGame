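; Wood stove puzzle prop that the player lights in stages, advancing the story from the basement fire phase to feeding the cat.
; A state machine in SetStoveState gates the valve, door and matches interaction for each step: open air, insert wood, light fire, close valve, fully on.
; Valve angle checks, a firewood overlap count and match use drive transitions.
; Closing the valve with the door at rest finishes it and shows dialogue.
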(event OnComponentBeginOverlap(FirewoodTriggerVolume)
  (params (OverlappedComponent :type Primitive%20Component%20Object%20Reference) (OtherActor :type Actor%20Object%20Reference) (OtherComp :type Primitive%20Component%20Object%20Reference) (OtherBodyIndex :type Integer) (bFromSweep :type Boolean) (SweepResult :type Hit%20Result%20Structure%20%28by%20ref%29))
  (if (Utilities|Array|ContainsItem (Variables|/Script/Engine.Actor|GetTags OtherActor) "Firewood")
    (bind _result (Math|Integer|IncrementInt (Variables|Default|GetWood%20Count))
      (:%20%20
        ;[0.15 0.15 0.15 0.5] Enable visibility block for item trigger volume
        (if (>= _result (Variables|Default|GetNum%20of%20logs%20required))
          ;[0.15 0.15 0.15 0.5] Will lock the last log out if i dont drop it in there
          (Rotatable|SetStoveState "NewEnumerator2"))))))

(event OnComponentEndOverlap(FirewoodTriggerVolume)
  (params (OverlappedComponent :type Primitive%20Component%20Object%20Reference) (OtherActor :type Actor%20Object%20Reference) (OtherComp :type Primitive%20Component%20Object%20Reference) (OtherBodyIndex :type Integer))
  (if (Utilities|Array|ContainsItem (Variables|/Script/Engine.Actor|GetTags OtherActor) "Firewood")
    (bind _result (Math|Integer|DecrementInt (Variables|Default|GetWood%20Count))
      (:%20%20
        ;[0.15 0.15 0.15 0.5] We need to disable the item trigger volume if it is less than 4
        (if (< _result (Variables|Default|GetNum%20of%20logs%20required))
          (Rotatable|SetStoveState "NewEnumerator1"))))))

(event OnInteractwithItem(ItemInteractableMatches)
  (params (Interactor :type Interactor%20Component%20Object%20Reference))
  (Rotatable|SetStoveState "NewEnumerator3")
  (Components|Activation|Activate (Variables|Default|GetNS_Fire_Floor_01_Simple) false))

(event OnInteractionEnds(Rotatable)
  (params (Interactor :type Interactor%20Component%20Object%20Reference))
  (if (Rotatable|IsinClosedPosition)
    (switch Utilities|FlowControl|Switch|SwitchonE_WoodStoveStates (Variables|Default|GetStove%20State)
      (:NewEnumerator3
        (if (Variables|/Script/ScareSpace.SimplePivotableComponent|GetbIsAtRest (Variables|Default|GetPivotable_Door))
          (Rotatable|SetStoveState "NewEnumerator4")
          (Development|PrintString "stove fully on"))))
    (elif (CallFunction|IsinOpenPosition)
      (switch Utilities|FlowControl|Switch|SwitchonE_WoodStoveStates (Variables|Default|GetStove%20State)
        (:NewEnumerator0
          (Rotatable|SetStoveState "NewEnumerator1"))))))

(event EventBeginPlay
  (Rotatable|SetStoveState "NewEnumerator0"))

(fn ConstructionScript)

(fn OpenAir
  (Variables|/Script/ScareSpace.InteractableComponent|SetbCanAcceptItem (Variables|Default|GetItemInteractableMatches) false)
  (Class|SimplePivotableComponent|SetIsLocked (Variables|Default|GetPivotable_Door) true)
  (Variables|/Script/ScareSpace.RotatableComponent|SetbCanRotate (Variables|Default|GetRotatable) true)
  (Collision|SetCollisionResponsetoChannel (Variables|Default|GetMatches%20Item%20Trigger%20Volume) "ECC_Visibility" "ECR_Ignore"))

(fn InsertWood
  (Variables|/Script/ScareSpace.RotatableComponent|SetbCanRotate (Variables|Default|GetRotatable) false)
  (Class|SimplePivotableComponent|SetIsLocked (Variables|Default|GetPivotable_Door) false)
  (Variables|/Script/ScareSpace.InteractableComponent|SetbCanAcceptItem (Variables|Default|GetItemInteractableMatches) false)
  (Collision|SetCollisionResponsetoChannel (Variables|Default|GetMatches%20Item%20Trigger%20Volume) "ECC_Visibility" "ECR_Ignore"))

(fn LightFire
  (Variables|/Script/ScareSpace.InteractableComponent|SetbCanAcceptItem (Variables|Default|GetItemInteractableMatches) true)
  (Collision|SetCollisionResponsetoChannel (Variables|Default|GetMatches%20Item%20Trigger%20Volume) "ECC_Visibility" "ECR_Block"))

(fn CloseValve
  (Variables|/Script/ScareSpace.RotatableComponent|SetbCanRotate (Variables|Default|GetRotatable) true)
  ;[0.15 0.15 0.15 0.5] Disable firewood interaction
  (for _array_element (Collision|GetOverlappingActors (Variables|Default|GetFirewood%20Trigger%20Volume) 0 :!class /Script/Engine.PrimitiveComponent)
    (bind _asbp_firewood_4 (Utilities|Casting|CastToBP_Firewood4 _array_element))
    (Variables|/Script/ScareSpace.InteractableComponent|SetbCanInteract (Variables|/Game/Props/BP_Firewood4.BP_Firewood4_C|GetBP_HoldableComponent _asbp_firewood_4) false)))

(fn Fullyon
  (bind _returnvalue (Subsystems|GetLinearStoryProgressionSubsystem))
  (Variables|/Script/ScareSpace.RotatableComponent|SetbCanRotate (Variables|Default|GetRotatable) false)
  (Class|SimplePivotableComponent|SetIsLocked (Variables|Default|GetPivotable_Door) true)
  (switch Utilities|FlowControl|Switch|SwitchonEStoryPhase (Class|LinearStoryProgressionSubsystem|GetCurrentPhase _returnvalue)
    (:StartBasementFire
      (if true
        (Class|LinearStoryProgressionSubsystem|AdvancetoPhase _returnvalue "FeedCat")
        (CallFunction|DisplayInternalDialogue (Variables|Default|GetFeed%20Cat%20Dialogue) 3.0)))))

(fn SetStoveState
  (params (New%20State :type E_WoodStoveStates%20Enum :default "NewEnumerator0"))
  (bind _output_get (Variables|Default|SetStove%20State New%20State))
  (switch Utilities|FlowControl|Switch|SwitchonE_WoodStoveStates _output_get
    (:NewEnumerator0
      (StoveStates|OpenAir))
    (:NewEnumerator1
      (StoveStates|InsertWood))
    (:NewEnumerator2
      (StoveStates|LightFire))
    (:NewEnumerator3
      (StoveStates|CloseValve))
    (:NewEnumerator4
      (StoveStates|Fullyon))))

(fn IsinClosedPosition
  (return (<= (Class|RotatableComponent|GetCurrentAngle (Variables|Default|GetRotatable)) (+ (Variables|/Script/ScareSpace.RotatableComponent|GetMinAngle (Variables|Default|GetRotatable)) 5.0))))

(fn IsinOpenPosition
  (return (>= (Class|RotatableComponent|GetCurrentAngle (Variables|Default|GetRotatable)) (- (Variables|/Script/ScareSpace.RotatableComponent|GetMaxAngle (Variables|Default|GetRotatable)) 5.0))))