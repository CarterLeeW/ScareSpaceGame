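; Cat food can prop that the player can interact with once the story reaches the Feed Cat phase.
; On BeginPlay it enables its Collectable's interaction only if the current phase is Feed Cat, then subscribes to the linear story progression subsystem's phase-advanced event.
; That event turns interaction on when Feed Cat begins, and nothing in the Blueprint turns it off again afterwards.
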(event Custom|OnStoryPhaseAdvanced_Event
  (params (NewPhase :type EStoryPhase%20Enum :default "ArriveAtHouse"))
  (switch Utilities|FlowControl|Switch|SwitchonEStoryPhase NewPhase
    (:FeedCat
      (Variables|/Script/ScareSpace.InteractableComponent|SetbCanInteract (Variables|Default|GetCollectable) true))))

(event EventBeginPlay
  (CallFunction|SetDefaultInteractionState)
  (EventDispatchers|AssignOnStoryPhaseAdvanced (Subsystems|GetLinearStoryProgressionSubsystem) (delegate Custom|OnStoryPhaseAdvanced_Event)))

(event Collision|EventActorBeginOverlap
  (params (OtherActor :type Actor%20Object%20Reference)))

(event EventTick
  (params (DeltaSeconds :type Float%20%28single-precision%29)))

(fn ConstructionScript)

(fn SetDefaultInteractionState
  (if (Utilities|Enum|Equal(Enum) (Class|LinearStoryProgressionSubsystem|GetCurrentPhase (Subsystems|GetLinearStoryProgressionSubsystem)) "FeedCat")
    (Variables|/Script/ScareSpace.InteractableComponent|SetbCanInteract (Variables|Default|GetCollectable) true)
    (else
      (Variables|/Script/ScareSpace.InteractableComponent|SetbCanInteract (Variables|Default|GetCollectable) false))))