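; Ceiling lamp prop Blueprint with a spot light, a point light and on/off states shown by swapping the mesh material.
; TurnLightOn, TurnLightOff and ToggleLight change material, light intensities and IsOn, with the point light scaled down from BaseIntensity.
; BeginPlay applies IsOn, while the construction script uses separate LampOn and AddLight flags to set the material and destroy the spot light when unwanted.
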(event EventBeginPlay
  (if (Variables|Default|GetIsOn)
    (CallFunction|TurnLighton)
    (else
      (CallFunction|TurnLightOff))))

(event Collision|EventActorBeginOverlap
  (params (OtherActor :type Actor%20Object%20Reference)))

(event EventTick
  (params (DeltaSeconds :type Float%20%28single-precision%29)))

(event EventTurnLightOff
  (Rendering|Material|SetMaterial (Variables|Debug|GetStaticMeshComponent) 0 "/Game/HousePropsFurniture/Materials/MI_Lamps_C_OFF.MI_Lamps_C_off")
  (Rendering|Components|Light|SetIntensity (Variables|Default|GetSpotLight) 0.0)
  (Rendering|Components|Light|SetIntensity (Variables|Default|GetPointLight) 0.0)
  (Variables|Default|SetIsOn false))

(event EventTurnLighton
  (bind _base_intensity (Variables|Default|GetBase%20Intensity))
  (Rendering|Material|SetMaterial (Variables|Debug|GetStaticMeshComponent) 0 "/Game/HousePropsFurniture/Materials/MI_Lamps_C_on.MI_Lamps_C_on")
  (Rendering|Components|Light|SetIntensity (Variables|Default|GetSpotLight) _base_intensity)
  (Rendering|Components|Light|SetIntensity (Variables|Default|GetPointLight) (/ _base_intensity 5e+01))
  (Variables|Default|SetIsOn true))

(event EventToggleLight
  (if (Variables|Default|GetIsOn)
    (CallFunction|TurnLightOff)
    (else
      (CallFunction|TurnLighton))))

(fn ConstructionScript
  (if (Variables|Lamp|GetLamp%20On?)
    (Rendering|Material|SetMaterial (Variables|Debug|GetStaticMeshComponent) 0 "/Game/HousePropsFurniture/Materials/MI_Lamps_C_on.MI_Lamps_C_on")
    (if (not (Variables|Lamp|GetAdd%20Light?))
      (Components|DestroyComponent (Variables|Default|GetSpotLight)))
    (else
      (Components|DestroyComponent (Variables|Default|GetSpotLight))
      (Rendering|Material|SetMaterial (Variables|Debug|GetStaticMeshComponent) 0 "/Game/HousePropsFurniture/Materials/MI_Lamps_C_OFF.MI_Lamps_C_off"))))