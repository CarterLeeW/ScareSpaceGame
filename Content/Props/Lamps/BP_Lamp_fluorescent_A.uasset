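; BP_Lamp_fluorescent_A is a fluorescent lamp prop with a rect light that switches on and off.
; The construction script uses LampOn to pick the on or off material, and destroys the RectLight unless both LampOn and AddLight are set.
; At BeginPlay a separate IsOn flag sets the state through turn-on and turn-off events, which swap the material, set light intensity and update IsOn.
; ToggleLight flips that state and GetIsOn returns it.
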(event EventBeginPlay
  (if (Variables|Default|GetIsOn)
    (CallFunction|TurnLighton)
    (else
      (CallFunction|TurnLightOff))))

(event EventTurnLightOff
  (Rendering|Material|SetMaterial (Variables|Debug|GetStaticMeshComponent) 0 "/Game/HousePropsFurniture/Materials/MI_Lamps_C_OFF.MI_Lamps_C_off")
  (Rendering|Components|Light|SetIntensity (Variables|Default|GetRectLight) 0.0)
  (Variables|Default|SetIsOn false))

(event EventTurnLighton
  (Rendering|Material|SetMaterial (Variables|Debug|GetStaticMeshComponent) 0 "/Game/HousePropsFurniture/Materials/MI_Lamps_C_on.MI_Lamps_C_on")
  (Rendering|Components|Light|SetIntensity (Variables|Default|GetRectLight) (Variables|Default|GetBase%20Intensity))
  (Variables|Default|SetIsOn true))

(event EventToggleLight
  (if (Variables|Default|GetIsOn)
    (CallFunction|TurnLightOff)
    (else
      (CallFunction|TurnLighton))))

(fn ConstructionScript
  (if (Variables|Default|GetLamp%20On?)
    (Rendering|Material|SetMaterial (Variables|Debug|GetStaticMeshComponent) 0 "/Game/HousePropsFurniture/Materials/MI_Lamps_C_on.MI_Lamps_C_on")
    (if (not (Variables|Lamp|GetAdd%20Light?))
      (Components|DestroyComponent (Variables|Default|GetRectLight)))
    (else
      (Components|DestroyComponent (Variables|Default|GetRectLight))
      (Rendering|Material|SetMaterial (Variables|Debug|GetStaticMeshComponent) 0 "/Game/HousePropsFurniture/Materials/MI_Lamps_C_OFF.MI_Lamps_C_off"))))

(fn GetIson
  (return (Variables|Default|GetIsOn)))