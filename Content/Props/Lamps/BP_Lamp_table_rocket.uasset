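; Rocket table lamp prop that switches between lit and unlit states, with events to turn on, turn off or toggle.
; Each switch swaps the shade and base materials, sets the point light to BaseIntensity or zero, and updates IsOn, which also picks the state at BeginPlay.
; The construction script previews materials from a separate LampOn flag, destroys the light when off or AddLight is false, and makes the shade static when off.
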(event EventBeginPlay
  (if (Variables|Default|GetIsOn)
    (CallFunction|TurnLighton)
    (else
      (CallFunction|TurnLightOff))))

(event Collision|EventActorBeginOverlap
  (params (OtherActor :type Actor%20Object%20Reference)))

(event EventTick
  (params (DeltaSeconds :type Float%20%28single-precision%29)))

(event EventTurnLightOff
  (Rendering|Material|SetMaterial (Variables|Default|GetLamp_table_rocket_shade) 0 "/Game/HousePropsFurniture/Materials/MI_Lamps_C_OFF.MI_Lamps_C_off")
  (Rendering|Material|SetMaterial (Variables|Default|GetLamp_table_rocket_base) 0 "/Game/HousePropsFurniture/Materials/MI_Lamps_C_OFF.MI_Lamps_C_off")
  (Rendering|Components|Light|SetIntensity (Variables|Default|GetPointLight) 0.0)
  (Variables|Default|SetIsOn false))

(event EventTurnLighton
  (Rendering|Material|SetMaterial (Variables|Default|GetLamp_table_rocket_shade) 0 "/Game/HousePropsFurniture/Materials/MI_Lamps_C_on.MI_Lamps_C_on")
  (Rendering|Material|SetMaterial (Variables|Default|GetLamp_table_rocket_base) 0 "/Game/HousePropsFurniture/Materials/MI_Lamps_C_on.MI_Lamps_C_on")
  (Rendering|Components|Light|SetIntensity (Variables|Default|GetPointLight) (Variables|Default|GetBase%20Intensity))
  (Variables|Default|SetIsOn true))

(event EventToggleLight
  (if (Variables|Default|GetIsOn)
    (CallFunction|TurnLightOff)
    (else
      (CallFunction|TurnLighton))))

(fn ConstructionScript
  (if (Variables|Lamp|GetLamp%20On?)
    (Rendering|Material|SetMaterial (Variables|Default|GetLamp_table_rocket_shade) 0 "/Game/HousePropsFurniture/Materials/MI_Lamps_C_on.MI_Lamps_C_on")
    (Rendering|Material|SetMaterial (Variables|Default|GetLamp_table_rocket_base) 0 "/Game/HousePropsFurniture/Materials/MI_Lamps_C_on.MI_Lamps_C_on")
    (if (not (Variables|Lamp|GetAdd%20Light?))
      (Components|DestroyComponent (Variables|Default|GetPointLight)))
    (else
      (Components|DestroyComponent (Variables|Default|GetPointLight))
      (Rendering|Material|SetMaterial (Variables|Default|GetLamp_table_rocket_shade) 0 "/Game/HousePropsFurniture/Materials/MI_Lamps_C_OFF.MI_Lamps_C_off")
      (Rendering|Material|SetMaterial (Variables|Default|GetLamp_table_rocket_base) 0 "/Game/HousePropsFurniture/Materials/MI_Lamps_C_OFF.MI_Lamps_C_off")
      (Transformation|SetMobility (Variables|Default|GetLamp_table_rocket_shade) "Static"))))