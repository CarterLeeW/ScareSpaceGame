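; Chandelier prop with shade and body meshes and a point light that can be switched on, off or toggled.
; Switch events swap both meshes between lit and unlit materials, set the light intensity and update IsOn, which BeginPlay applies at start.
; The construction script instead uses LampOn and AddLight, destroying the light when either is false and making the shades static when the lamp is off.
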(event EventBeginPlay
  (if (Variables|Default|GetIsOn)
    (CallFunction|TurnLighton)
    (else
      (CallFunction|TurnLightOff))))

(event EventTurnLightOff
  (Rendering|Material|SetMaterial (Variables|Default|GetChandelier_A_shades) 0 "/Game/HousePropsFurniture/Materials/MI_Lamps_B_off.MI_Lamps_B_off")
  (Rendering|Material|SetMaterial (Variables|Default|GetChandelier_A_body) 0 "/Game/HousePropsFurniture/Materials/MI_Lamps_B_off.MI_Lamps_B_off")
  (Rendering|Components|Light|SetIntensity (Variables|Default|GetPointLight) 0.0)
  (Variables|Default|SetIsOn false))

(event EventTurnLighton
  (Rendering|Material|SetMaterial (Variables|Default|GetChandelier_A_shades) 0 "/Game/HousePropsFurniture/Materials/MI_Lamps_B_on.MI_Lamps_B_on")
  (Rendering|Material|SetMaterial (Variables|Default|GetChandelier_A_body) 0 "/Game/HousePropsFurniture/Materials/MI_Lamps_B_on.MI_Lamps_B_on")
  (Rendering|Components|Light|SetIntensity (Variables|Default|GetPointLight) (Variables|Default|GetBaseIntensity))
  (Variables|Default|SetIsOn true))

(event EventToggleLight
  (if (Variables|Default|GetIsOn)
    (CallFunction|TurnLightOff)
    (else
      (CallFunction|TurnLighton))))

(fn ConstructionScript
  (if (Variables|Lamp|GetLamp%20On?)
    (Rendering|Material|SetMaterial (Variables|Default|GetChandelier_A_shades) 0 "/Game/HousePropsFurniture/Materials/MI_Lamps_B_on.MI_Lamps_B_on")
    (Rendering|Material|SetMaterial (Variables|Default|GetChandelier_A_body) 0 "/Game/HousePropsFurniture/Materials/MI_Lamps_B_on.MI_Lamps_B_on")
    (if (not (Variables|Lamp|GetAdd%20Light?))
      (Components|DestroyComponent (Variables|Default|GetPointLight)))
    (else
      (Components|DestroyComponent (Variables|Default|GetPointLight))
      (Rendering|Material|SetMaterial (Variables|Default|GetChandelier_A_shades) 0 "/Game/HousePropsFurniture/Materials/MI_Lamps_B_off.MI_Lamps_B_off")
      (Rendering|Material|SetMaterial (Variables|Default|GetChandelier_A_body) 0 "/Game/HousePropsFurniture/Materials/MI_Lamps_B_off.MI_Lamps_B_off")
      (Transformation|SetMobility (Variables|Default|GetChandelier_A_shades) "Static"))))