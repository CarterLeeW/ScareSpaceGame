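; BP_Generator is a story-gated generator prop that the player must fuel and start to restore lighting.
; Its interactable component accepts interaction and items only during the StartGenerator phase, updated through LinearStoryProgressionSubsystem.
; First interaction fires a dispatcher (opens the basement gate) and adds a fuel journal entry; using an item fuels it and removes that entry.
; Starting it advances to AnswerPhone1 and re-enables GS_Main lights; BeginPlay replays its sound for later-phase loads.
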(event OnInteracted(BP_SimpleInteractableComponent)
  (params (Interactor :type Interactor%20Component%20Object%20Reference))
  (if (Variables|Default|GetIsFirstInteraction)
    (Variables|Default|SetIsFirstInteraction false)
    ;[0.15 0.15 0.15 0.5] Causes basement gate to open
    (Default|CallOnFirstInteractionOccured)
    (Class|LinearStoryProgressionSubsystem|AddJournalEntry (Subsystems|GetLinearStoryProgressionSubsystem) (Variables|Default|GetGet%20Fuel%20Memento))
    (CallFunction|DisplayInternalDialogue (Variables|Default|GetGet%20Fuel%20Internal%20Dialogue) 3.0 :!label _label)
    (elif (Variables|Default|GetIsFueled)
      ;[0.15 0.15 0.15 0.5] Turn on and proceed to next step
      (Audio|SpawnSoundatLocation "/Game/SoundEffects/Generator/MSS_Generator.MSS_Generator" (Transformation|GetActorLocation) "0, 0, 0" 1.0 1.0 0.0 0 0)
      (Variables|/Script/ScareSpace.InteractableComponent|SetbCanInteract (Variables|Default|GetBP_SimpleInteractableComponent) false)
      (Class|LinearStoryProgressionSubsystem|AdvancetoPhase (Subsystems|GetLinearStoryProgressionSubsystem) "AnswerPhone1")
      (bind _asgs_main (Utilities|Casting|CastToGS_Main (Game|GetGameState)))
      (Default|EnableLightSwitches _asgs_main true)
      (Default|RestoreonLights _asgs_main)
      (Default|ClearonLightsArray _asgs_main)
      (else
        (goto _label)))))

(event OnInteractwithItem(BP_SimpleInteractableComponent)
  (params (Interactor :type Interactor%20Component%20Object%20Reference))
  (Variables|Default|SetIsFueled true)
  (Class|LinearStoryProgressionSubsystem|RemoveJournalEntry (Subsystems|GetLinearStoryProgressionSubsystem) (Variables|Default|GetGet%20Fuel%20Memento)))

(event Custom|OnStoryPhaseAdvanced_Event
  (params (NewPhase :type EStoryPhase%20Enum :default "ArriveAtHouse"))
  (bind _returnvalue (Utilities|Enum|Equal(Enum) NewPhase "StartGenerator"))
  (bind _bp_simpleinteractablecomponent (Variables|Default|GetBP_SimpleInteractableComponent))
  (Variables|/Script/ScareSpace.InteractableComponent|SetbCanInteract _bp_simpleinteractablecomponent _returnvalue)
  (Variables|/Script/ScareSpace.InteractableComponent|SetbCanAcceptItem _bp_simpleinteractablecomponent _returnvalue))

(event EventBeginPlay
  (bind _returnvalue (Subsystems|GetLinearStoryProgressionSubsystem))
  (bind _bp_simpleinteractablecomponent (Variables|Default|GetBP_SimpleInteractableComponent))
  (bind _returnvalue_2 (Class|LinearStoryProgressionSubsystem|GetCurrentPhase _returnvalue))
  (bind _returnvalue_3 (Utilities|Enum|Equal(Enum) _returnvalue_2 "StartGenerator"))
  (Variables|/Script/ScareSpace.InteractableComponent|SetbCanInteract _bp_simpleinteractablecomponent _returnvalue_3)
  (Variables|/Script/ScareSpace.InteractableComponent|SetbCanAcceptItem _bp_simpleinteractablecomponent _returnvalue_3)
  (EventDispatchers|AssignOnStoryPhaseAdvanced (Subsystems|GetLinearStoryProgressionSubsystem) (delegate Custom|OnStoryPhaseAdvanced_Event))
  (CallFunction|PlaySoundifLoadingGameAfterPhase))

(fn ConstructionScript)

(fn PlaySoundifLoadingGameAfterPhase
  (if (>= (Class|LinearStoryProgressionSubsystem|GetCurrentPhase (Subsystems|GetLinearStoryProgressionSubsystem)) (Math|Conversions|ToInteger(Byte) (Utilities|Enum|LiteralenumEStoryPhase "AnswerPhone1")))
    (Audio|SpawnSoundatLocation "/Game/SoundEffects/Generator/MSS_Generator.MSS_Generator" (Transformation|GetActorLocation) "0, 0, 0" 1.0 1.0 0.0 0 0)))