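; Wood stove prop that runs a step-by-step fire-lighting interaction and, in the basement fire story phase, advances to feeding the cat with internal dialogue.
; A state machine sequences opening the air valve, inserting logs, lighting with an item, and closing the valve with the pivotable shut.
; Rotatable angle checks, tagged firewood overlap counts and item interaction drive transitions.
; Each state toggles component locks, item acceptance or trigger collision.
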(event OnComponentBeginOverlap(FirewoodTriggerVolume)
  (params (OverlappedComponent :type Primitive%20Component%20Object%20Reference) (OtherActor :type Actor%20Object%20Reference) (OtherComp :type Primitive%20Component%20Object%20Reference) (OtherBodyIndex :type Integer) (bFromSweep :type Boolean) (SweepResult :type Hit%20Result%20Structure%20%28by%20ref%29))
  (if (Utilities|Array|ContainsItem (Variables|/Script/Engine.Actor|GetTags OtherActor) "Firewood")
    (bind _result (Math|Integer|IncrementInt (Variables|Default|GetWood%20Count))
      (:%20%20
        ;[0.15 0.15 0.15 0.5] Enable visibility block for item trigger volume
        (if (>= _result (Variables|Default|GetNum%20of%20logs%20required))
          ;[0.15 0.15 0.15 0.5] Will lock the last log out if i dont drop it in there
          (CallFunction|SetStoveState "NewEnumerator2"))))))

(event OnComponentEndOverlap(FirewoodTriggerVolume)
  (params (OverlappedComponent :type Primitive%20Component%20Object%20Reference) (OtherActor :type Actor%20Object%20Reference) (OtherComp :type Primitive%20Component%20Object%20Reference) (OtherBodyIndex :type Integer))
  (if (Utilities|Array|ContainsItem (Variables|/Script/Engine.Actor|GetTags OtherActor) "Firewood")
    (bind _result (Math|Integer|DecrementInt (Variables|Default|GetWood%20Count))
      (:%20%20
        ;[0.15 0.15 0.15 0.5] We need to disable the item trigger volume if it is less than 4
        (if (< _result (Variables|Default|GetNum%20of%20logs%20required))
          (CallFunction|SetStoveState "NewEnumerator1"))))))

(event OnInteractionEnds(Pivotable)
  (params (Interactor :type Interactor%20Component%20Object%20Reference))
  (Development|PrintString "interaction ends"))

(event OnInteractwithItem(ItemInteractable)
  (params (Interactor :type Interactor%20Component%20Object%20Reference))
  (CallFunction|SetStoveState "NewEnumerator3"))

(event OnInteractionEnds(Rotatable)
  (params (Interactor :type Interactor%20Component%20Object%20Reference))
  (if (Rotatable|IsinClosedPosition)
    (switch Utilities|FlowControl|Switch|SwitchonE_WoodStoveStates (Variables|Default|GetStove%20State)
      (:NewEnumerator3
        (if (Variables|/Script/ScareSpace.PivotableComponent|GetbIsClosed (Variables|Default|GetPivotable))
          (CallFunction|SetStoveState "NewEnumerator4")
          (Development|PrintString "stove fully on"))))
    (elif (Rotatable|IsinOpenPosition)
      (switch Utilities|FlowControl|Switch|SwitchonE_WoodStoveStates (Variables|Default|GetStove%20State)
        (:NewEnumerator0
          (CallFunction|SetStoveState "NewEnumerator1"))))))

(event EventBeginPlay
  (CallFunction|SetStoveState "NewEnumerator0"))

(fn ConstructionScript)

(fn SetStoveState
  (params (New%20State :type E_WoodStoveStates%20Enum :default "NewEnumerator0"))
  (bind _output_get (Variables|Default|SetStove%20State New%20State))
  (switch Utilities|FlowControl|Switch|SwitchonE_WoodStoveStates _output_get
    (:NewEnumerator0
      (StoveStates|OpenAir))
    (:NewEnumerator1
      (StoveStates|InsertWood))
    (:NewEnumerator2
      (StoveStates|LightFire))
    (:NewEnumerator3
      (StoveStates|CloseValve))
    (:NewEnumerator4
      (StoveStates|Fullyon))))

(fn OpenAir
  (Variables|/Script/ScareSpace.InteractableComponent|SetbCanAcceptItem (Variables|Default|GetItemInteractable) false)
  (Variables|/Script/ScareSpace.PivotableComponent|SetbIsLocked (Variables|Default|GetPivotable) true)
  (Variables|/Script/ScareSpace.RotatableComponent|SetbCanRotate (Variables|Default|GetRotatable) true)
  (Collision|SetCollisionResponsetoChannel (Variables|Default|GetMatches%20Item%20Trigger%20Volume) "ECC_Visibility" "ECR_Ignore"))

(fn InsertWood
  (Variables|/Script/ScareSpace.RotatableComponent|SetbCanRotate (Variables|Default|GetRotatable) false)
  (Variables|/Script/ScareSpace.PivotableComponent|SetbIsLocked (Variables|Default|GetPivotable) false)
  (Variables|/Script/ScareSpace.InteractableComponent|SetbCanAcceptItem (Variables|Default|GetItemInteractable) false)
  (Collision|SetCollisionResponsetoChannel (Variables|Default|GetMatches%20Item%20Trigger%20Volume) "ECC_Visibility" "ECR_Ignore"))

(fn LightFire
  (Variables|/Script/ScareSpace.InteractableComponent|SetbCanAcceptItem (Variables|Default|GetItemInteractable) true)
  (Collision|SetCollisionResponsetoChannel (Variables|Default|GetMatches%20Item%20Trigger%20Volume) "ECC_Visibility" "ECR_Block"))

(fn CloseValve
  (Variables|/Script/ScareSpace.RotatableComponent|SetbCanRotate (Variables|Default|GetRotatable) true)
  ;[0.15 0.15 0.15 0.5] Disable firewood interaction
  (for _array_element (Collision|GetOverlappingActors (Variables|Default|GetFirewood%20Trigger%20Volume) 0 :!class /Script/Engine.PrimitiveComponent)
    (bind _asbp_firewood_4 (Utilities|Casting|CastToBP_Firewood4 _array_element))
    (Variables|/Script/ScareSpace.InteractableComponent|SetbCanInteract (Variables|/Game/Props/BP_Firewood4.BP_Firewood4_C|GetBP_HoldableComponent _asbp_firewood_4) false)))

(fn IsinClosedPosition
  (return (<= (Class|RotatableComponent|GetCurrentAngle (Variables|Default|GetRotatable)) (+ (Variables|/Script/ScareSpace.RotatableComponent|GetMinAngle (Variables|Default|GetRotatable)) 5.0))))

(fn IsinOpenPosition
  (return (>= (Class|RotatableComponent|GetCurrentAngle (Variables|Default|GetRotatable)) (- (Variables|/Script/ScareSpace.RotatableComponent|GetMaxAngle (Variables|Default|GetRotatable)) 5.0))))

(fn Fullyon
  (bind _returnvalue (Subsystems|GetLinearStoryProgressionSubsystem))
  (Variables|/Script/ScareSpace.RotatableComponent|SetbCanRotate (Variables|Default|GetRotatable) false)
  (Variables|/Script/ScareSpace.PivotableComponent|SetbIsLocked (Variables|Default|GetPivotable) true)
  (switch Utilities|FlowControl|Switch|SwitchonEStoryPhase (Class|LinearStoryProgressionSubsystem|GetCurrentPhase _returnvalue)
    (:StartBasementFire
      (if true
        (Class|LinearStoryProgressionSubsystem|AdvancetoPhase _returnvalue "FeedCat")
        (CallFunction|DisplayInternalDialogue (Variables|Default|GetFeed%20Cat%20Dialogue) 3.0)))))