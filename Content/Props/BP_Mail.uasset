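; BP_Mail is a mail prop whose Collectable component is interactable only during the BringInMail story phase.
; On BeginPlay it sets the component's CanInteract from the current phase in LinearStoryProgressionSubsystem, then binds to that subsystem's phase-advanced event to update the flag on each change.
; Tick, the interaction-begin event and the construction script are empty, so the Blueprint adds no collection logic of its own.
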(event OnInteractionBegins(Collectable)
  (params (Interactor :type Interactor%20Component%20Object%20Reference)))

(event Custom|OnStoryPhaseAdvanced_Event
  (params (NewPhase :type EStoryPhase%20Enum :default "ArriveAtHouse"))
  (Variables|/Script/ScareSpace.InteractableComponent|SetbCanInteract (Variables|Default|GetCollectable) (Utilities|Enum|Equal(Enum) NewPhase "BringInMail")))

(event EventBeginPlay
  (Variables|/Script/ScareSpace.InteractableComponent|SetbCanInteract (Variables|Default|GetCollectable) (Utilities|Enum|Equal(Enum) (Class|LinearStoryProgressionSubsystem|GetCurrentPhase (Subsystems|GetLinearStoryProgressionSubsystem)) "BringInMail"))
  (EventDispatchers|AssignOnStoryPhaseAdvanced (Subsystems|GetLinearStoryProgressionSubsystem) (delegate Custom|OnStoryPhaseAdvanced_Event)))

(event EventTick
  (params (DeltaSeconds :type Float%20%28single-precision%29)))

(fn ConstructionScript)