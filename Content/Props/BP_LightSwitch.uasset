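; BP_LightSwitch is an interactable light switch prop that toggles a set of linked lamps.
; When its BP_SimpleInteractableComponent fires OnInteracted and ShouldLightsWork is true, it sends ToggleLightMessage to every entry in ControlledLamps.
; The switch leaves the toggling to each lamp, so several switches can share the same lights.
; Older IsFlippedOn-based on/off logic remains disconnected and never runs.
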(event OnInteracted(BP_SimpleInteractableComponent)
  (params (Interactor :type Interactor%20Component%20Object%20Reference))
  (if (Variables|Default|GetShould%20Lights%20Work?)
    (for _array_element (Variables|Default|GetControlled%20Lamps)
      (Class|BILamp|ToggleLight(Message) _array_element))))

(event EventBeginPlay)

(fn ConstructionScript)