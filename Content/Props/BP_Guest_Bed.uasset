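; Guest bed prop that starts the bedtime cutscene, interactable only while the linear story is in the GoToBed phase.
; Phase-change events toggle the interactable component; interacting disables it and starts the sequence, with a tag check that only prints debug text.
; The sequence kills flashlight and input, fades out, teleports the player, then plays LS_SleepScene.
; Its finish handler is empty; older logic advancing to GetWater is disconnected.
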(event OnInteracted(BP_SimpleInteractableComponent)
  (params (Interactor :type Interactor%20Component%20Object%20Reference))
  (Development|PrintString (Utilities|String|SelectString "bed time" "not bed time" (Utilities|Array|ContainsItem (Variables|/Script/Engine.ActorComponent|GetComponentTags Interactor) "teeth_brushed")))
  (Variables|/Script/ScareSpace.InteractableComponent|SetbCanInteract (Variables|Default|GetBP_SimpleInteractableComponent) false)
  (CallFunction|BeginSequence))

(event Custom|OnStoryPhaseAdvanced_Event
  (params (NewPhase :type EStoryPhase%20Enum :default "ArriveAtHouse"))
  (Variables|/Script/ScareSpace.InteractableComponent|SetbCanInteract (Variables|Default|GetBP_SimpleInteractableComponent) (Utilities|Enum|Equal(Enum) NewPhase "GoToBed")))

(event Custom|OnFinished_Event
  (bind _post_cutscene_spawn_point (Variables|Default|GetPost%20Cutscene%20Spawn%20Point))
  ;[0.15 0.15 0.15 0.5] Old level sequence stuff
  (Development|PrintString "finished")
  (bind _ascharacter (Utilities|Casting|CastToCharacter (Components|GetOwner (stale OnInteracted(BP_SimpleInteractableComponent) Interactor))))
  (Transformation|SetActorLocation _ascharacter (Transformation|GetActorLocation _post_cutscene_spawn_point) false true)
  (Pawn|SetControlRotation (Pawn|GetController _ascharacter) (Transformation|GetActorRotation _post_cutscene_spawn_point))
  (Class|LinearStoryProgressionSubsystem|AdvancetoPhase (Subsystems|GetLinearStoryProgressionSubsystem) "GetWater"))

(event EventBeginPlay
  (Variables|/Script/ScareSpace.InteractableComponent|SetbCanInteract (Variables|Default|GetBP_SimpleInteractableComponent) (Utilities|Enum|Equal(Enum) (Class|LinearStoryProgressionSubsystem|GetCurrentPhase (Subsystems|GetLinearStoryProgressionSubsystem)) "GoToBed"))
  (EventDispatchers|AssignOnStoryPhaseAdvanced (Subsystems|GetLinearStoryProgressionSubsystem) (delegate Custom|OnStoryPhaseAdvanced_Event)))

(event Custom|On%20Cutscene%20Finished)

(event Custom|Begin%20Sequence
  (bind _cutscene_player_location (Variables|Default|GetCutscene%20Player%20Location))
  (bind _asplayer_character (Utilities|Casting|CastToPlayerCharacter (Game|GetPlayerCharacter 0)))
  (Class|SimpleFlashlightComponent|TurnFlashlightOff (Variables|/Script/ScareSpace.PlayerCharacter|GetFlashlightComponent _asplayer_character))
  (bind _asmain_player_controller (Utilities|Casting|CastToMainPlayerController (Pawn|GetController _asplayer_character)))
  (Class|MainPlayerController|DisablePlayerInput _asmain_player_controller)
  (CameraFades|StartCameraFade :self (Variables|/Script/Engine.PlayerController|GetPlayerCameraManager _asmain_player_controller) :ToAlpha 1.0 :Duration 1.0 :bHoldWhenFinished true)
  (Utilities|FlowControl|Delay 1.2)
  (Collision|SetCollisionEnabled (Variables|/Script/Engine.Character|GetCapsuleComponent _asplayer_character) "NoCollision")
  (Transformation|SetActorLocation _asplayer_character (Transformation|GetWorldLocation _cutscene_player_location) false true)
  (Pawn|SetControlRotation _asmain_player_controller (Transformation|GetWorldRotation _cutscene_player_location))
  (Utilities|FlowControl|Delay 2.0)
  (bind _returnvalue (Sequencer|Player|CreateLevelSequencePlayer "/Game/LevelSequences/LS_SleepScene.LS_SleepScene" (Utilities|Struct|MakeMovieSceneSequencePlaybackSettings true "(Value=0)")))
  (EventDispatchers|AssignOnFinished _returnvalue (delegate Custom|On%20Cutscene%20Finished)))

(fn ConstructionScript)