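; BP_GuestRoomAmbient is a switchable point light prop, named as ambient lighting for a guest room.
; On BeginPlay it caches the component's authored intensity, then applies either that value or zero based on IsOn.
; TurnLightOff and TurnLighton events toggle it by setting intensity to zero or the cached value and updating IsOn, without changing the component's visibility.
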(event EventBeginPlay
  (Variables|Default|SetBaseIntensity (Variables|/Script/Engine.LightComponentBase|GetIntensity (Variables|Default|GetPointLightComponent)))
  (if (Variables|Default|GetIsOn)
    (Rendering|Components|Light|SetIntensity (Variables|Default|GetPointLightComponent) (Variables|Default|GetBaseIntensity))
    (else
      (Rendering|Components|Light|SetIntensity (Variables|Default|GetPointLightComponent) 0.0))))

(event EventTurnLightOff
  (Rendering|Components|Light|SetIntensity (Variables|Default|GetPointLightComponent) 0.0)
  (Variables|Default|SetIsOn false))

(event EventTurnLighton
  (Rendering|Components|Light|SetIntensity (Variables|Default|GetPointLightComponent) (Variables|Default|GetBaseIntensity))
  (Variables|Default|SetIsOn true))

(fn ConstructionScript)