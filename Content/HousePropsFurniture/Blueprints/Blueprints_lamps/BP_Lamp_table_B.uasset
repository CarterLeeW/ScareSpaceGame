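; Table lamp prop whose shade, body and bulb share switchable on and off materials, with an optional point light.
; The construction script applies the materials from LampOn and destroys the point light if the lamp is off or AddLight is false.
; TurnLighton and TurnLightOff events swap the materials and set the light to BaseIntensity or zero, without recreating a destroyed light.
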(event EventBeginPlay)

(event Collision|EventActorBeginOverlap
  (params (OtherActor :type Actor%20Object%20Reference)))

(event EventTick
  (params (DeltaSeconds :type Float%20%28single-precision%29)))

(event EventTurnLightOff
  (Rendering|Material|SetMaterial (Variables|Default|GetLamp_table_B_shade) 0 "/Game/HousePropsFurniture/Materials/MI_Lamps_table_off.MI_Lamps_table_off")
  (Rendering|Material|SetMaterial (Variables|Default|GetLamp_table_B) 0 "/Game/HousePropsFurniture/Materials/MI_Lamps_table_off.MI_Lamps_table_off")
  (Rendering|Material|SetMaterial (Variables|Default|GetLamp_bulb) 0 "/Game/HousePropsFurniture/Materials/MI_Lamps_table_off.MI_Lamps_table_off")
  (Rendering|Components|Light|SetIntensity (Variables|Default|GetPointLight) 0.0))

(event EventTurnLighton
  (Rendering|Material|SetMaterial (Variables|Default|GetLamp_table_B_shade) 0 "/Game/HousePropsFurniture/Materials/MI_Lamps_table_on.MI_Lamps_table_on")
  (Rendering|Material|SetMaterial (Variables|Default|GetLamp_table_B) 0 "/Game/HousePropsFurniture/Materials/MI_Lamps_table_on.MI_Lamps_table_on")
  (Rendering|Material|SetMaterial (Variables|Default|GetLamp_bulb) 0 "/Game/HousePropsFurniture/Materials/MI_Lamps_table_on.MI_Lamps_table_on")
  (Rendering|Components|Light|SetIntensity (Variables|Default|GetPointLight) (Variables|Default|GetBase%20Intensity)))

(fn ConstructionScript
  (if (Variables|Lamp|GetLamp%20On?)
    (Rendering|Material|SetMaterial (Variables|Default|GetLamp_table_B_shade) 0 "/Game/HousePropsFurniture/Materials/MI_Lamps_table_on.MI_Lamps_table_on")
    (Rendering|Material|SetMaterial (Variables|Default|GetLamp_table_B) 0 "/Game/HousePropsFurniture/Materials/MI_Lamps_table_on.MI_Lamps_table_on")
    (Rendering|Material|SetMaterial (Variables|Default|GetLamp_bulb) 0 "/Game/HousePropsFurniture/Materials/MI_Lamps_table_on.MI_Lamps_table_on")
    (if (not (Variables|Lamp|GetAdd%20Light?))
      (Components|DestroyComponent (Variables|Default|GetPointLight)))
    (else
      (Components|DestroyComponent (Variables|Default|GetPointLight))
      (Rendering|Material|SetMaterial (Variables|Default|GetLamp_table_B_shade) 0 "/Game/HousePropsFurniture/Materials/MI_Lamps_table_off.MI_Lamps_table_off")
      (Rendering|Material|SetMaterial (Variables|Default|GetLamp_table_B) 0 "/Game/HousePropsFurniture/Materials/MI_Lamps_table_off.MI_Lamps_table_off")
      (Rendering|Material|SetMaterial (Variables|Default|GetLamp_bulb) 0 "/Game/HousePropsFurniture/Materials/MI_Lamps_table_off.MI_Lamps_table_off")
      (Transformation|SetMobility (Variables|Default|GetLamp_table_B_shade) "Static"))))