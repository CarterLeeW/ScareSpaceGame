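; Ceiling fan lamp prop whose lit or unlit look is configured at construction.
; The construction script uses LampOn to apply the on or off lamp material to the blade and base meshes.
; The SpotLight component survives only when both LampOn and AddLight are set, otherwise it is destroyed.
; The event graph holds no active logic, so nothing toggles or animates at runtime through this Blueprint's graphs.
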(event EventBeginPlay)

(event Collision|EventActorBeginOverlap
  (params (OtherActor :type Actor%20Object%20Reference)))

(event EventTick
  (params (DeltaSeconds :type Float%20%28single-precision%29)))

(fn ConstructionScript
  (if (Variables|Lamp|GetLamp%20On?)
    (Rendering|Material|SetMaterial (Variables|Default|GetLamp_ceilingfan_blades) 0 "/Game/HousePropsFurniture/Materials/MI_Lamps_C_on.MI_Lamps_C_on")
    (Rendering|Material|SetMaterial (Variables|Default|GetLamp_ceilingfan_base) 0 "/Game/HousePropsFurniture/Materials/MI_Lamps_C_on.MI_Lamps_C_on")
    (if (not (Variables|Lamp|GetAdd%20Light?))
      (Components|DestroyComponent (Variables|Default|GetSpotLight)))
    (else
      (Components|DestroyComponent (Variables|Default|GetSpotLight))
      (Rendering|Material|SetMaterial (Variables|Default|GetLamp_ceilingfan_blades) 0 "/Game/HousePropsFurniture/Materials/MI_Lamps_C_OFF.MI_Lamps_C_off")
      (Rendering|Material|SetMaterial (Variables|Default|GetLamp_ceilingfan_base) 0 "/Game/HousePropsFurniture/Materials/MI_Lamps_C_OFF.MI_Lamps_C_off"))))