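; BP_Lamp_fluorescent_A is a placeable fluorescent lamp prop with a switchable lit or unlit look and an optional light.
; The construction script uses LampOn to set the mesh's first material slot to an on or off material.
; It destroys the RectLight component when the lamp is off or AddLight is false.
; The event graph holds only disabled placeholder events, so nothing changes at runtime.
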(event EventBeginPlay)

(event Collision|EventActorBeginOverlap
  (params (OtherActor :type Actor%20Object%20Reference)))

(event EventTick
  (params (DeltaSeconds :type Float%20%28single-precision%29)))

(fn ConstructionScript
  (if (Variables|Default|GetLamp%20On?)
    (Rendering|Material|SetMaterial (Variables|Debug|GetStaticMeshComponent) 0 "/Game/HousePropsFurniture/Materials/MI_Lamps_C_on.MI_Lamps_C_on")
    (if (not (Variables|Lamp|GetAdd%20Light?))
      (Components|DestroyComponent (Variables|Default|GetRectLight)))
    (else
      (Components|DestroyComponent (Variables|Default|GetRectLight))
      (Rendering|Material|SetMaterial (Variables|Debug|GetStaticMeshComponent) 0 "/Game/HousePropsFurniture/Materials/MI_Lamps_C_OFF.MI_Lamps_C_off"))))