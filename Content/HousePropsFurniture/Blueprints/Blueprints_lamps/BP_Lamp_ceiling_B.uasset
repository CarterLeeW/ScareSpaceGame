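; BP_Lamp_ceiling_B is a ceiling lamp prop with a static mesh and a spot light that can be on or off.
; The construction script sets the on or off material from LampOn and destroys the spot light unless both LampOn and AddLight are true.
; TurnLightOff and TurnLighton events swap the material at runtime and set the light intensity to zero or BaseIntensity.
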(event EventBeginPlay)

(event Collision|EventActorBeginOverlap
  (params (OtherActor :type Actor%20Object%20Reference)))

(event EventTick
  (params (DeltaSeconds :type Float%20%28single-precision%29)))

(event EventTurnLightOff
  (Rendering|Material|SetMaterial (Variables|Debug|GetStaticMeshComponent) 0 "/Game/HousePropsFurniture/Materials/MI_Lamps_C_OFF.MI_Lamps_C_off")
  (Rendering|Components|Light|SetIntensity (Variables|Default|GetSpotLight) 0.0))

(event EventTurnLighton
  (Rendering|Material|SetMaterial (Variables|Debug|GetStaticMeshComponent) 0 "/Game/HousePropsFurniture/Materials/MI_Lamps_C_on.MI_Lamps_C_on")
  (Rendering|Components|Light|SetIntensity (Variables|Default|GetSpotLight) (Variables|Default|GetBase%20Intensity)))

(fn ConstructionScript
  (if (Variables|Lamp|GetLamp%20On?)
    (Rendering|Material|SetMaterial (Variables|Debug|GetStaticMeshComponent) 0 "/Game/HousePropsFurniture/Materials/MI_Lamps_C_on.MI_Lamps_C_on")
    (if (not (Variables|Lamp|GetAdd%20Light?))
      (Components|DestroyComponent (Variables|Default|GetSpotLight)))
    (else
      (Components|DestroyComponent (Variables|Default|GetSpotLight))
      (Rendering|Material|SetMaterial (Variables|Debug|GetStaticMeshComponent) 0 "/Game/HousePropsFurniture/Materials/MI_Lamps_C_OFF.MI_Lamps_C_off"))))