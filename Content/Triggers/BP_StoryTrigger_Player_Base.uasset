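; Base story trigger Blueprint that gives trigger actors helpers for advancing the linear story when the player is involved.
; One helper checks whether an overlapping actor is a valid, player-controlled PlayerCharacter other than itself.
; The other advances the LinearStoryProgressionSubsystem to a new phase only if the current phase matches a required one, returning whether it succeeded.
; Its own event graph is empty.
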(event EventBeginPlay)

(event Collision|EventActorBeginOverlap
  (params (OtherActor :type Actor%20Object%20Reference)))

(event EventTick
  (params (DeltaSeconds :type Float%20%28single-precision%29)))

(fn ConstructionScript)

(fn IsCollisionwithPlayerCharacter
  (params (Other%20Actor :type Object%20Object%20Reference))
  (if (and (Utilities|IsValid Other%20Actor) (!= self Other%20Actor))
    (bind _asplayer_character (Utilities|Casting|CastToPlayerCharacter Other%20Actor)
      (:then
        (return (and (Pawn|IsPlayerControlled _asplayer_character) (Utilities|IsValid _asplayer_character))))
      (:CastFailed
        (return false)))))

(fn TriggerNewPhase
  (params (New%20Phase :type EStoryPhase%20Enum :default "ArriveAtHouse") (Required%20Current%20Phase :type EStoryPhase%20Enum :default "ArriveAtHouse"))
  (if (Utilities|Enum|Equal(Enum) Required%20Current%20Phase (Class|LinearStoryProgressionSubsystem|GetCurrentPhase (Subsystems|GetLinearStoryProgressionSubsystem)))
    (Class|LinearStoryProgressionSubsystem|AdvancetoPhase (Subsystems|GetLinearStoryProgressionSubsystem) New%20Phase)
    (return true)
    (else
      (return false))))