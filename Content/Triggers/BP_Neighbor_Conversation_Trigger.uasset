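; A one-shot trigger volume that stages the neighbor conversation when the player arrives during the ArriveAtHouse story phase.
; On overlap it spawns BP_Neighbor at a spawn point facing the player, head-tracking their camera, then starts the neighbor dialogue and disables its collision.
; When dialogue ends, it stops head tracking and sends the neighbor walking away via two target points.
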(event OnComponentBeginOverlap(TriggerVolume)
  (params (OverlappedComponent :type Primitive%20Component%20Object%20Reference) (OtherActor :type Actor%20Object%20Reference) (OtherComp :type Primitive%20Component%20Object%20Reference) (OtherBodyIndex :type Integer) (bFromSweep :type Boolean) (SweepResult :type Hit%20Result%20Structure%20%28by%20ref%29))
  (if (and (Utilities|Enum|Equal(Enum) (Class|LinearStoryProgressionSubsystem|GetCurrentPhase (Subsystems|GetLinearStoryProgressionSubsystem)) "ArriveAtHouse") (not (Variables|Default|GetHas%20Been%20Triggered)))
    (if (CallFunction|IsCollisionwithPlayerCharacter OtherActor)
      (Variables|Default|SetHas%20Been%20Triggered true)
      (bind _neighbor (CallFunction|SpawnNeighbor))
      (bind _dialogue_object (CallFunction|StartDialogueSequence "/Game/Data/Dialogue/DDA_Neighbor.DDA_Neighbor" _neighbor))
      (EventDispatchers|AssignDialogueEnds _dialogue_object (delegate Custom|Dialogue%20Ends_Event))
      (Collision|SetCollisionEnabled (Variables|Default|GetTrigger%20Volume) "NoCollision"))))

(event Custom|Dialogue%20Ends_Event
  (Utilities|IsValid (stale OnComponentBeginOverlap(TriggerVolume) _neighbor)
    (:Is%20Valid
      (Default|DisableHeadTracking (stale OnComponentBeginOverlap(TriggerVolume) _neighbor))
      (Variables|/Game/Characters/Urban_Nomad/BP_Neighbor.BP_Neighbor_C|SetFirst%20Walk%20Away%20Target (stale OnComponentBeginOverlap(TriggerVolume) _neighbor) (Variables|Default|GetNeighbor%20Walk%20Away%20First%20Target))
      (Variables|/Game/Characters/Urban_Nomad/BP_Neighbor.BP_Neighbor_C|SetSecond%20Walk%20Away%20Target (stale OnComponentBeginOverlap(TriggerVolume) _neighbor) (Variables|Default|GetNeighbor%20Walk%20Away%20Second%20Target))
      (Default|StartWalkingAwaySequence (stale OnComponentBeginOverlap(TriggerVolume) _neighbor) true))))

(event EventBeginPlay
  (|CallParentFunction) ; This node is disabled and will not be called.\nDrag off pins to build functionality.
)

(event Collision|EventActorBeginOverlap
  (params (OtherActor :type Actor%20Object%20Reference))
  (|CallParentFunction OtherActor) ; This node is disabled and will not be called.\nDrag off pins to build functionality.
)

(fn ConstructionScript
  (|CallParentFunction))

(fn SpawnNeighbor
  (bind _returnvalue (Game|SpawnActorfromClass "/Game/Characters/Urban_Nomad/BP_Neighbor.BP_Neighbor_C" (Math|Transform|MakeTransform (Transformation|GetActorLocation (Variables|Default|GetNeighbor%20Spawn%20Point)) (Math|Rotator|FindLookatRotation (Transformation|GetActorLocation (Variables|Default|GetNeighbor%20Spawn%20Point)) (Transformation|GetActorLocation (Game|GetPlayerCharacter 0)))) "AlwaysSpawn" "MultiplyWithRoot" 0 0))
  (bind _asbp_player_character (Utilities|Casting|CastToBP_PlayerCharacter (Game|GetPlayerCharacter 0))
    (:then
      (Utilities|IsValid _returnvalue
        (:Is%20Valid
          (Default|UpdateHeadTrackingComponent _returnvalue (Variables|/Script/ScareSpace.PlayerCharacter|GetFirstPersonCameraComponent _asbp_player_character)))
        (:Is%20Not%20Valid
          _)))
    (:CastFailed
      _))
  (return _returnvalue))