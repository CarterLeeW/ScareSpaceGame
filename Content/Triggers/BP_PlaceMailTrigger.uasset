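; Story trigger actor where the player places the mail during the BringInMail phase.
; Interaction is enabled only in that phase, tracked through the linear story progression subsystem.
; An inventory-update binding and a dynamic material let the interaction area show only while the mail is in the player's inventory.
; Interacting reveals the mail mesh and advances the story to GoToBed.
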(event OnInteractwithItem(ItemInteractable)
  (params (Interactor :type Interactor%20Component%20Object%20Reference))
  (Rendering|SetVisibility (Variables|Default|GetMail%20Mesh) true false)
  (Class|LinearStoryProgressionSubsystem|AdvancetoPhase (Subsystems|GetLinearStoryProgressionSubsystem) "GoToBed"))

(event Custom|OnStoryPhaseAdvanced_Event
  (params (NewPhase :type EStoryPhase%20Enum :default "ArriveAtHouse"))
  (Variables|/Script/ScareSpace.InteractableComponent|SetbCanInteract (Variables|Default|GetItemInteractable) (Utilities|Enum|Equal(Enum) NewPhase "BringInMail")))

(event EventBeginPlay
  (Variables|/Script/ScareSpace.InteractableComponent|SetbCanInteract (Variables|Default|GetItemInteractable) (Utilities|Enum|Equal(Enum) (Class|LinearStoryProgressionSubsystem|GetCurrentPhase (Subsystems|GetLinearStoryProgressionSubsystem)) "BringInMail"))
  (EventDispatchers|AssignOnStoryPhaseAdvanced (Subsystems|GetLinearStoryProgressionSubsystem) (delegate Custom|OnStoryPhaseAdvanced_Event))
  (bind _asplayer_character (Utilities|Casting|CastToPlayerCharacter (Game|GetPlayerCharacter 0)))
  (EventDispatchers|BindEventtoOnInventoryUpdated (Variables|/Script/ScareSpace.PlayerCharacter|GetInventoryComponent _asplayer_character) (EventDispatchers|CreateEvent :!event ToggleOpacity)))

(event Collision|EventActorBeginOverlap
  (params (OtherActor :type Actor%20Object%20Reference)))

(event EventTick
  (params (DeltaSeconds :type Float%20%28single-precision%29)))

(fn ConstructionScript
  (bind _returnvalue (Rendering|Material|CreateDynamicMaterialInstance (Variables|Default|GetInteraction%20Area) 0 0 "None" :!class /Script/Engine.PrimitiveComponent))
  (bind _output_get (Variables|Default|SetDynamic%20Material%20Instance _returnvalue))
  (Rendering|Material|SetScalarParameterValue _output_get "Opacity" 0.0 :!class /Script/Engine.MaterialInstanceDynamic))

(fn ToggleOpacity
  (params (NewItemSet :type Array%20of%20Data%20Table%20Row%20Handle%20Structures))
  (Rendering|Material|SetScalarParameterValue (Variables|Default|GetDynamic%20Material%20Instance) "Opacity" (Math|Float|SelectFloat 0.6 0.0 (!= (Utilities|Array|FindItem NewItemSet (LocalVariables|GetMail%20Data%20Table%20Row%20Handle)) -1)) :!class /Script/Engine.MaterialInstanceDynamic)
  (return))