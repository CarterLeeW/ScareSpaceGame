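; BP_HoseSpline is a spline-based prop that builds a hose from repeated static meshes in the Construction Script.
; It steps along the spline at a fixed Spacing, adding mesh components with the configured Mesh and Size, aligned to the spline's local rotation.
; Each step places meshes at both its current and previous distance, so interior points receive overlapping duplicates.
; Meshes are placed rigidly, without spline-mesh deformation.
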(fn ConstructionScript
  (for _index (range 1 (.ReturnValue (Math|Float|Division(WholeandRemainder) (Spline|GetSplineLength (Variables|Default|GetSpline)) (Variables|Default|GetSpacing))))
    (bind _returnvalue (AddComponent|AddStaticMeshComponent false (Math|Transform|MakeTransform (Spline|GetLocationatDistanceAlongSpline (Variables|Default|GetSpline) (* _index (Variables|Default|GetSpacing)) "Local") (Spline|GetRotationatDistanceAlongSpline (Variables|Default|GetSpline) (* _index (Variables|Default|GetSpacing)) "Local") (Variables|Default|GetSize))))
    (Components|StaticMesh|SetStaticMesh _returnvalue (Variables|Default|GetMesh))
    (bind _returnvalue_2 (AddComponent|AddStaticMeshComponent false (Math|Transform|MakeTransform (Spline|GetLocationatDistanceAlongSpline (Variables|Default|GetSpline) (- (* _index (Variables|Default|GetSpacing)) (Variables|Default|GetSpacing)) "Local") (Math|Rotator|MakeRotator (.Roll (Math|Rotator|BreakRotator (Spline|GetRotationatDistanceAlongSpline (Variables|Default|GetSpline) (- (* _index (Variables|Default|GetSpacing)) (Variables|Default|GetSpacing)) "Local"))) (.Pitch (Math|Rotator|BreakRotator (Spline|GetRotationatDistanceAlongSpline (Variables|Default|GetSpline) (- (* _index (Variables|Default|GetSpacing)) (Variables|Default|GetSpacing)) "Local"))) (.Yaw (Math|Rotator|BreakRotator (Spline|GetRotationatDistanceAlongSpline (Variables|Default|GetSpline) (- (* _index (Variables|Default|GetSpacing)) (Variables|Default|GetSpacing)) "Local")))) (Variables|Default|GetSize))))
    (Components|StaticMesh|SetStaticMesh _returnvalue_2 (Variables|Default|GetMesh))))